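; Paired UXT pinch slider that drives assembly of the Island 03 bridge, mirroring its value and interaction state to its TwinSlider.
; While active, dragging feeds the inverted value to the bridge; near zero, both sliders deactivate and the ramp completes, though they remain grabbable.
; When released early, Tick eases the slider back to start, reversing assembly.
; A spawned outline actor and hint component give visual feedback; thumb speed sets tick volume, slider value its pitch.
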(event `self.ReceiveBeginPlay`
  (bind _interactiveeffect (`self.interactiveEffect`))
  (bind _sliderthumb (`self.SliderThumb`))
  (`parent.ReceiveBeginPlay`)
  (`|ExecutionSequence`
    (:`then_0`
      (bind _returnvalue (`GameplayStatics.GetActorOfClass` "/Game/Blueprints/BP_Island03Bridge.BP_Island03Bridge_C"))
      (`/Engine/EditorBlueprintResources/StandardMacros.IsValid` _returnvalue
        (:`Is Valid`
          (set `self.LinkedBridge` _returnvalue))
        (:`Is Not Valid`
          (`KismetSystemLibrary.PrintString` "Error: Slider not associated with a bridge" true true (struct :`R` 1.0 :`A` 1.0)))))
    (:`then_1`
      ;[1 1 1] Spawn interactive object effect BP
      (bind _returnvalue_2 (`|SpawnActorFromClass` "/Game/Blueprints/BP_InteractiveObjectsEffect_Outline.BP_InteractiveObjectsEffect_Outline_C" (`KismetMathLibrary.MakeTransform` (`SceneComponent.K2_GetComponentLocation` _sliderthumb) (`SceneComponent.K2_GetComponentRotation` _sliderthumb) (`SceneComponent.K2_GetComponentScale` _sliderthumb)) "Undefined" "OverrideRootScale" null null))
      (set `self.interactiveEffect` _returnvalue_2)
      (`self.K2_AttachToComponent` _interactiveeffect _sliderthumb "None" "KeepWorld" "KeepWorld" "KeepWorld" true)
      (`StaticMeshComponent.SetStaticMesh` (`/Game/Blueprints/BP_InteractiveObjectsEffect_Outline.outlineMesh` _interactiveeffect) "/Game/Art/Temple/SM_Temple_Lever_Outline.SM_Temple_Lever_Outline"))))

(event `/Game/Blueprints/BP_GlowHintInterface.EnableHintParticles`
  ;[0 0 0] Activate/Deactivate hint effect
  (`/Game/Blueprints/BP_GlowHintComponent.ActivateParticleSystem` (`self.BP_GlowHintComponent`) :!label _label))

(event `/Game/Blueprints/BP_GlowHintInterface.ActivateHint`
  ;[0 0 0] Activate/Deactivate hint effect
  (`/Game/Blueprints/BP_GlowHintComponent.ActivateOutliner` (`self.BP_GlowHintComponent`) (`self.SliderThumb`))
  (goto _label))

(event `ActivateSlider`
  ;[1 0.8965 0] Slider is still grabbable unforntualy
  (set `self.Active` true)
  (set `/Game/Blueprints/BP_InteractiveObjectsEffect_Outline.isActive` true (`self.interactiveEffect`)))

(event `/Game/Blueprints/BP_GlowHintInterface.DisableHintParticles`
  ;[0 0 0] Activate/Deactivate hint effect
  (`/Game/Blueprints/BP_GlowHintComponent.DeactivateParticleSystem` (`self.BP_GlowHintComponent`) :!label _label_2))

(event `/Game/Blueprints/BP_GlowHintInterface.DeactivateHint`
  ;[0 0 0] Activate/Deactivate hint effect
  (`/Game/Blueprints/BP_GlowHintComponent.DeactivateOutliner` (`self.BP_GlowHintComponent`) (`self.SliderThumb`))
  (goto _label_2))

(event `DeactivateSlider`
  ;[1 0.8965 0] Slider is still grabbable unforntualy
  (set `self.Active` false)
  (set `/Game/Blueprints/BP_InteractiveObjectsEffect_Outline.isActive` false (`self.interactiveEffect`)))

(event `/Game/Framework/BP_GazeTriggerInterface.OnGazeBegin`
  ;[1 1 1] Gaze
  (set `/Game/Blueprints/BP_InteractiveObjectsEffect_Outline.isLookedAt` true (`self.interactiveEffect`))
  (set `/Game/Blueprints/BP_InteractiveObjectsEffect_Outline.isLookedAt` true (`/Game/Blueprints/BP_TwinSlider.interactiveEffect` (`self.twinSlider`))))

(event `self.UxtPinchSlider.OnBeginFocus`
  (params (Slider :type "UxtPinchSliderComponent Object Reference") (Pointer :type "UxtPointerComponent Object Reference") (bWasAlreadyFocused :type Boolean))
  ;[1 1 1] Grab Focus
  (set `/Game/Blueprints/BP_InteractiveObjectsEffect_Outline.grabFocus` true (`self.interactiveEffect`))
  (set `/Game/Blueprints/BP_InteractiveObjectsEffect_Outline.grabFocus` true (`/Game/Blueprints/BP_TwinSlider.interactiveEffect` (`self.twinSlider`))))

(event `self.UxtPinchSlider.OnInteractionStarted`
  (bind _thumbinteract (`self.ThumbInteract`))
  ;[1 1 1] Grab
  (`/Game/Blueprints/BP_GlowHintComponent.DeactivateParticleSystem` (`self.BP_GlowHintComponent`))
  (`/Game/Blueprints/BP_GlowHintComponent.DeactivateParticleSystem` (`/Game/Blueprints/BP_TwinSlider.BP_GlowHintComponent` (`self.twinSlider`)))
  (set `self.Held` true)
  (set `/Game/Blueprints/BP_TwinSlider.Held` true (`self.twinSlider`))
  (set `/Game/Blueprints/BP_InteractiveObjectsEffect_Outline.isGrabbed` true (`self.interactiveEffect`))
  ;;[0 0 0] GCVRS - fade in/out looping audio based on interaction
  (`AudioComponent.SetSound` _thumbinteract "/UXTools/Slider/Audio/A_Slider_Grab.A_Slider_Grab")
  (`AudioComponent.Play` _thumbinteract 0.0)
  (`AudioComponent.FadeIn` (`self.ThumbNotchTick`) 0.1 1.0 0.0 "Linear"))

(event `/Game/Framework/BP_GazeTriggerInterface.OnGazeEnd`
  ;[1 1 1] Gaze
  (set `/Game/Blueprints/BP_InteractiveObjectsEffect_Outline.isLookedAt` false (`self.interactiveEffect`))
  (set `/Game/Blueprints/BP_InteractiveObjectsEffect_Outline.isLookedAt` false (`/Game/Blueprints/BP_TwinSlider.interactiveEffect` (`self.twinSlider`))))

(event `self.UxtPinchSlider.OnEndFocus`
  (params (Slider :type "UxtPinchSliderComponent Object Reference") (Pointer :type "UxtPointerComponent Object Reference") (bIsStillFocused :type Boolean))
  ;[1 1 1] Grab Focus
  (set `/Game/Blueprints/BP_InteractiveObjectsEffect_Outline.grabFocus` false (`self.interactiveEffect`))
  (set `/Game/Blueprints/BP_InteractiveObjectsEffect_Outline.grabFocus` false (`/Game/Blueprints/BP_TwinSlider.interactiveEffect` (`self.twinSlider`))))

(event `self.UxtPinchSlider.OnInteractionEnded`
  (bind _thumbinteract (`self.ThumbInteract`))
  ;[1 1 1] Grab
  (set `self.Held` false)
  (set `/Game/Blueprints/BP_TwinSlider.Held` false (`self.twinSlider`))
  (set `/Game/Blueprints/BP_InteractiveObjectsEffect_Outline.isGrabbed` false (`self.interactiveEffect`))
  ;;[0 0 0] GCVRS - fade in/out looping audio based on interaction
  (`AudioComponent.SetSound` _thumbinteract "/UXTools/Slider/Audio/A_Slider_Release.A_Slider_Release")
  (`AudioComponent.Play` _thumbinteract 0.0)
  (`AudioComponent.FadeOut` (`self.ThumbNotchTick`) 0.1 0.0 "Linear"))

(event `self.UxtPinchSlider.OnUpdateValue`
  (params (Slider :type "UxtPinchSliderComponent Object Reference") (NewValue :type "Float (single-precision)"))
  (bind _aud_sliderlock_cue (`self.AUD_SliderLock_Cue`))
  (set `UxtPinchSliderComponent.SliderValue` NewValue (`/UXTools/Slider/BP_SimpleSlider.UxtPinchSlider` (`self.twinSlider`)))
  ;[0 0 0] GVCRS
  (`self.ControlSliderAudio`)
  (if (`self.Active`)
    (`|ExecutionSequence`
      (:`then_0`
        (`/Game/Blueprints/BP_Island03Bridge.Event_BridgeAssemble` (`self.LinkedBridge`) (- 1.0 NewValue)))
      (:`then_1`
        ;[1 1 1] TODO: Implement slider disable
        (if (<= NewValue 0.1)
          (`self.DeactivateSlider`)
          (`self.DeactivateSlider` (`self.twinSlider`))
          (`/Game/Blueprints/BP_Island03Bridge.Event_RampCompleted` (`self.LinkedBridge`))
          ;[0 0 0] GCVRS - deactivate slider audio, silence for now
          (`/Engine/EditorBlueprintResources/StandardMacros.DoOnce` false
            (:`Completed`
              (if (not (`AudioComponent.IsPlaying` _aud_sliderlock_cue))
                (`AudioComponent.Play` _aud_sliderlock_cue 0.0)
                (`AudioComponent.FadeOut` (`self.ThumbNotchTick`) 0.2 0.0 "Linear")))))))))

(event `self.UxtPinchSlider.OnStateUpdated`)

(event `self.ReceiveTick`
  (params (DeltaSeconds :type "Float (single-precision)"))
  (bind _slidervalue (`UxtPinchSliderComponent.SliderValue` (`/UXTools/Slider/BP_SimpleSlider.UxtPinchSlider` (`self.twinSlider`))))
  ;[0 0 0] GCVRS - Pitch of notch tick
  (`AudioComponent.SetFloatParameter` (`self.ThumbNotchTick`) "pitch" _slidervalue)
  ;[1 1 1] moves sliders back to initial position
  (if (`self.Held`)
    _
    (elif (not (`KismetMathLibrary.NearlyEqual_FloatFloat` _slidervalue 1.0 0.01))
      (if (`self.Active`)
        (set `UxtPinchSliderComponent.SliderValue` (`KismetMathLibrary.FInterpTo` _slidervalue 1.0 (`GameplayStatics.GetWorldDeltaSeconds`) 1.0) (`self.UxtPinchSlider`))
        (`/Game/Blueprints/BP_Island03Bridge.Event_BridgeAssemble` (`self.LinkedBridge`) (- 1.0 _slidervalue))))))

(fn `ControlSliderAudio`
  (locals (Speed :type "Float (double-precision)" :default 0.0))
  (set `self.PrevPosition` (`self.CurrPosition`))
  (bind _output_get (set `self.CurrPosition` (`SceneComponent.K2_GetComponentLocation` (`self.SliderThumb`))))
  (`AudioComponent.SetVolumeMultiplier` (`self.ThumbNotchTick`) (`KismetMathLibrary.MapRangeClamped` (/ (`KismetMathLibrary.VSize` (- _output_get (`self.PrevPosition`))) (`GameplayStatics.GetWorldDeltaSeconds`)) 0.0 50.0 0.0 1.0)))

(fn `DisableSlider`
  (return))

(fn `IsGrabFocusable`
  (params (Primitive :type "PrimitiveComponent Object Reference"))
  (returns (ReturnValue :type Boolean))
  (return false))

(fn `UserConstructionScript`
  (`parent.UserConstructionScript`))