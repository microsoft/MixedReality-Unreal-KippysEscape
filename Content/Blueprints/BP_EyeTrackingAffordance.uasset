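; BP_EyeTrackingAffordance is a sphere indicator that responds to a ray hit state, named as an affordance for eye tracking.
; The construction script creates a dynamic material instance on the sphere.
; Event_RayHit shows the sphere in green on a hit, and otherwise recolors it salmon and hides it.
; An AffordanceAnim timeline would drive the sphere's scale, but nothing runs it.
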(event `Event_RayHit`
  (params (RayHit :type Boolean))
  (bind _mat (`self.Mat`))
  (if RayHit
    (`MaterialInstanceDynamic.SetVectorParameterValue` _mat "Color" (struct :`G` 1.0 :`B` 0.332452 :`A` 1.0))
    (`SceneComponent.SetVisibility` (`self.Sphere`) true true)
    (else
      (`MaterialInstanceDynamic.SetVectorParameterValue` _mat "Color" (struct :`R` 1.0 :`G` 0.531848 :`B` 0.451961 :`A` 1.0))
      (`SceneComponent.SetVisibility` (`self.Sphere`) false false))))

(fn `UserConstructionScript`
  (bind _sphere (`self.Sphere`))
  (bind _returnvalue (`PrimitiveComponent.CreateDynamicMaterialInstance` _sphere 0 (`PrimitiveComponent.GetMaterial` _sphere 0) "None"))
  (set `self.Mat` _returnvalue))