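; Reset button actor built on a UXT pressable button, which announces its release through an event dispatcher for other logic to handle.
; On BeginPlay it spawns and attaches an outline effect actor, and Activate/Deactivate gate both that effect and button input.
; Focus and press events drive a scale timeline, outline states and sounds.
; A glow hint component provides toggleable outline and particle hints, with the outline cleared on release.
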(event `self.ReceiveBeginPlay`
  (bind _interactiveeffect (`self.interactiveEffect`))
  (bind _base (`self.Base`))
  (bind _interactiveeffect_2 (`self.interactiveEffect`))
  ;[0.3 0.3 0.3] Spawn interactive object effect BP
  (bind _returnvalue (`|SpawnActorFromClass` "/Game/Blueprints/BP_InteractiveObjectsEffect_Outline.BP_InteractiveObjectsEffect_Outline_C" (`KismetMathLibrary.MakeTransform` (`SceneComponent.K2_GetComponentLocation` _base) (`SceneComponent.K2_GetComponentRotation` _base) (`SceneComponent.K2_GetComponentScale` (`self.UxtPressableButton`))) "Undefined" "OverrideRootScale" self null))
  (set `self.interactiveEffect` _returnvalue)
  (`self.K2_AttachToComponent` _interactiveeffect_2 (`self.Base`) "None" "KeepWorld" "KeepWorld" "KeepWorld" true)
  (`StaticMeshComponent.SetStaticMesh` (`/Game/Blueprints/BP_InteractiveObjectsEffect_Outline.outlineMesh` _interactiveeffect_2) "/Game/Art/Button/SM_Button_sphere_Outline.SM_Button_sphere_Outline")
  (set `/Game/Blueprints/BP_InteractiveObjectsEffect_Outline.isActive` false _interactiveeffect)
  (set `/Game/Blueprints/BP_InteractiveObjectsEffect_Outline.thicknessActiveTarget` 0.4 _interactiveeffect)
  (set `/Game/Blueprints/BP_InteractiveObjectsEffect_Outline.thicknessFocusTarget` 0.75 _interactiveeffect)
  (set `/Game/Blueprints/BP_InteractiveObjectsEffect_Outline.activateEffectDistance` 35.0 _interactiveeffect))

(event `Activate`
  (set `self.Active` true)
  (set `/Game/Blueprints/BP_InteractiveObjectsEffect_Outline.isActive` true (`self.interactiveEffect`)))

(event `Deactivate`
  (set `self.Active` false)
  (set `/Game/Blueprints/BP_InteractiveObjectsEffect_Outline.isActive` false (`self.interactiveEffect`)))

(event `ScaleUp`
  ;[1 1 1] Interactive Scaling
  (bind (_direction _scale) (`Timeline|GrabFocusScaleTimeline` :!label _label)
    (:`Update`
      (`SceneComponent.SetRelativeScale3D` (`self.Movable`) (`KismetMathLibrary.Conv_DoubleToVector` (`KismetMathLibrary.Lerp` 1.0 1.225 _scale))))))

(event `ScaleDown`
  ;[1 1 1] Interactive Scaling
  (goto _label :!via `Reverse`))

(event `self.UxtPressableButton.OnButtonPressed`
  (params (Button :type "UxtPressableButtonComponent Object Reference") (Pointer :type "UxtPointerComponent Object Reference"))
  (if (`self.Active`)
    (`GameplayStatics.PlaySoundAtLocation` "/Game/Sounds/KippysEscape_Demo_Button_Up.KippysEscape_Demo_Button_Up" (0.0 0.0 0.0) (struct) 1.0 1.0 0.0 "/Game/Sounds/DefaultAttenuationSettings.DefaultAttenuationSettings" null null)
    (`self.ScaleDown`)
    (set `/Game/Blueprints/BP_InteractiveObjectsEffect_Outline.isGrabbed` true (`self.interactiveEffect`))))

(event `self.UxtPressableButton.OnButtonReleased`
  (params (Button :type "UxtPressableButtonComponent Object Reference") (Pointer :type "UxtPointerComponent Object Reference"))
  (if (`self.Active`)
    (`GameplayStatics.PlaySoundAtLocation` "/Game/Sounds/KippysEscape_Demo_Button_Down.KippysEscape_Demo_Button_Down" (0.0 0.0 0.0) (struct) 1.0 1.0 0.0 "/Game/Sounds/DefaultAttenuationSettings.DefaultAttenuationSettings" null null)
    (`/Game/Blueprints/BP_GlowHintInterface.DeactivateHint`)
    (`self.EventDisp_ButtonReleased`)
    (`self.ScaleUp`)
    (set `/Game/Blueprints/BP_InteractiveObjectsEffect_Outline.isGrabbed` false (`self.interactiveEffect`))
    (set `self.PressedOnce` true)))

(event `self.UxtPressableButton.OnBeginFocus`
  (params (Button :type "UxtPressableButtonComponent Object Reference") (Pointer :type "UxtPointerComponent Object Reference") (bWasAlreadyFocused :type Boolean))
  (if (`self.Active`)
    (`self.ScaleUp`)
    (set `/Game/Blueprints/BP_InteractiveObjectsEffect_Outline.grabFocus` true (`self.interactiveEffect`))))

(event `/Game/Blueprints/BP_GlowHintInterface.ActivateHint`
  (`/Game/Blueprints/BP_GlowHintComponent.ActivateOutliner` (`self.BP_GlowHintComponent`) (`self.Base`)))

(event `/Game/Blueprints/BP_GlowHintInterface.EnableHintParticles`
  (`/Game/Blueprints/BP_GlowHintComponent.ActivateParticleSystem` (`self.BP_GlowHintComponent`)))

(event `self.UxtPressableButton.OnEndFocus`
  (params (Button :type "UxtPressableButtonComponent Object Reference") (Pointer :type "UxtPointerComponent Object Reference") (bIsStillFocused :type Boolean))
  (if (`self.Active`)
    (`self.ScaleDown`)
    (set `/Game/Blueprints/BP_InteractiveObjectsEffect_Outline.grabFocus` false (`self.interactiveEffect`))))

(event `/Game/Blueprints/BP_GlowHintInterface.DeactivateHint`
  (`/Game/Blueprints/BP_GlowHintComponent.DeactivateOutliner` (`self.BP_GlowHintComponent`) (`self.Base`)))

(event `/Game/Blueprints/BP_GlowHintInterface.DisableHintParticles`
  (`/Game/Blueprints/BP_GlowHintComponent.DeactivateParticleSystem` (`self.BP_GlowHintComponent`)))

(fn `GetPokeBehaviour`
  (returns (ReturnValue :type "EUxtPokeBehaviour Enum"))
  (return "FrontFace"))

(fn `IsPokeFocusable`
  (params (Primitive :type "PrimitiveComponent Object Reference"))
  (returns (ReturnValue :type Boolean))
  (return false))

(fn `UserConstructionScript`
  (`|ExecutionSequence`
    (:`then_2`
      (`TimelineComponent.SetPlayRate` (`self.GrabFocusScaleTimeline`) 3.5))))