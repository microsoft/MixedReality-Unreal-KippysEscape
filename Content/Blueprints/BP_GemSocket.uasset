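; BP_GemSocket is a puzzle socket that accepts a BP_Gem of matching color.
; Activate waits a given delay, then rotates the socket out from the wall with a timeline and arms it.
; An overlapping matching gem snaps to the socket, which later rotates back flush, animates its light intensity and flags GemInserted.
; The construction script picks the plate mesh from ColorMatch and tints the light from GemColor.
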(event `Activate`
  (params (Delay :type "Float (double-precision)"))
  (bind _sm_socketbase (`self.SM_socketBase`))
  (bind (_relativerotation_roll _relativerotation_pitch _relativerotation_yaw) (`KismetMathLibrary.BreakRotator` (`SceneComponent.RelativeRotation` _sm_socketbase)))
  ;[1 0.7644 0 0.488] Activate - rotate socket away from wall
  (`KismetSystemLibrary.Delay` Delay)
  (`AudioComponent.Play` (`self.SocketClosed`) 0.0)
  (bind (_direction _rotateslope) (`Timeline|ActivateSocket` :!via `PlayFromStart`)
    (:`Update`
      (`SceneComponent.K2_SetRelativeRotation` _sm_socketbase (`KismetMathLibrary.RLerp` (`KismetMathLibrary.MakeRotator` _relativerotation_roll _relativerotation_pitch _relativerotation_yaw) (`KismetMathLibrary.MakeRotator` -30.0 _relativerotation_pitch _relativerotation_yaw) _rotateslope) false false)
      (set `self.Active` true))))

(event `self.ReceiveActorBeginOverlap`
  (params (OtherActor :type "Actor Object Reference"))
  (bind _correspondinggem (`self.CorrespondingGem`))
  (bind _correspondinggem_2 (`self.CorrespondingGem`))
  (bind _sm_socketbase (`self.SM_socketBase`))
  (bind (_returnvalue_location _returnvalue_rotation) (`KismetMathLibrary.BreakTransform` (`SceneComponent.GetSocketTransform` (`self.OverlapSphere`) "GemSocket" "RTS_World")))
  (bind (_relativerotation_roll _relativerotation_pitch _relativerotation_yaw) (`KismetMathLibrary.BreakRotator` (`SceneComponent.RelativeRotation` _sm_socketbase)))
  ;[0.8249 0.2058 1] Gem overlap
  (if (`self.Active`)
    ;[0.02416 0.1356 0.1413] Check if gem is correct
    (bind _asbp_gem (cast `/Game/Blueprints/BP_Gem` OtherActor))
    (if (== (`/Game/Blueprints/BP_Gem.GemColor` _asbp_gem) (`self.GemColor`))
      (set `self.CorrespondingGem` _asbp_gem)
      ;[1 0.8688 0] store socket transforms - Move to event beginPlay
      (set `/Game/Blueprints/BP_Gem.SocketLocation` _returnvalue_location _correspondinggem)
      (set `/Game/Blueprints/BP_Gem.SocketRotation` _returnvalue_rotation _correspondinggem)
      ;[0.3191 0.6674 1 0.478] deals with gem BP - Fires gem animation event and attaches it to the socket
      (`/Game/Blueprints/BP_Gem.Event InsertGem` _correspondinggem_2)
      (`SceneComponent.K2_AttachToComponent` (`Actor.RootComponent` _correspondinggem_2) (`self.OverlapSphere`) "GemSocket" "SnapToTarget" "SnapToTarget" "SnapToTarget" false)
      (`KismetSystemLibrary.Delay` 2.5)
      (`AudioComponent.Play` (`self.SocketClosed`) 0.0)
      ;[0.06125 0.1384 0.2016] Socket effect
      (bind (_direction _rotateslope _lightintensity) (`Timeline|RotateSocketToFlush` :!via `PlayFromStart`)
        (:`Update`
          (`SceneComponent.K2_SetRelativeRotation` _sm_socketbase (`KismetMathLibrary.RLerp` (`KismetMathLibrary.MakeRotator` _relativerotation_roll _relativerotation_pitch _relativerotation_yaw) (`KismetMathLibrary.MakeRotator` 0.0 _relativerotation_pitch _relativerotation_yaw) _rotateslope) false false)
          (`LightComponent.SetIntensity` (`self.PointLight`) _lightintensity))
        (:`Finished`
          ;[1 1 1] Gem inserted State change
          (set `self.GemInserted` true))))))

(fn `Get Socket Location`
  (returns (SocketLocation :type "Vector Structure"))
  (return (`SceneComponent.K2_GetComponentLocation` (`self.OverlapSphere`))))

(fn `UserConstructionScript`
  (bind _colormatch (`self.ColorMatch`))
  (`|ExecutionSequence`
    (:`then_0`
      ;[1 0.3926 0.4524] Set corresponding mesh for gem color (exposed param)
      (if (== _colormatch (struct :`R` 1.0 :`A` 1.0))
        (`SceneComponent.SetVisibility` (`self.SM_EmeraldPlate`) true false)
        (elif (== _colormatch (struct :`G` 1.0 :`A` 1.0))
          (`SceneComponent.SetVisibility` (`self.SM_RadiantPlate`) true false)
          (else
            (`SceneComponent.SetVisibility` (`self.SM_TrillionPlate`) true false)))))
    (:`then_1`
      ;[1 1 1] Set up light
      (`LightComponent.SetLightColor` (`self.PointLight`) (select `/Game/Blueprints/Enums/E_GemColor` (`self.GemColor`) :`NewEnumerator0` (make `LinearColor` 1.0 0.0 0.0 1.0) :`NewEnumerator1` (make `LinearColor` 0.0 1.0 0.0 1.0) :`NewEnumerator2` (make `LinearColor` 0.0 0.0 1.0 1.0)) true)
      (`LightComponent.SetIntensity` (`self.PointLight`) 0.0))))