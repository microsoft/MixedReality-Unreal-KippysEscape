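; Island 03 bridge that a slider interaction raises, then rotates and unfolds into a deployed state.
; The slider value scrubs a timeline that lifts segments in staggered height steps and switches their shared dynamic material between red and blue.
; Ramp completion plays a sound and rotates the segments, then a timeline animates inserts, hinges and pistons and unhides hidden hinges.
; The Construction Script caches each part's rest transform as the lerp base.
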(event `TurnBridgeEmissiveOn`
  (bind _bridgemat (`self.BridgeMat`))
  ;[1 1 1] Turn on red/BlueLights
  (`MaterialInstanceDynamic.SetScalarParameterValue` _bridgemat "EmissiveIntensity" 2.0)
  (`MaterialInstanceDynamic.SetVectorParameterValue` _bridgemat "EmissiveColour" (struct :`R` 1.0 :`B` 0.165132 :`A` 1.0)))

(event `Event_BridgeAssemble`
  (params (LerpResult :type "Float (double-precision)"))
  (bind _bridgemat (`self.BridgeMat`))
  ;[0.04025 0.5884 1 0.478] Slider Interaction - Move bridge up
  (`|ExecutionSequence`
    (:`then_0`
      (if (<= LerpResult 0.1)
        (`MaterialInstanceDynamic.SetVectorParameterValue` _bridgemat "EmissiveColour" (struct :`R` 1.0 :`B` 0.165132 :`A` 1.0))
        (else
          (`MaterialInstanceDynamic.SetVectorParameterValue` _bridgemat "EmissiveColour" (struct :`G` 1.333333 :`B` 2.0 :`A` 1.0)))))
    (:`then_1`
      (bind (_direction _moveplatforms) (`Timeline|Island03Bridge_Anim` :`NewTime` LerpResult :!via `SetNewTime`)
        (:`Update`
          (set `self.Height` (* _moveplatforms 30.0))
          (`self.MoveMe` (`self.SM_bridge_03_BridgeBase1`) 2
            (:`EventOut`
              (`self.MoveMe` (`self.SM_bridge_03_BridgeBase2`) 3
                (:`EventOut`
                  (`self.MoveMe` (`self.SM_bridge_03_BridgeBase3`) 4
                    (:`EventOut`
                      (`self.MoveMe` (`self.SM_bridge_03_BridgeBase4`) 5))))))))
        (:`Finished`
          (`self.Event_RampCompleted`))))))

(event `Event_RampCompleted`
  ;[1 0.7926 0 0.347] Rotate Bridge To Correct Angle
  (`AudioComponent.Play` (`self.GDC2020_LastBridge`) 0.0)
  (bind (_direction _rotateplatforms) (`Timeline|Island03Bridge_Rotate` :!via `PlayFromStart`)
    (:`Update`
      (`|ExecutionSequence`
        (:`then_0`
          (bind _returnvalue (* _rotateplatforms (`self.Rotation`)))
          (`self.RotateMe` (`self.SM_bridge_03_BridgeBase`) _returnvalue))
        (:`then_1`
          (`self.RotateMe` (`self.SM_bridge_03_BridgeBase1`) _returnvalue))
        (:`then_2`
          (`self.RotateMe` (`self.SM_bridge_03_BridgeBase2`) _returnvalue))
        (:`then_3`
          (`self.RotateMe` (`self.SM_bridge_03_BridgeBase3`) _returnvalue))
        (:`then_4`
          (`self.RotateMe` (`self.SM_bridge_03_BridgeBase4`) _returnvalue))))
    (:`Finished`
      (`self.PlayAnimation`))))

(event `PlayAnimation`
  (bind (_direction _insertanimation _front_hinge_animation _backhingeanimation _extendpistonsanimation) (`Timeline|OpenBridgeAnimation` :!via `PlayFromStart`)
    (:`Update`
      ;[1 1 1] Move Inserts Down
      (for _array_element (`self.InsertsArray`)
        (bind (_staticmesh _relativelocation) (break `/Game/Meshes/Island03Bridge/V2/BridgePartsRelativeData` _array_element))
        (`SceneComponent.K2_SetRelativeLocation` _staticmesh (`KismetMathLibrary.VLerp` _relativelocation (- _relativelocation (0.0 0.0 0.62)) _insertanimation) false false)
        ;[1 1 1] RotateFrontHinge
        (for _array_element_2 (`self.FrontHingeArray`)
          (bind (_staticmesh_2 _relativelocation_2 _relativerotation) (break `/Game/Meshes/Island03Bridge/V2/BridgePartsRelativeData` _array_element_2))
          (`SceneComponent.K2_SetRelativeRotation` _staticmesh_2 (`KismetMathLibrary.MakeRotator` (`KismetMathLibrary.Lerp` (.roll _relativerotation) (+ (.roll _relativerotation) 180.0) _front_hinge_animation) (.pitch _relativerotation) (.yaw _relativerotation)) false false)
          ;[1 1 1] RotateFrontHinge
          (for _array_element_3 (`self.BackHingeArray`)
            (bind (_staticmesh_3 _relativelocation_3 _relativerotation_2) (break `/Game/Meshes/Island03Bridge/V2/BridgePartsRelativeData` _array_element_3))
            (`SceneComponent.K2_SetRelativeRotation` _staticmesh_3 (`KismetMathLibrary.MakeRotator` (`KismetMathLibrary.Lerp` (.roll _relativerotation_2) (+ (.roll _relativerotation_2) 60.0) _backhingeanimation) (.pitch _relativerotation_2) (.yaw _relativerotation_2)) false false)
            ;[1 1 1] Extend pistons
            (for _array_element_4 (`self.PistonArray`)
              (bind ((`StaticMesh_11_E0C75F46430C8EB8F52DA2A9EF833FBA` _staticmesh_4) (`RelativeLocation_13_BD724A4C45F4B74CF3F2E58187FBD467` _relativelocation_4)) (break `/Game/Meshes/Island03Bridge/V2/BridgePartsRelativeData` _array_element_4))
              (`SceneComponent.K2_SetRelativeLocation` _staticmesh_4 (`KismetMathLibrary.VLerp` _relativelocation_4 (- _relativelocation_4 (0.0 3.0 0.0)) _extendpistonsanimation) false false))))))
    (:`Finished`
      (set `self.Deployed` true))
    (:`UnhideHinges`
      ;[1 1 1] Unhide hidden hinges
      (for _array_element_5 (`self.HiddenHingeArray`)
        (`SceneComponent.SetHiddenInGame` _array_element_5 false false)))))

(fn `UserConstructionScript`
  (bind _sm_bridge_03_bridgebase (`self.SM_bridge_03_BridgeBase`))
  (`|ExecutionSequence`
    (:`then_0`
      ;[0.1375 0.466 1 0.457] Setup Dyanamic material Instances for red/blue light
      (bind _returnvalue (`PrimitiveComponent.CreateDynamicMaterialInstance` _sm_bridge_03_bridgebase 0 "/Game/Meshes/Island03Bridge/V2/MI_Bridge03.MI_Bridge03" "None"))
      (bind _output_get (set `self.BridgeMat` _returnvalue))
      (bind _output_get_2 (set `self.BridgePartsArray` (`|MakeArray` _sm_bridge_03_bridgebase (`self.SM_bridge_03_BridgeBase1`) (`self.SM_bridge_03_BridgeBase2`) (`self.SM_bridge_03_BridgeBase3`) (`self.SM_bridge_03_BridgeBase4`))))
      (for _array_element _output_get_2
        (`PrimitiveComponent.SetMaterial` _array_element 0 _output_get)))
    (:`then_1`
      ;[0 0.9157 1 0.65] Get Inserts RelativeLocation
      (for (_array_element_2 _array_index) (`|MakeArray` (`self.SM_bridge_03_Insert_Ends1`) (`self.SM_bridge_03_Insert_Ends2`) (`self.SM_bridge_03_Insert_Ends3`) (`self.SM_bridge_03_Insert_Ends`) (`self.SM_bridge_03_Insert_Ends4`))
        (`KismetArrayLibrary.Array_Set` (`self.InsertsArray`) _array_index (make `/Game/Meshes/Island03Bridge/V2/BridgePartsRelativeData` _array_element_2 (`SceneComponent.RelativeLocation` _array_element_2)) true)))
    (:`then_2`
      ;[0.4074 0.9 1 0.284] Set front hinges relative Location
      (for (_array_element_3 _array_index_2) (`|MakeArray` (`self.SM_bridge_03_HingeFront1`) (`self.SM_bridge_03_HingeFront3`) (`self.SM_bridge_03_HingeFront2`) (`self.SM_bridge_03_HingeFront4`))
        (`KismetArrayLibrary.Array_Set` (`self.FrontHingeArray`) _array_index_2 (make `/Game/Meshes/Island03Bridge/V2/BridgePartsRelativeData` _array_element_3 (0.0 0.0 0.0) (`SceneComponent.RelativeRotation` _array_element_3)) true)))
    (:`then_3`
      ;[0.4074 0.9 1 0.284] Set front hinges relative Location
      (for (_array_element_4 _array_index_3) (`|MakeArray` (`self.SM_bridge_03_HingeBack`) (`self.SM_bridge_03_HingeBack1`) (`self.SM_bridge_03_HingeBack2`) (`self.SM_bridge_03_HingeBack3`) (`self.SM_bridge_03_HingeBack4`))
        (`KismetArrayLibrary.Array_Set` (`self.BackHingeArray`) _array_index_3 (make `/Game/Meshes/Island03Bridge/V2/BridgePartsRelativeData` _array_element_4 (0.0 0.0 0.0) (`SceneComponent.RelativeRotation` _array_element_4)) true)))
    (:`then_4`
      ;[0.1546 0.9502 1 0.431] Setup Piston RelativeLocation
      (for (_array_element_5 _array_index_4) (`|MakeArray` (`self.SM_bridge_03_Pistons`) (`self.SM_bridge_03_Pistons1`) (`self.SM_bridge_03_Pistons2`) (`self.SM_bridge_03_Pistons3`))
        (`KismetArrayLibrary.Array_Set` (`self.PistonArray`) _array_index_4 (make `/Game/Meshes/Island03Bridge/V2/BridgePartsRelativeData` _array_element_5 (`SceneComponent.RelativeLocation` _array_element_5)) true)))
    (:`then_5`
      ;[0.284 0.9002 1] Setup Hidden Hinge Array
      (set `self.HiddenHingeArray` (`|MakeArray` (`self.SM_bridge_03_HingeHidden`) (`self.SM_bridge_03_HingeHidden2`) (`self.SM_bridge_03_HingeHidden3`) (`self.SM_bridge_03_HingeHidden4`))))))