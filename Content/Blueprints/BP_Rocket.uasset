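; Rocket actor that opens and closes its door and launches into space on blast-off.
; A dynamic display material changes colour as the door opens and when blast-off begins, while a timeline rotates the door.
; BlastOff closes the door, then runs delayed audio, trail, puff and explosion particles alongside a timeline that lifts the fuselage and drives takeoff volume.
; When that timeline finishes, the fuselage is hidden and InSpace is set.
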(event `self.ReceiveBeginPlay`
  (bind _returnvalue (`KismetMaterialLibrary.CreateDynamicMaterialInstance` "/Game/Art/Astro/MI_RocketDisplay.MI_RocketDisplay"))
  (set `self.displayMaterial` _returnvalue)
  (`PrimitiveComponent.SetMaterial` (`self.Rocket_Fuselage`) 2 (`self.displayMaterial`)))

(event `OpenDoor`
  (`KismetSystemLibrary.Delay` 3.0)
  (`GameplayStatics.PlaySoundAtLocation` "/Game/Sounds/Rocket/SC_RocketDoorOpen.SC_RocketDoorOpen" (`SceneComponent.K2_GetComponentLocation` (`self.Rocket_Door`)) (struct) 1.0 1.0 0.0 "/Game/Sounds/DefaultAttenuationSettings.DefaultAttenuationSettings" null null)
  (`MaterialInstanceDynamic.SetVectorParameterValue` (`self.displayMaterial`) "Colour" (make `LinearColor` 0.982251 0.94251 0.0 1.0))
  (bind (_direction _lerp) (`Timeline|AnimateDoor` :!via `PlayFromStart` :!label _label)
    (:`Update`
      (`SceneComponent.K2_SetRelativeRotation` (`self.Rocket_Door`) (`KismetMathLibrary.RLerp` (struct) (struct :`Roll` 140.0) _lerp) false false))))

(event `CloseDoor`
  (`GameplayStatics.PlaySoundAtLocation` "/Game/Sounds/Rocket/SC_RocketDoorClose.SC_RocketDoorClose" (`SceneComponent.K2_GetComponentLocation` (`self.Rocket_Door`)) (struct) 1.0 1.0 0.0 "/Game/Sounds/DefaultAttenuationSettings.DefaultAttenuationSettings" null null)
  (goto _label :!via `ReverseFromEnd`))

(event `Event BlastOff`
  (bind (_returnvalue_x _returnvalue_y _returnvalue_z) (`KismetMathLibrary.BreakVector` (`SceneComponent.K2_GetComponentLocation` (`self.Rocket_Fuselage`))))
  (`KismetSystemLibrary.Delay` 2.0)
  (`MaterialInstanceDynamic.SetVectorParameterValue` (`self.displayMaterial`) "Colour" (make `LinearColor` 0.0 0.27451 1.0 1.0))
  (`self.CloseDoor`)
  (`KismetSystemLibrary.Delay` 4.0)
  (`|ExecutionSequence`
    (:`then_1`
      (`KismetSystemLibrary.Delay` 0.253)
      (`AudioComponent.Play` (`self.RopeAttachedAudio`) 0.0))
    (:`then_2`
      (`KismetSystemLibrary.Delay` 2.0)
      (`AudioComponent.Play` (`self.TakeoffAudio`) 0.0)
      ;[0 0 0] GCVRS astro take off
      (`AudioComponent.Play` (`self.AstroTakeOffCue`) 0.0)
      (`ActorComponent.Activate` (`self.RocketTrailParticles1`) false)
      (`ActorComponent.Activate` (`self.RocketTrailParticles2`) false)
      (`ActorComponent.Activate` (`self.RocketTrailParticles3`) false)
      (`ActorComponent.Activate` (`self.SinglePuff1`) false)
      (`ActorComponent.Activate` (`self.SinglePuff2`) false)
      (`ActorComponent.Activate` (`self.SinglePuff3`) false)
      (`ActorComponent.Activate` (`self.ConstantPuff1`) false)
      (`ActorComponent.Activate` (`self.ConstantPuff2`) false)
      (`ActorComponent.Activate` (`self.ConstantPuff3`) false)
      (`ActorComponent.Activate` (`self.RocketExplosionParticles`) false)
      (`ActorComponent.Activate` (`self.RocketImpactParticles`) false)
      (bind (_direction _blastoff _volume) (`Timeline|RocketBlast` :!via `PlayFromStart`)
        (:`Update`
          (`AudioComponent.AdjustVolume` (`self.TakeoffAudio`) 0.0 _volume "Linear")
          (`SceneComponent.K2_SetWorldLocation` (`self.Rocket_Fuselage`) (`KismetMathLibrary.MakeVector` _returnvalue_x _returnvalue_y (+ _blastoff _returnvalue_z)) false false))
        (:`Finished`
          (`AudioComponent.Stop` (`self.TakeoffAudio`))
          (`SceneComponent.SetHiddenInGame` (`self.Rocket_Fuselage`) true true)
          (set `self.InSpace` true))))))

(fn `UserConstructionScript`)