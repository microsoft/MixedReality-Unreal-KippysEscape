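; Bomb dispenser machine whose pressable button, once the machine is active, swings four blades open and releases its child BP_Bomb when none is armed or already out.
; Timelines animate the blades, then fly the bomb up to a looping hover until it is held.
; BombMachineHover raises and turns the casing, ramps its emissive glow and activates the machine.
; The power cable is built from spline meshes in construction and re-fitted to handle components as the casing moves.
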(event `ActivateDeactivate`
  (params (Activate :type Boolean))
  (bind _asbp_bomb_machine_button (cast `/Game/Blueprints/BP_BombMachineButton` (`ChildActorComponent.ChildActor` (`self.BP_BombMachineButton`))))
  (`/Game/Blueprints/BP_BombMachineButton.ActivateDeactivateAffordance` _asbp_bomb_machine_button Activate))

(event `self.ReceiveBeginPlay`
  (`|ExecutionSequence`
    (:`then_0`
      ;[1 0.3879 0 0.585] Set array of blade positions to lerp to
      (bind _output_get (set `self.BladeArray` (`|MakeArray` (`self.SM_BombMachineBlade1`) (`self.SM_BombMachineBlade2`) (`self.SM_BombMachineBlade3`) (`self.SM_BombMachineBlade4`))))
      (for (_array_element _array_index) _output_get
        (`KismetArrayLibrary.Array_Set` (`self.BladeTransforms`) _array_index (`SceneComponent.GetRelativeTransform` _array_element) true)
        (bind _returnvalue (`SceneComponent.GetRelativeTransform` _array_element))
        ;[1 0.7326 0 0.467] Reset blades back to origin (Closed)
        (`SceneComponent.K2_SetRelativeTransform` _array_element (`KismetMathLibrary.MakeTransform` (0.0 0.0 0.0) (`KismetMathLibrary.MakeRotator` (.roll (.rotation _returnvalue)) (.pitch (.rotation _returnvalue)) (+ (.yaw (.rotation _returnvalue)) -45.0))) false false)))
    (:`then_1`
      ;[1 0.1231 0.09321 0.546] SetupBomb Refs
      (bind _asbp_bomb (cast `/Game/Blueprints/BP_Bomb` (`ChildActorComponent.ChildActor` (`self.BP_Bomb`))))
      (set `self.BombRef` _asbp_bomb))
    (:`then_2`
      ;[0.8697 0.04638 1 0.389] Bind event to button press
      (bind _asbp_bomb_machine_button (cast `/Game/Blueprints/BP_BombMachineButton` (`ChildActorComponent.ChildActor` (`self.BP_BombMachineButton`))))
      (bind _output_get_2 (set `self.BombButtonRef` _asbp_bomb_machine_button))
      (add `UxtPressableButtonComponent.OnButtonReleased` (`/UXTools/Buttons/Common/BP_BaseButton.UxtPressableButton` _output_get_2) (delegate `ButtonReleased`)))
    (:`then_3`
      ;[1 0.3097 0 0.264] Apply mat to bomb button ref
      (`PrimitiveComponent.SetMaterial` (`/Game/Blueprints/BP_BombMachineButton.MovingVisuals` (`self.BombButtonRef`)) 0 (`self.BombMachineMat`)))))

(event `ButtonReleased`
  (params (Button :type "UxtPressableButtonComponent Object Reference") (Pointer :type "UxtPointerComponent Object Reference"))
  (bind _bombref (`self.BombRef`))
  (bind _bombref_2 (`self.BombRef`))
  (bind _returnvalue (`SceneComponent.K2_GetComponentLocation` (`self.SpawnLocation`)))
  (bind (_returnvalue_x _returnvalue_y) (`KismetMathLibrary.BreakVector` (`SceneComponent.K2_GetComponentLocation` (`self.SpawnLocation`))))
  (bind (_returnvalue_x_2 _returnvalue_y_2 _returnvalue_z) (`KismetMathLibrary.BreakVector` (`SceneComponent.K2_GetComponentLocation` (`self.SpawnLocation`))))
  (bind (_returnvalue_x_3 _returnvalue_y_3 _returnvalue_z_2) (`KismetMathLibrary.BreakVector` (+ (`SceneComponent.K2_GetComponentLocation` (`self.SpawnLocation`)) (`KismetMathLibrary.MakeVector` 0.0 0.0 (* (`self.HoverHeight`) 1.25)))))
  ;[0.8697 0.04638 1 0.389] Bind event to button press
  (if (`self.Active`)
    (if (not (or (`/Game/Blueprints/BP_Bomb.BombArmedToBlow` _bombref) (`/Game/Blueprints/BP_Bomb.BombAlreadyExists` _bombref) (`self.BladesCurrentlyOpen?`)))
      (set `self.BladesCurrentlyOpen?` true)
      (`GameplayStatics.PlaySoundAtLocation` "/Game/Sounds/BombMachine/SC_BombDispensed.SC_BombDispensed" (`SceneComponent.K2_GetComponentLocation` (`self.SpawnLocation`)) (struct) 1.0 1.0 0.0 "/Game/Sounds/DefaultAttenuationSettings.DefaultAttenuationSettings" null null)
      ;[0.1194 1 0 0.462] Lerp blade positions to open and close on press
      (bind (_direction _newtrack_0) (`Timeline|OpenBlades` :!via `PlayFromStart`)
        (:`Update`
          (for (_array_element _array_index) (`self.BladeArray`)
            (bind _output (`|GetArrayItem` (`self.BladeTransforms`) _array_index))
            (`SceneComponent.K2_SetRelativeTransform` _array_element (`KismetMathLibrary.MakeTransform` (`KismetMathLibrary.VLerp` (.location _output) (0.0 0.0 0.0) _newtrack_0) (`KismetMathLibrary.RLerp` (`KismetMathLibrary.MakeRotator` (.roll (.rotation _output)) (.pitch (.rotation _output)) (.yaw (.rotation _output))) (`KismetMathLibrary.MakeRotator` (.roll (.rotation _output)) (.pitch (.rotation _output)) (- (.yaw (.rotation _output)) 45.0)) 0.0 true)) false false)))
        (:`Finished`
          (set `self.BladesCurrentlyOpen?` false))
        (:`SpawnBomb`
          ;[0.4623 0.476 1 0.467] Wake bomb and fire sound
          (`/Game/Blueprints/BP_Bomb.WakeBomb` (`self.BombRef`) false)
          (`AudioComponent.Play` (`self.Audio_Click`) 0.2)
          (set `/Game/Blueprints/BP_Bomb.BombAlreadyExists` true (`self.BombRef`))
          ;[1 0.646 0.03523 0.399] Lerp bomb to hover position
          (bind (_direction_2 _newtrack_0_2) (`Timeline|Bomb fly out of machine` :!via `PlayFromStart` :!label _label)
            (:`Update`
              (if (`/Game/Blueprints/BP_Bomb.IsBombHeld?` _bombref_2)
                (goto _label :!via `Stop`)
                (else
                  (`SceneComponent.K2_SetWorldLocation` (`/Game/Blueprints/BP_Bomb.BombMesh` _bombref_2) (`KismetMathLibrary.VLerp` _returnvalue (+ _returnvalue (`KismetMathLibrary.MakeVector` 0.0 0.0 (`self.HoverHeight`))) _newtrack_0_2) false false))))
            (:`Finished`
              (if (not (`/Game/Blueprints/BP_Bomb.IsBombHeld?` (`self.BombRef`)))
                ;[1 0.943 0 0.337] Make bomb hover on loop until grabbed
                (bind (_direction_3 _zoffset) (`Timeline|Bomb hover` :!via `PlayFromStart` :!label _label_2)
                  (:`Update`
                    (if (`/Game/Blueprints/BP_Bomb.IsBombHeld?` (`self.BombRef`))
                      (goto _label_2 :!via `Stop`)
                      (else
                        (`SceneComponent.K2_SetWorldLocation` (`/Game/Blueprints/BP_Bomb.BombMesh` (`self.BombRef`)) (`KismetMathLibrary.MakeVector` _returnvalue_x _returnvalue_y (`KismetMathLibrary.Lerp` (+ _returnvalue_z (`self.HoverHeight`)) _returnvalue_z_2 _zoffset)) false false)))))))))))))

(event `BombMachineHover`
  (bind _bombmachinetransform (`self.BombMachineTransform`))
  (bind _slackstartloc (`self.SlackStartLoc`))
  ;[1 0.7595 0 0.295] Move bomb machine and spline cable to active position
  (set `self.BombMachineTransform` (`SceneComponent.GetRelativeTransform` (`self.SM_BombMachineCasing`)))
  (set `self.SlackStartLoc` (`SceneComponent.K2_GetComponentLocation` (`self.WireSlackLoc`)))
  (bind (_direction _lerptransforms _emissiveglowonbombmachine) (`Timeline|MachineHover` :!via `PlayFromStart`)
    (:`Update`
      (`SceneComponent.K2_SetWorldLocation` (`self.WireSlackLoc`) (`KismetMathLibrary.VLerp` _slackstartloc (+ _slackstartloc (0.0 -1.0 1.0)) _lerptransforms) false false)
      (`SceneComponent.K2_SetRelativeTransform` (`self.SM_BombMachineCasing`) (`KismetMathLibrary.TLerp` (`self.BombMachineTransform`) (`KismetMathLibrary.MakeTransform` (+ (.location _bombmachinetransform) (0.0 0.0 3.0)) (`KismetMathLibrary.MakeRotator` 0.0 0.0 (- (.yaw (.rotation _bombmachinetransform)) 25.0)) (.scale _bombmachinetransform)) _lerptransforms) false false)
      (`self.UpdateSpline`)
      (`MaterialInstanceDynamic.SetScalarParameterValue` (`self.BombMachineMat`) "EmissiveIntensity" _emissiveglowonbombmachine))
    (:`Finished`
      (set `self.BombMachineReady` true)
      (set `self.Active` true))))

(fn `CreateSpline`
  (bind _wire (`self.Wire`))
  (bind _wirescale (`self.WireScale`))
  (bind _wire_2 (`self.Wire`))
  (bind _wire_3 (`self.Wire`))
  (bind _returnvalue (`KismetMathLibrary.MakeVector2D` _wirescale _wirescale))
  (bind _returnvalue_2 (+ (`self.InnerSpinePoints`) 1))
  ;[0 0.03576 0.3177 0.546] Divide spline into even segments and setup array
  (set `self.DistanceOfInbetweenPoints` (/ (`SplineComponent.GetSplineLength` _wire_2) (`KismetMathLibrary.Conv_IntToDouble` _returnvalue_2)))
  (for _index (range (+ _returnvalue_2 1))
    (bind _output_get (set `self.SplineArrayIndex` _index))
    (bind _returnvalue_3 (* _output_get (`self.DistanceOfInbetweenPoints`)))
    (`KismetArrayLibrary.Array_Set` (`self.SplinePointLocation`) (`self.SplineArrayIndex`) (make `/Game/Blueprints/Structs/SplineAttributes` (`SplineComponent.GetLocationAtDistanceAlongSpline` _wire_2 _returnvalue_3 "Local") (`SplineComponent.GetTangentAtDistanceAlongSpline` _wire_2 _returnvalue_3 "Local")) true))
  ;[0.05725 0 1 0.204] Set points along spline based on distance
  (`SplineComponent.ClearSplinePoints` _wire_3 true)
  (for _index_2 (range (+ (+ (`self.InnerSpinePoints`) 1) 1))
    (bind (_pointlocation _pointtangent) (break `/Game/Blueprints/Structs/SplineAttributes` (`|GetArrayItem` (`self.SplinePointLocation`) _index_2)))
    (`SplineComponent.AddSplinePoint` _wire_3 _pointlocation "Local" true)
    (`SplineComponent.SetTangentAtSplinePoint` _wire_3 _index_2 _pointtangent "Local" true)
    (`SplineComponent.SetSplinePointType` _wire_3 _index_2 "Curve" true))
  ;[0.625 0.3255 0 0.235] Set static mesh to start and end of spline points
  (for _index_3 (range (+ (- (`SplineComponent.GetNumberOfSplinePoints` _wire) 2) 1))
    (bind _returnvalue_4 (`AddComponent|NODE_AddSplineMeshComponent-2` :`RelativeTransform` (`SceneComponent.GetRelativeTransform` _wire)))
    (`KismetArrayLibrary.Array_Set` (`self.SplineMeshes`) _index_3 _returnvalue_4 true)
    (bind (_location _tangent) (`SplineComponent.GetLocationAndTangentAtSplinePoint` _wire _index_3 "Local"))
    (bind (_location_2 _tangent_2) (`SplineComponent.GetLocationAndTangentAtSplinePoint` _wire (+ _index_3 1) "Local"))
    (`SplineMeshComponent.SetStartAndEnd` _returnvalue_4 _location _tangent _location_2 _tangent_2 true)
    (`SplineMeshComponent.SetStartScale` _returnvalue_4 _returnvalue true)
    (`SplineMeshComponent.SetEndScale` _returnvalue_4 _returnvalue true)))

(fn `UpdateSpline`
  (bind _wire (`self.Wire`))
  (bind _wire_2 (`self.Wire`))
  ;[1 0.8224 0 0.42] Reset spline points to current handle location
  (`SplineComponent.SetLocationAtSplinePoint` _wire 0 (`SceneComponent.K2_GetComponentLocation` (`self.WireEndLoc2`)) "World" true)
  (`SplineComponent.SetLocationAtSplinePoint` _wire 1 (`SceneComponent.K2_GetComponentLocation` (`self.WireEndLoc1`)) "World" true)
  (`SplineComponent.SetLocationAtSplinePoint` _wire 2 (`SceneComponent.K2_GetComponentLocation` (`self.WireSlackLoc`)) "World" true)
  (`SplineComponent.SetLocationAtSplinePoint` _wire 3 (`SceneComponent.K2_GetComponentLocation` (`self.WireStartLoc1`)) "World" true)
  (`SplineComponent.SetLocationAtSplinePoint` _wire 4 (`SceneComponent.K2_GetComponentLocation` (`self.WireStartLoc2`)) "World" true)
  ;[0.8815 1 0 0.389] Set Mesh location to spline location/tangent
  (for (_array_element _array_index) (`self.SplineMeshes`)
    (bind (_location _tangent) (`SplineComponent.GetLocationAndTangentAtSplinePoint` _wire_2 _array_index "Local"))
    (bind (_location_2 _tangent_2) (`SplineComponent.GetLocationAndTangentAtSplinePoint` _wire_2 (+ _array_index 1) "Local"))
    (`SplineMeshComponent.SetStartAndEnd` _array_element _location _tangent _location_2 _tangent_2 true)))

(fn `UserConstructionScript`
  ;[0.1406 0.1406 0.1406 0.666] UpdateSpline on start
  (`self.CreateSpline`)
  (`self.UpdateSpline`)
  ;[0.04746 0.7892 1 0.384] Set material for bomb machine
  (bind _returnvalue (`PrimitiveComponent.CreateDynamicMaterialInstance` (`self.SM_BombMachineCasing`) 0 null "None"))
  (set `self.BombMachineMat` _returnvalue))