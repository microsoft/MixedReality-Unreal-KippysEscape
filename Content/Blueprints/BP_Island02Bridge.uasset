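; Island 02 bridge actor that folds out one segment at a time when ExtendBridge is called.
; The construction script chains the segment meshes by socket, so each rotates with its parent.
; ExtendBridge immediately updates four front BP_Ballast posts and, after a short delay, starts the unfold.
; One reused timeline lerps the current segment's rotation, revealing segments progressively and playing sounds after each step until HasExtended is set.
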(event `Unfold`
  (bind _returnvalue (`KismetMathLibrary.MakeRotator` 0.0 -180.0))
  (bind _returnvalue_2 (`KismetMathLibrary.MakeRotator` -180.0 -180.0 180.0))
  (bind _returnvalue_3 (`KismetMathLibrary.MakeRotator` -180.0 0.0 180.0))
  (bind _sm_bridge_segment1 (`self.SM_Bridge_segment1`))
  (bind _currentindex (`self.currentIndex`))
  ;[1 1 1] Extend Bridge Logic
  (if (<= (`self.currentIndex`) 5) :!label _label
    (`SceneComponent.SetVisibility` (select `int` (`self.currentIndex`) :`0` _sm_bridge_segment1 :`1` (`self.SM_Bridge_segment2`) :`2` (`self.SM_Bridge_segment3`) :`3` (`self.SM_Bridge_segment4`) :`4` (`self.SM_Bridge_segment5`) :`5` _sm_bridge_segment1) true false)
    (bind (_direction _lerp) (`Timeline|UnfoldAnimation` :!via `PlayFromStart`)
      (:`Update`
        (`SceneComponent.K2_SetRelativeRotation` (select `int` (`self.currentIndex`) :`0` (`self.SM_Bridge_segment0`) :`1` (`self.SM_Bridge_segment1`) :`2` (`self.SM_Bridge_segment2`) :`3` (`self.SM_Bridge_segment3`) :`4` (`self.SM_Bridge_segment4`) :`5` (`self.SM_Bridge_segment5`)) (`KismetMathLibrary.RLerp` (select `int` _currentindex :`0` (struct :`Pitch` -90.0 :`Yaw` 180.0) :`1` _returnvalue_3 :`2` _returnvalue :`3` _returnvalue_3 :`4` _returnvalue :`5` _returnvalue_3) (select `int` _currentindex :`0` (struct :`Pitch` 30.5 :`Yaw` 180.0) :`1` _returnvalue_2 :`2` (struct) :`3` _returnvalue_2 :`4` (struct) :`5` _returnvalue_2) _lerp) false false))
      (:`Finished`
        (`/Engine/EditorBlueprintResources/StandardMacros.IncrementInt` (`self.currentIndex`)
          (:`  `
            (`self.Unfold`)
            (`AudioComponent.Play` (`self.96136__bmaczero__clink3`) 0.0)
            (`AudioComponent.Play` (`self.GDC2020_Demo_Bridge_Section_Last`) 0.0)))))
    (else
      (set `self.HasExtended` true))))

(event `ExtendBridge`
  ;[1 1 1] Extend Bridge Logic
  (`|ExecutionSequence`
    (:`then_0`
      (`KismetSystemLibrary.Delay` 0.5)
      (`TimelineComponent.SetPlayRate` (`self.UnfoldAnimation`) 2.0)
      (goto _label))
    (:`then_1`
      ;;[1 1 1] activate posts
      (bind _asbp_ballast (cast `/Game/Blueprints/newBridge/BP_Ballast` (`ChildActorComponent.ChildActor` (`self.Post_Front_1L`))))
      (`/Game/Blueprints/newBridge/BP_Ballast.UpdateState` _asbp_ballast "NewEnumerator0")
      (bind _asbp_ballast_2 (cast `/Game/Blueprints/newBridge/BP_Ballast` (`ChildActorComponent.ChildActor` (`self.Post_Front_1R`))))
      (`/Game/Blueprints/newBridge/BP_Ballast.UpdateState` _asbp_ballast_2 "NewEnumerator0")
      (bind _asbp_ballast_3 (cast `/Game/Blueprints/newBridge/BP_Ballast` (`ChildActorComponent.ChildActor` (`self.Post_Front_2L`))))
      (`/Game/Blueprints/newBridge/BP_Ballast.UpdateState` _asbp_ballast_3 "NewEnumerator0")
      (bind _asbp_ballast_4 (cast `/Game/Blueprints/newBridge/BP_Ballast` (`ChildActorComponent.ChildActor` (`self.Post_Front_2R`))))
      (`/Game/Blueprints/newBridge/BP_Ballast.UpdateState` _asbp_ballast_4 "NewEnumerator0"))))

(fn `UserConstructionScript`
  (bind _sm_bridge_segment1 (`self.SM_Bridge_segment1`))
  (bind _sm_bridge_segment2 (`self.SM_Bridge_segment2`))
  (bind _sm_bridge_segment4 (`self.SM_Bridge_segment4`))
  (bind _sm_bridge_segment3 (`self.SM_Bridge_segment3`))
  (`SceneComponent.K2_AttachToComponent` _sm_bridge_segment1 (`self.SM_Bridge_segment0`) "friend" "KeepRelative" "KeepRelative" "SnapToTarget" true)
  (`SceneComponent.K2_AttachToComponent` _sm_bridge_segment2 _sm_bridge_segment1 "friend" "KeepRelative" "KeepRelative" "SnapToTarget" true)
  (`SceneComponent.K2_AttachToComponent` _sm_bridge_segment3 _sm_bridge_segment2 "friend" "KeepRelative" "KeepRelative" "SnapToTarget" true)
  (`SceneComponent.K2_AttachToComponent` _sm_bridge_segment4 _sm_bridge_segment3 "friend" "KeepRelative" "KeepRelative" "SnapToTarget" true)
  (`SceneComponent.K2_AttachToComponent` (`self.SM_Bridge_segment5`) _sm_bridge_segment4 "friend" "KeepRelative" "KeepRelative" "SnapToTarget" true))