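; Camera-facing circle effect for interactive objects that signals hand proximity, gaze and grab state in an Unreal UXTools (UXT) scene.
; Each tick it measures left index-tip distance and picks Off, Active or Grabbing, using IsGrabbed and IsLookedAt flags set outside this file.
; The state shrinks or grows the plane, with distance driving the dynamic material's waving and filling plus overall scale; grabbing fixes them.
; Debug prints remain active.
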(event `self.ReceiveBeginPlay`
  ;[1 0 0] This only get 1 interactor - will this be an issue?
  ;;[1 1 1] Get hands
  (bind _returnvalue (`GameplayStatics.GetActorOfClass` "/Script/UXToolsInputSimulation.UxtInputSimulationActor"))
  (set `self.hands` _returnvalue))

(event `self.ReceiveTick`
  (params (DeltaSeconds :type "Float (single-precision)"))
  (bind _dynamicmaterial (`self.dynamicMaterial`))
  (bind _dynamicmaterial_2 (`self.dynamicMaterial`))
  (bind _generalscale (`self.generalScale`))
  (bind _returnvalue (- 1.0 (`KismetMathLibrary.MapRangeClamped` (`self.closerHandDistance`) 3.0 20.0 0.0 1.0)))
  (`|ExecutionSequence`
    (:`then_0`
      ;[1 1 1] Comment
      (`self.K2_SetActorRotation` (`KismetMathLibrary.FindLookAtRotation` (`self.K2_GetActorLocation`) (`self.K2_GetActorLocation` (`GameplayStatics.GetPlayerCameraManager` 0)))))
    (:`then_1`
      (bind (_outorientation _outposition) (`UxtHandTrackingFunctionLibrary.GetHandJointState` "Left" "IndexTip"))
      (bind _output_get (set `self.closerHandDistance` (`KismetMathLibrary.FClamp` (`KismetMathLibrary.Vector_Distance` _outposition (`SceneComponent.K2_GetComponentLocation` (`self.DefaultSceneRoot`))) 3.0 20.0)))
      (`KismetSystemLibrary.PrintString` (`KismetStringLibrary.Conv_DoubleToString` _output_get) true true (struct :`G` 0.66 :`B` 1.0 :`A` 1.0) 0.0))
    (:`then_2`
      (`|ExecutionSequence`
        (:`then_0`
          (if (< (`self.closerHandDistance`) 20.0)
            (set `self.handIsClose` true)
            (else
              (set `self.handIsClose` false))))
        (:`then_1`
          (if (`self.isGrabbed`)
            (set `self.effectState` "NewEnumerator4")
            (elif (or (`self.isLookedAt`) (`self.handIsClose`))
              (set `self.effectState` "NewEnumerator1")
              (else
                (set `self.effectState` "NewEnumerator0")))))))
    (:`then_3`
      ;[1 1 1] Comment
      (`KismetSystemLibrary.PrintString` (`|GetEnumeratorNameAsString` (`self.effectState`)) true true (struct :`G` 0.158961 :`B` 0.130136 :`A` 1.0) 0.0)
      (switch `/Game/Blueprints/Enums/E_InteractiveObjectsState` (`self.effectState`)
        (:`NewEnumerator0`
          (`SceneComponent.SetRelativeScale3D` (`self.SM_PlaneInteractiveObjects`) (`KismetMathLibrary.VInterpTo` (`SceneComponent.RelativeScale3D` (`self.SM_PlaneInteractiveObjects`)) (0.0 0.0 0.0) (`GameplayStatics.GetWorldDeltaSeconds`) (`self.interpSpeed`))))
        (:`NewEnumerator1`
          (`SceneComponent.SetRelativeScale3D` (`self.SM_PlaneInteractiveObjects`) (`KismetMathLibrary.VInterpTo` (`SceneComponent.RelativeScale3D` (`self.SM_PlaneInteractiveObjects`)) (1.0 1.0 1.0) (`GameplayStatics.GetWorldDeltaSeconds`) (`self.interpSpeed`)))
          (`MaterialInstanceDynamic.SetScalarParameterValue` _dynamicmaterial_2 "waving" _returnvalue)
          (`MaterialInstanceDynamic.SetScalarParameterValue` _dynamicmaterial_2 "filling" _returnvalue)
          (`SceneComponent.SetRelativeScale3D` (`self.scene_generalScale`) (`KismetMathLibrary.VLerp` _generalscale (* _generalscale 1.25) _returnvalue)))
        (:`NewEnumerator4`
          (`MaterialInstanceDynamic.SetScalarParameterValue` _dynamicmaterial "waving" 0.0)
          (`MaterialInstanceDynamic.SetScalarParameterValue` _dynamicmaterial "filling" 1.0)
          (`SceneComponent.SetRelativeScale3D` (`self.scene_generalScale`) (`self.generalScale`)))))))

(fn `IsGrabFocusable`
  (params (Primitive :type "PrimitiveComponent Object Reference"))
  (returns (ReturnValue :type Boolean))
  (return false))

(fn `UserConstructionScript`
  (`|ExecutionSequence`
    (:`then_0`
      (`SceneComponent.SetRelativeScale3D` (`self.scene_generalScale`) (`self.generalScale`)))
    (:`then_1`
      (bind _returnvalue (`PrimitiveComponent.CreateDynamicMaterialInstance` (`self.SM_PlaneInteractiveObjects`) 0 "/Game/Effects/ObjectInteraction/M_ObjectInteraction.M_ObjectInteraction" "None"))
      (set `self.dynamicMaterial` _returnvalue))))