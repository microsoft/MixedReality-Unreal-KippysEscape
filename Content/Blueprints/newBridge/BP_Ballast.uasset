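; BP_Ballast is a bridge ballast block with On, Flicker and Off states that drive its emissive colour and motion.
; UpdateState switches the dynamic material colour or runs a looping timer that randomly flickers it.
; Tick bobs the block when On, jitters it in Flicker, and slowly sinks and tilts it when Off.
; In On or Flicker, UXT grab focus triggers a rate-limited timeline wobble away from the closer hand, then back.
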(event `UpdateState`
  (params (newState :type "/Game/Blueprints/newBridge/E_BallastState Enum" :default "NewEnumerator0"))
  ;[1 1 1] udate State
  (set `self.ballastState` newState)
  (switch `/Game/Blueprints/newBridge/E_BallastState` newState
    (:`NewEnumerator0`
      (`self.StopFlickering`)
      (`MaterialInstanceDynamic.SetVectorParameterValue` (`self.materialInstance`) "Emissive" (`self.colourON`)))
    (:`NewEnumerator1`
      (`self.StartFlickering`))
    (:`NewEnumerator2`
      (`self.StopFlickering`)
      (`MaterialInstanceDynamic.SetVectorParameterValue` (`self.materialInstance`) "Emissive" (`self.colourOFF`)))))

(event `StartFlickering`
  ;[1 1 1] Flickering
  (`KismetSystemLibrary.K2_SetTimer` null "Flicker" 0.1 true))

(event `self.ReceiveBeginPlay`
  (`|ExecutionSequence`
    (:`then_0`
      (set `self.initialLocationInteraction` (`SceneComponent.K2_GetComponentLocation` (`self.InteractionMotion`))))
    (:`then_1`
      ;[1 1 1] idle anim value
      (`TimelineComponent.SetPlayRate` (`self.IdleAnimation`) 0.5)
      (bind (_direction _lerpz) (`Timeline|IdleAnimation` :!via `PlayFromStart`)
        (:`Update`
          (set `self.idleLocation` (`KismetMathLibrary.MakeVector` 0.0 0.0 (`KismetMathLibrary.Lerp` -0.5 0.5 _lerpz))))))))

(event `StopFlickering`
  ;[1 1 1] Flickering
  (`KismetSystemLibrary.K2_PauseTimer` null "Flicker")
  (`KismetSystemLibrary.K2_ClearTimer` null "Flicker"))

(event `self.ReceiveTick`
  (params (DeltaSeconds :type "Float (single-precision)"))
  (bind _idlemotion (`self.IdleMotion`))
  (bind _idlemotion_2 (`self.IdleMotion`))
  (bind _jitteramount (`self.jitterAmount`))
  (bind _returnvalue (* _jitteramount -1.0))
  ;[1 1 1] Animation
  (switch `/Game/Blueprints/newBridge/E_BallastState` (`self.ballastState`)
    (:`NewEnumerator0`
      ;;[1 1 1] OFF state
      (`SceneComponent.K2_SetRelativeLocation` _idlemotion_2 (`KismetMathLibrary.VInterpTo` (`SceneComponent.RelativeLocation` _idlemotion_2) (`self.idleLocation`) (`GameplayStatics.GetWorldDeltaSeconds`) 5.0) false false)
      (`SceneComponent.K2_SetRelativeRotation` _idlemotion_2 (`KismetMathLibrary.RInterpTo` (`SceneComponent.RelativeRotation` _idlemotion_2) (struct) (`GameplayStatics.GetWorldDeltaSeconds`) 5.0) false false))
    (:`NewEnumerator1`
      ;;[1 1 1] Jitter State
      (if (== (`self.newJitterLocation`) (`SceneComponent.RelativeLocation` (`self.Ballast`)) :`ErrorTolerance` 0.001)
        ;;;[1 1 1] set new values
        (set `self.newJitterLocation` (`KismetMathLibrary.MakeVector` (`KismetMathLibrary.RandomFloatInRange` _returnvalue _jitteramount) (`KismetMathLibrary.RandomFloatInRange` _returnvalue _jitteramount) (`KismetMathLibrary.RandomFloatInRange` _returnvalue _jitteramount)))
        (set `self.jitterInterpSpeed` (`KismetMathLibrary.RandomFloatInRange` 1.0 2.0))
        (else
          (`SceneComponent.K2_SetRelativeLocation` (`self.Ballast`) (`KismetMathLibrary.VInterpTo_Constant` (`SceneComponent.RelativeLocation` (`self.Ballast`)) (`self.newJitterLocation`) (`GameplayStatics.GetWorldDeltaSeconds`) (`self.jitterInterpSpeed`)) false false))))
    (:`NewEnumerator2`
      ;;[1 1 1] ON state
      (`SceneComponent.K2_SetRelativeLocation` _idlemotion (`KismetMathLibrary.VInterpTo` (`SceneComponent.RelativeLocation` _idlemotion) (0.0 0.0 -1.0) (`GameplayStatics.GetWorldDeltaSeconds`) 0.5) false false)
      (`SceneComponent.K2_SetRelativeRotation` _idlemotion (`KismetMathLibrary.RInterpTo` (`SceneComponent.RelativeRotation` _idlemotion) (`KismetMathLibrary.SelectRotator` (struct :`Pitch` 10.0 :`Roll` 20.0) (struct :`Pitch` -10.0 :`Roll` 20.0) (`self.endIsland`)) (`GameplayStatics.GetWorldDeltaSeconds`) 0.5) false false))))

(event `self.UxtGrabTarget.OnEnterGrabFocus`
  (params (Grabbable :type "UxtGrabTargetComponent Object Reference") (Pointer :type "UxtNearPointerComponent Object Reference"))
  (bind _locationpriorwobble (`self.locationPriorWobble`))
  (bind _returnvalue (`SceneComponent.K2_GetComponentLocation` (`self.InteractionMotion`)))
  (bind _returnvalue_2 (`SceneComponent.K2_GetComponentLocation` (`self.InteractionMotion`)))
  (bind _returnvalue_3 (+ _locationpriorwobble (* (* (`KismetMathLibrary.Normal` (`self.wobbleDirection`)) -1.0) (`self.wobbleAmount`))))
  ;[1 1 1] Hands interaction
  (switch `/Game/Blueprints/newBridge/E_BallastState` (`self.ballastState`)
    (:`NewEnumerator0`
      _)
    (:`NewEnumerator1`
      _))
  ;;[1 1 1] lets timeline finish when you trigger the wobble 5 times in a row
  (if (`self.canWobble`)
    (set `self.interactionsCounter` (+ (`self.interactionsCounter`) 1))
    (if (!= (`self.interactionsCounter`) 4)
      (set `self.canWobble` false) ; decreases interaction frequency allowed
      (`KismetSystemLibrary.Delay` 0.33)
      (set `self.canWobble` true)
      (else
        (set `self.canWobble` false) ; allows interaction logic to reset
      ))
    (`|ExecutionSequence`
      (:`then_0`
        ;;[1 1 1] gets distance of the closer hand
        (bind (_outorientation _outposition) (`UxtHandTrackingFunctionLibrary.GetHandJointState` "Left" "IndexIntermediate"))
        (bind (_outorientation_2 _outposition_2) (`UxtHandTrackingFunctionLibrary.GetHandJointState` "Right" "IndexIntermediate"))
        (set `self.leftHandCloser` (< (`KismetMathLibrary.Vector_Distance` _outposition _returnvalue_2) (`KismetMathLibrary.Vector_Distance` _outposition_2 _returnvalue_2))))
      (:`then_1`
        ;;[1 1 1] sets variables needed
        ;;;[1 1 1] calculates direction
        (if (`self.leftHandCloser`)
          (bind (_outorientation_3 _outposition_3) (`UxtHandTrackingFunctionLibrary.GetHandJointState` "Left" "IndexTip"))
          (set `self.wobbleDirection` (`KismetMathLibrary.GetDirectionUnitVector` _returnvalue _outposition_3))
          (else
            (bind (_outorientation_4 _outposition_4) (`UxtHandTrackingFunctionLibrary.GetHandJointState` "Right" "IndexTip"))
            (set `self.wobbleDirection` (`KismetMathLibrary.GetDirectionUnitVector` _returnvalue _outposition_4))))
        (set `self.locationPriorWobble` (`SceneComponent.K2_GetComponentLocation` (`self.InteractionMotion`)))
        (set `self.wobbleAmount` (`KismetMathLibrary.RandomFloatInRange` 0.25 0.5))
        (set `self.goBackToOriginalLoc` false))
      (:`then_2`
        ;;[1 1 1] Animates block
        (bind (_direction _lerp) (`Timeline|Timeline_0` :!via `PlayFromStart`)
          (:`Update`
            (`SceneComponent.K2_SetWorldLocation` (`self.InteractionMotion`) (`KismetMathLibrary.SelectVector` (`KismetMathLibrary.VLerp` (`self.initialLocationInteraction`) _returnvalue_3 _lerp) (`KismetMathLibrary.VLerp` _locationpriorwobble _returnvalue_3 _lerp) (`self.goBackToOriginalLoc`)) false false))
          (:`Finished`
            ;;[1 1 1] reset
            (set `self.canWobble` true)
            (set `self.interactionsCounter` 0))
          (:`pushCompletedEvent`
            (set `self.goBackToOriginalLoc` true)))))))

(fn `Flicker`
  (locals (OnOff :type Boolean))
  (set `local.OnOff` (`KismetMathLibrary.RandomBool`))
  (`MaterialInstanceDynamic.SetVectorParameterValue` (`self.materialInstance`) "Emissive" (`KismetMathLibrary.SelectColor` (`self.colourON`) (`self.colourOFF`) (`local.OnOff`))))

(fn `UserConstructionScript`
  (bind _returnvalue (`KismetMaterialLibrary.CreateDynamicMaterialInstance` "/Game/Art/Bridge/M_BridgePost.M_BridgePost"))
  (set `self.materialInstance` _returnvalue)
  (`PrimitiveComponent.SetMaterial` (`self.Ballast`) 0 (`self.materialInstance`))
  (`self.UpdateState` (`self.initialState`)))