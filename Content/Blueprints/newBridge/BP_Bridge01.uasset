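; Holographic bridge puzzle that forms when the player's hanging cable plug reaches its receiver.
; Until triggered, a looping timer sparks and wiggles the cable; InitialSequence then releases the plug and updates the ballasts, while gaze twitches the back cable.
; On overlap, chained timelines snap the plug in, tighten cables, sweep beams and reveal the bridge through a dynamic material's BridgeReveal parameter, setting PlugInserted and Extended for a state machine.
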(event `self.ReceiveBeginPlay`
  (`self.SetupInitialSequence`))

(event `SetupInitialSequence`
  (bind (_receiversetupwrot_roll _receiversetupwrot_pitch _receiversetupwrot_yaw) (`KismetMathLibrary.BreakRotator` (`self.receiverSetupWRot`)))
  (bind _hangingcable (`self.hangingCable`))
  (bind _hangingcable_2 (`self.hangingCable`))
  ;[1 1 1] InitialSequence
  ;;[1 1 1] Setup
  (`|ExecutionSequence`
    (:`then_0`
      (`|ExecutionSequence`
        (:`then_0`
          (`/Game/Blueprints/newBridge/BP_HangingCable.ActivateDeactivatePlug` _hangingcable false)
          (`/Game/Blueprints/newBridge/BP_HangingCable.ChangeHeldState` _hangingcable true))
        (:`then_1`
          (`SceneComponent.K2_SetWorldLocation` (`Actor.RootComponent` (`ChildActorComponent.ChildActor` (`/Game/Blueprints/newBridge/BP_HangingCable.pickupable` _hangingcable_2))) (- (`self.receiverLandingWLoc`) (0.0 -0.5 0.8)) false false)
          (`SceneComponent.K2_SetWorldLocation` (`/Game/Blueprints/newBridge/BP_HangingCable.dummyRoot` _hangingcable_2) (- (`self.receiverLandingWLoc`) (0.0 -0.5 0.8)) false false)
          (`SceneComponent.K2_SetWorldLocation` (`/Game/Blueprints/newBridge/BP_HangingCable.attachmentEnd` _hangingcable_2) (- (`self.receiverLandingWLoc`) (0.0 -0.5 0.8)) false false)
          (`SceneComponent.K2_SetWorldRotation` (`/Game/Blueprints/newBridge/BP_HangingCable.dummyRoot` _hangingcable_2) (`KismetMathLibrary.MakeRotator` _receiversetupwrot_roll (+ _receiversetupwrot_pitch 20.0) _receiversetupwrot_yaw) false false)
          (`SceneComponent.K2_SetRelativeRotation` (`/Game/Blueprints/newBridge/BP_HangingCable.plugDummy` _hangingcable_2) (struct :`Yaw` -90.0 :`Roll` -90.0) false false))
        (:`then_2`
          (set `CableComponent.CableLength` 20.0 (`/Game/Blueprints/newBridge/BP_HangingCable.Cable` (`self.hangingCable`)))
          (`KismetSystemLibrary.Delay` 2.0)
          (`KismetSystemLibrary.K2_SetTimer` null "WiggleFrontCable" 4.0 true))))
    (:`then_1`
      (`MaterialInstanceDynamic.SetScalarParameterValue` (`self.holoBridge`) "Flicker" 1.0)
      ;;;[1 1 1] Ballasts
      (bind _asbp_ballast (cast `/Game/Blueprints/newBridge/BP_Ballast` (`ChildActorComponent.ChildActor` (`self.Ballast_Front1`))))
      (`/Game/Blueprints/newBridge/BP_Ballast.UpdateState` _asbp_ballast "NewEnumerator1")
      (bind _asbp_ballast_2 (cast `/Game/Blueprints/newBridge/BP_Ballast` (`ChildActorComponent.ChildActor` (`self.Ballast_Front2`))))
      (`/Game/Blueprints/newBridge/BP_Ballast.UpdateState` _asbp_ballast_2 "NewEnumerator1"))))

(event `WiggleFrontCable`
  (bind _frontbeam (`self.frontBeam`))
  (bind (_returnvalue_x _returnvalue_y _returnvalue_z) (`KismetMathLibrary.BreakVector` (- (`self.receiverLandingWLoc`) (0.0 -0.6 0.8))))
  (bind _cable (`/Game/Blueprints/newBridge/BP_HangingCable.Cable` (`self.hangingCable`)))
  ;[1 1 1] InitialSequence
  ;;[1 1 1] Setup
  ;;;[0.1804 0.6471 1] Wiggle front cable
  ;;;;[1 1 1] beam fx
  (`ActorComponent.Activate` _frontbeam false)
  (`self.SetBeamParameters` _frontbeam (- (`SceneComponent.K2_GetComponentLocation` (`self.Plug_1`)) (-8.8 0.0 0.0)) (- (`SceneComponent.K2_GetComponentLocation` (`self.Plug_2`)) (-8.8 0.0 0.0)) (struct :`G` 1.0 :`B` 1.0 :`A` 1.0) 10.0)
  (`KismetSystemLibrary.Delay` 0.2)
  (`ActorComponent.Deactivate` _frontbeam)
  (`KismetSystemLibrary.Delay` 0.5)
  (`|ExecutionSequence`
    (:`then_0`
      (set `CableComponent.bEnableStiffness` false _cable)
      (`KismetSystemLibrary.Delay` 0.15)
      (set `CableComponent.bEnableStiffness` true _cable))
    (:`then_1`
      (`GameplayStatics.PlaySoundAtLocation` "/Game/Sounds/Bridge01/SC_LargeSpark.SC_LargeSpark" (`SceneComponent.K2_GetComponentLocation` (`self.Sparks`)) (struct) 1.0 1.0 0.0 "/Game/Sounds/DefaultAttenuationSettings.DefaultAttenuationSettings" null null)
      (`ActorComponent.Activate` (`self.Sparks`) true)
      (bind (_direction _offset) (`Timeline|WigglePlug` :!via `PlayFromStart`)
        (:`Update`
          (`SceneComponent.K2_SetWorldLocation` (`/Game/Blueprints/newBridge/BP_HangingCable.dummyRoot` (`self.hangingCable`)) (`KismetMathLibrary.MakeVector` _returnvalue_x (+ _returnvalue_y (* _offset 0.5)) (- _returnvalue_z _offset)) false false))))))

(event `InitialSequence`
  (bind _hangingcable (`self.hangingCable`))
  ;[1 1 1] InitialSequence
  ;;[1 1 1] Trigger
  (`KismetSystemLibrary.K2_PauseTimer` null "WiggleFrontCable")
  (`KismetSystemLibrary.K2_ClearTimer` null "WiggleFrontCable")
  (`self.WiggleFrontCable`)
  (`KismetSystemLibrary.Delay` 1.6)
  (`|ExecutionSequence`
    (:`then_0`
      ;;;[1 1 1] Ballasts
      (bind _asbp_ballast (cast `/Game/Blueprints/newBridge/BP_Ballast` (`ChildActorComponent.ChildActor` (`self.Ballast_Front1`))))
      (`/Game/Blueprints/newBridge/BP_Ballast.StopFlickering` _asbp_ballast)
      (`/Game/Blueprints/newBridge/BP_Ballast.UpdateState` _asbp_ballast "NewEnumerator2")
      (bind _asbp_ballast_2 (cast `/Game/Blueprints/newBridge/BP_Ballast` (`ChildActorComponent.ChildActor` (`self.Ballast_Front2`))))
      (`/Game/Blueprints/newBridge/BP_Ballast.StopFlickering` _asbp_ballast_2)
      (`/Game/Blueprints/newBridge/BP_Ballast.UpdateState` _asbp_ballast_2 "NewEnumerator2"))
    (:`then_1`
      ;;;[1 1 1] HangingCable
      (`/Game/Blueprints/newBridge/BP_HangingCable.ActivateDeactivatePlug` _hangingcable true)
      (`/Game/Blueprints/newBridge/BP_HangingCable.ChangeHeldState` _hangingcable false)
      (set `CableComponent.CableLength` 17.0 (`/Game/Blueprints/newBridge/BP_HangingCable.Cable` (`self.hangingCable`)))
      (`MaterialInstanceDynamic.SetScalarParameterValue` (`self.holoBridge`) "Flicker" 0.0))
    (:`then_2`
      ;;;[1 1 1] Self
      (`ParticleSystemComponent.SetTemplate` (`self.Sparks`) "/Game/Explosions/Particles/P_ElecticalSparksIdle.P_ElecticalSparksIdle"))))

(event `self.plugOverlap.OnComponentBeginOverlap`
  (params (OverlappedComponent :type "PrimitiveComponent Object Reference") (OtherActor :type "Actor Object Reference") (OtherComp :type "PrimitiveComponent Object Reference") (OtherBodyIndex :type Integer) (bFromSweep :type Boolean) (SweepResult :type "HitResult Structure (by ref)"))
  (bind _hangingcable (`self.hangingCable`))
  (bind _hangingcable_2 (`self.hangingCable`))
  (bind _bridgingbeam (`self.bridgingBeam`))
  (bind _returnvalue (`SceneComponent.K2_GetComponentLocation` (`self.Plug_1`)))
  (bind _returnvalue_2 (`SceneComponent.K2_GetComponentLocation` (`self.Plug_2`)))
  (bind _dummyroot (`/Game/Blueprints/newBridge/BP_HangingCable.dummyRoot` _hangingcable_2))
  (bind _dummyroot_2 (`/Game/Blueprints/newBridge/BP_HangingCable.dummyRoot` _hangingcable))
  ;[1 1 1] Building Sequence
  (if (`self.Active`)
    (if (== OtherActor (`ChildActorComponent.ChildActor` (`/Game/Blueprints/newBridge/BP_HangingCable.pickupable` (`self.hangingCable`))))
      (`|ExecutionSequence`
        (:`then_0`
          (`/Game/Blueprints/newBridge/BP_HangingCable.ActivateDeactivatePlug` _hangingcable false)
          (set `self.canWiggleGaze` false)
          (`ActorComponent.Deactivate` (`self.backBeam`))
          (`GameplayStatics.PlaySoundAtLocation` "/Game/Sounds/Bridge01/KippysEscape_Bridge_Activation_Cue.KippysEscape_Bridge_Activation_Cue" (`SceneComponent.K2_GetComponentLocation` (`self.plugOverlap`)) (struct) 1.0 1.0 0.0 "/Game/Sounds/DefaultAttenuationSettings.DefaultAttenuationSettings" null null))
        (:`then_1`
          ;;[1 1 1] Plug Setup
          (set `self.receiverArrivingWLoc` (`SceneComponent.K2_GetComponentLocation` _dummyroot_2))
          (set `self.receiverArrivingWRot` (`SceneComponent.K2_GetComponentRotation` _dummyroot_2))
          (set `self.receiverArrivingRrot` (`SceneComponent.RelativeRotation` (`/Game/Blueprints/newBridge/BP_HangingCable.plugDummy` (`self.hangingCable`))))
          (bind (_direction _lineup _insert _directinsert) (`Timeline|plugSetup` :!via `PlayFromStart`)
            (:`Update`
              (`SceneComponent.K2_SetWorldLocation` _dummyroot (`KismetMathLibrary.VLerp` (`self.receiverArrivingWLoc`) (`self.receiverLandingWLoc`) _directinsert) false false)
              (`SceneComponent.K2_SetWorldRotation` _dummyroot (`KismetMathLibrary.RLerp` (`self.receiverArrivingWRot`) (`self.receiverSetupWRot`) _directinsert) false false)
              (`SceneComponent.K2_SetRelativeRotation` (`/Game/Blueprints/newBridge/BP_HangingCable.plugDummy` _hangingcable_2) (`KismetMathLibrary.RLerp` (`self.receiverArrivingRrot`) (struct :`Pitch` 90.0) _directinsert) false false))
            (:`Finished`
              (set `self.PlugInserted` true) ; 4 state machine
              (`|ExecutionSequence`
                (:`then_0`
                  ;;[1 1 1] turn on Ballasts
                  (`|ExecutionSequence`
                    (:`then_0`
                      (bind _asbp_ballast (cast `/Game/Blueprints/newBridge/BP_Ballast` (`ChildActorComponent.ChildActor` (`self.Ballast_Front1`))))
                      (`/Game/Blueprints/newBridge/BP_Ballast.UpdateState` _asbp_ballast "NewEnumerator0"))
                    (:`then_1`
                      (bind _asbp_ballast_2 (cast `/Game/Blueprints/newBridge/BP_Ballast` (`ChildActorComponent.ChildActor` (`self.Ballast_Front2`))))
                      (`/Game/Blueprints/newBridge/BP_Ballast.UpdateState` _asbp_ballast_2 "NewEnumerator0"))))
                (:`then_1`
                  (`MaterialInstanceDynamic.SetScalarParameterValue` (`self.holoBridge`) "Flicker" 1.0)
                  (`KismetSystemLibrary.Delay` 0.15)
                  ;;[1 1 1] Cable
                  (bind (_direction_2 _lenght) (`Timeline|CablesAnim` :!via `PlayFromStart`)
                    (:`Update`
                      (`|ExecutionSequence`
                        (:`then_0`
                          (bind _returnvalue_3 (`KismetMathLibrary.Lerp` 20.0 17.0 _lenght))
                          (set `CableComponent.CableLength` _returnvalue_3 (`self.CableBack`))
                          (set `CableComponent.CableLength` _returnvalue_3 (`/Game/Blueprints/newBridge/BP_HangingCable.Cable` (`self.hangingCable`))))))
                    (:`Finished`
                      ;;[1 1 1] Beams
                      (`|ExecutionSequence`
                        (:`then_0`
                          (`ActorComponent.ToggleActive` (`self.bridgingBeam`))
                          (`ActorComponent.ToggleActive` (`self.backBeam`))
                          (`ActorComponent.ToggleActive` (`self.frontBeam`))
                          (`self.SetBeamParameters` (`self.backBeam`) _returnvalue _returnvalue_2)
                          (`self.SetBeamParameters` (`self.frontBeam`) (- _returnvalue (-8.8 0.0 0.0)) (- _returnvalue_2 (-8.8 0.0 0.0))))
                        (:`then_1`
                          (bind (_direction_3 _bridgingbeam_2) (`Timeline|BeamsAnim` :!via `PlayFromStart`)
                            (:`Update`
                              (`FXSystemComponent.SetColorParameter` _bridgingbeam "Beam_Colour" (struct :`G` 50.0 :`B` 50.0 :`A` 1.0))
                              (bind _returnvalue_4 (`KismetMathLibrary.VLerp` (`SceneComponent.K2_GetComponentLocation` (`self.Plug_1`)) (`SceneComponent.K2_GetComponentLocation` (`self.Plug_2`)) _bridgingbeam_2))
                              (`ParticleSystemComponent.SetBeamSourcePoint` _bridgingbeam 0 _returnvalue_4 0)
                              (`ParticleSystemComponent.SetBeamTargetPoint` _bridgingbeam 0 (- _returnvalue_4 (-8.8 0.0 0.0)) 0))
                            (:`Finished`
                              (`|ExecutionSequence`
                                (:`then_0`
                                  (`ActorComponent.Deactivate` (`self.bridgingBeam`))
                                  (`ActorComponent.Deactivate` (`self.backBeam`))
                                  (`ActorComponent.Deactivate` (`self.frontBeam`))
                                  (`ActorComponent.ToggleActive` (`self.SparksRecieverFront`))
                                  (`ActorComponent.ToggleActive` (`self.SparksRecieverBack`))
                                  (`GameplayStatics.PlaySoundAtLocation` "/Game/Sounds/Bridge01/SC_LargeSpark.SC_LargeSpark" (`SceneComponent.K2_GetComponentLocation` (`self.SparksRecieverFront`)) (struct) 1.0 1.0 0.0 "/Game/Sounds/DefaultAttenuationSettings.DefaultAttenuationSettings" null null)
                                  (`GameplayStatics.PlaySoundAtLocation` "/Game/Sounds/Bridge01/SC_LargeSpark.SC_LargeSpark" (`SceneComponent.K2_GetComponentLocation` (`self.SparksRecieverBack`)) (struct) 1.0 1.0 0.0 "/Game/Sounds/DefaultAttenuationSettings.DefaultAttenuationSettings" null null)
                                  (`/Game/Blueprints/newBridge/BP_HangingCable.DeactivateIdleSparks` (`self.hangingCable`)))
                                (:`then_1`
                                  (`MaterialInstanceDynamic.SetScalarParameterValue` (`self.holoBridge`) "Flicker" 0.0)
                                  (bind (_direction_4 _lerp) (`Timeline|BridgeAnim` :!via `PlayFromStart`)
                                    (:`Update`
                                      (`MaterialInstanceDynamic.SetScalarParameterValue` (`self.holoBridge`) "BridgeReveal" _lerp))
                                    (:`Finished`
                                      (set `self.Extended` true) ; 4 state machine
                                    )))))))))))))))))))

(event `/Game/Framework/BP_GazeTriggerInterface.OnGazeBegin`
  (bind _backbeam (`self.backBeam`))
  (bind _cableback (`self.CableBack`))
  ;[1 1 1] Gaze Sequence
  (if (`self.canWiggleGaze`)
    (set `self.canWiggleGaze` false)
    (`ActorComponent.Activate` _backbeam false)
    (`self.SetBeamParameters` _backbeam (`SceneComponent.K2_GetComponentLocation` (`self.Plug_1`)) (`SceneComponent.K2_GetComponentLocation` (`self.Plug_2`)) (struct :`G` 1.0 :`B` 1.0 :`A` 1.0) 7.0)
    (`KismetSystemLibrary.Delay` 0.2)
    (`ActorComponent.Deactivate` _backbeam)
    (`KismetSystemLibrary.Delay` 0.5)
    (set `CableComponent.bEnableStiffness` false _cableback)
    (`KismetSystemLibrary.Delay` 0.1)
    (set `CableComponent.bEnableStiffness` true _cableback)
    (`KismetSystemLibrary.Delay` 4.0)
    (set `self.canWiggleGaze` true)))

(fn `SetBeamParameters`
  (params (particleSystem :type "ParticleSystemComponent Object Reference") (sourceLocation :type "Vector Structure") (targetLocation :type "Vector Structure") (colour :type "LinearColor Structure" :default (struct :`G` 1.0 :`B` 1.0 :`A` 1.0)) (tangent :type "Float (double-precision)"))
  (`|ExecutionSequence`
    (:`then_0`
      (`ParticleSystemComponent.SetBeamSourcePoint` particleSystem 0 sourceLocation 0)
      (`ParticleSystemComponent.SetBeamTargetPoint` particleSystem 0 targetLocation 0))
    (:`then_1`
      (`FXSystemComponent.SetColorParameter` particleSystem "Beam_Colour" colour))
    (:`then_2`
      (`FXSystemComponent.SetVectorParameter` particleSystem "SourceTangent" (`KismetMathLibrary.MakeVector` 0.0 0.0 (* tangent -1.0)))
      (`FXSystemComponent.SetVectorParameter` particleSystem "TargetTangent" (`KismetMathLibrary.MakeVector` 0.0 0.0 tangent)))))

(fn `SetupRecieverTransforms`
  (bind _plugoverlap (`self.plugOverlap`))
  (bind _returnvalue (`SceneComponent.K2_GetComponentToWorld` (`self.DefaultSceneRoot`)))
  (bind (_relativelocation_x _relativelocation_y _relativelocation_z) (`KismetMathLibrary.BreakVector` (`SceneComponent.RelativeLocation` _plugoverlap)))
  (set `self.receiverSetupWRot` (`SceneComponent.K2_GetComponentRotation` _plugoverlap))
  (set `self.receiverSetupWLoc` (`KismetMathLibrary.TransformLocation` _returnvalue (`KismetMathLibrary.MakeVector` _relativelocation_x (- _relativelocation_y -3.0) _relativelocation_z)))
  (set `self.receiverLandingWLoc` (`KismetMathLibrary.TransformLocation` _returnvalue (`KismetMathLibrary.MakeVector` _relativelocation_x (- _relativelocation_y -2.5) _relativelocation_z))))

(fn `UserConstructionScript`
  (`|ExecutionSequence`
    (:`then_0`
      (`self.SetupRecieverTransforms`))
    (:`then_1`
      (bind _returnvalue (`KismetMaterialLibrary.CreateDynamicMaterialInstance` "/Game/Materials/M_HoloBridge.M_HoloBridge"))
      (set `self.holoBridge` _returnvalue)
      (`PrimitiveComponent.SetMaterial` (`self.Bridge`) 0 (`self.holoBridge`)))))