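; A sparking hanging cable with a plug that hands can grab, using a BP_Pickupable child actor with UXT manipulation.
; While held, Tick eases the cable end toward the pickupable within a clamped radius, force-releasing it if too far; otherwise plug and pickupable follow the physics-simulated end.
; A spawned outline actor and glow component show gaze, grab and hint states.
; Timers drive idle sparks and, when still, beam flashes and radial-impulse wiggles.
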(event `self.ReceiveBeginPlay`
  (bind _interactiveeffect (`self.interactiveEffect`))
  (bind _plugdummy (`self.plugDummy`))
  (bind _interactiveeffect_2 (`self.interactiveEffect`))
  (set `self.PreviousLocation` (`SceneComponent.K2_GetComponentLocation` (`self.dummyRoot`)))
  (bind _returnvalue (`KismetSystemLibrary.K2_SetTimer` null "TriggerIdleSparks" 5.0 true 5.0))
  (set `self.SparksTimerHandle` _returnvalue)
  ;[1 1 1] Spawn interactive object effect BP
  (bind _returnvalue_2 (`|SpawnActorFromClass` "/Game/Blueprints/BP_InteractiveObjectsEffect_Outline.BP_InteractiveObjectsEffect_Outline_C" (`KismetMathLibrary.MakeTransform` (`SceneComponent.K2_GetComponentLocation` _plugdummy) (`SceneComponent.K2_GetComponentRotation` _plugdummy)) "Undefined" "OverrideRootScale" null null))
  (set `self.interactiveEffect` _returnvalue_2)
  (`self.K2_AttachToComponent` _interactiveeffect _plugdummy "None" "KeepWorld" "KeepWorld" "KeepWorld" true)
  (`StaticMeshComponent.SetStaticMesh` (`/Game/Blueprints/BP_InteractiveObjectsEffect_Outline.outlineMesh` _interactiveeffect) "/Game/Art/Bridge/SM_Bridge_plugMale_Outline.SM_Bridge_plugMale_Outline")
  (set `/Game/Blueprints/BP_InteractiveObjectsEffect_Outline.isActive` true _interactiveeffect_2)
  (set `/Game/Blueprints/BP_InteractiveObjectsEffect_Outline.thicknessFocusTarget` 0.55 _interactiveeffect_2))

(event `ChangeHeldState`
  (params (isHeld :type Boolean))
  (bind _interactiveeffect (`self.interactiveEffect`))
  (bind _interactiveeffect_2 (`self.interactiveEffect`))
  ;[1 1 1] Change Held State
  (bind _output_get (set `self.isHeld` isHeld))
  (if _output_get
    (`PrimitiveComponent.SetSimulatePhysics` (`self.attachmentEnd`) false)
    (`/Game/Blueprints/BP_GlowHintInterface.DeactivateHint`)
    (`self.ScaleDown`)
    (`/Engine/EditorBlueprintResources/StandardMacros.IsValid` _interactiveeffect
      (:`Is Valid`
        (set `/Game/Blueprints/BP_InteractiveObjectsEffect_Outline.isGrabbed` true _interactiveeffect)))
    (else
      (`PrimitiveComponent.SetSimulatePhysics` (`self.attachmentEnd`) true)
      (`/Engine/EditorBlueprintResources/StandardMacros.IsValid` _interactiveeffect_2
        (:`Is Valid`
          (set `/Game/Blueprints/BP_InteractiveObjectsEffect_Outline.isGrabbed` false _interactiveeffect_2))))))

(event `/Game/Blueprints/BP_GlowHintInterface.ActivateHint`
  (bind _bp_glowhintcomponent (`self.BP_GlowHintComponent`))
  ;[0.3294 1 0.9302 0.154] Hint Glow Effects
  (`/Game/Blueprints/BP_GlowHintComponent.ActivateOutliner` _bp_glowhintcomponent (`self.plugDummy`))
  (set `self.canWiggle` false :!label _label)
  (`/Game/Blueprints/BP_GlowHintComponent.ActivateParticleSystem` _bp_glowhintcomponent))

(event `/Game/Framework/BP_GazeTriggerInterface.OnGazeBegin`
  ;[1 1 1] Gaze
  (set `/Game/Blueprints/BP_InteractiveObjectsEffect_Outline.isLookedAt` true (`self.interactiveEffect`)))

(event `EnterGrabFocus`
  (set `/Game/Blueprints/BP_InteractiveObjectsEffect_Outline.grabFocus` true (`self.interactiveEffect`))
  (`self.ScaleUp`))

(event `/Game/Blueprints/BP_GlowHintInterface.EnableHintParticles`
  ;[0.3294 1 0.9302 0.154] Hint Glow Effects
  (goto _label))

(event `ScaleUp`
  (bind (_direction _scale) (`Timeline|GrabFocusScaleTimeline` :!label _label_2)
    (:`Update`
      (`SceneComponent.SetRelativeScale3D` (`self.plugDummy`) (`KismetMathLibrary.Conv_DoubleToVector` (`KismetMathLibrary.Lerp` 1.0 1.175 _scale))))))

(event `/Game/Blueprints/BP_GlowHintInterface.DeactivateHint`
  (bind _bp_glowhintcomponent (`self.BP_GlowHintComponent`))
  ;[0.3294 1 0.9302 0.154] Hint Glow Effects
  (`/Game/Blueprints/BP_GlowHintComponent.DeactivateOutliner` _bp_glowhintcomponent (`self.plugDummy`))
  (set `self.canWiggle` true :!label _label_3)
  (`/Game/Blueprints/BP_GlowHintComponent.DeactivateParticleSystem` _bp_glowhintcomponent))

(event `ScaleDown`
  (goto _label_2 :!via `Reverse`))

(event `ExitGrabFocus`
  (set `/Game/Blueprints/BP_InteractiveObjectsEffect_Outline.grabFocus` false (`self.interactiveEffect`))
  (`self.ScaleDown`))

(event `/Game/Framework/BP_GazeTriggerInterface.OnGazeEnd`
  ;[1 1 1] Gaze
  (set `/Game/Blueprints/BP_InteractiveObjectsEffect_Outline.isLookedAt` false (`self.interactiveEffect`)))

(event `/Game/Blueprints/BP_GlowHintInterface.DisableHintParticles`
  ;[0.3294 1 0.9302 0.154] Hint Glow Effects
  (goto _label_3))

(event `ActivateDeactivatePlug`
  (params (Active :type Boolean :default true))
  (bind _interactiveeffect (`self.interactiveEffect`))
  ;[1 1 1] Activeate Deactivate
  (set `self.isActive` Active)
  (`|ExecutionSequence`
    (:`then_0`
      (`/Engine/EditorBlueprintResources/StandardMacros.IsValid` _interactiveeffect
        (:`Is Valid`
          _)
        (:`Is Not Valid`
          (`KismetSystemLibrary.Delay` 0.1)))
      (set `/Game/Blueprints/BP_InteractiveObjectsEffect_Outline.isActive` Active _interactiveeffect))
    (:`then_1`
      (bind _asbp_pickupable (cast `/Game/Blueprints/newBridge/BP_Pickupable` (`ChildActorComponent.ChildActor` (`self.pickupable`))))
      (`/Game/Blueprints/newBridge/BP_Pickupable.ActivateDeactivate` _asbp_pickupable Active))))

(event `self.ReceiveTick`
  (params (DeltaSeconds :type "Float (single-precision)"))
  (bind _dummyroot (`self.dummyRoot`))
  (bind _dummyroot_2 (`self.dummyRoot`))
  (bind _plugdummy (`self.plugDummy`))
  (bind _previouslocation (`self.PreviousLocation`))
  (bind _returnvalue (`KismetMathLibrary.SelectFloat` 20.0 17.0 (`self.isHeld`)))
  (bind _returnvalue_2 (`SceneComponent.K2_GetComponentLocation` (`self.DefaultSceneRoot`)))
  (bind _returnvalue_3 (`KismetMathLibrary.SelectVector` (`self.K2_GetActorLocation`) (`SceneComponent.K2_GetComponentLocation` (`self.dummyRoot`)) (`self.isHeld`)))
  (if (`self.isActive`)
    (`|ExecutionSequence`
      (:`then_0`
        (if (`self.isHeld`)
          ;[1 1 1] Follow Attachment or Pickuapable
          (`SceneComponent.K2_SetWorldLocation` (`self.attachmentEnd`) (`KismetMathLibrary.VInterpTo` (`SceneComponent.K2_GetComponentLocation` (`self.dummyRoot`)) (+ (`KismetMathLibrary.ClampVectorSize` (- (`SceneComponent.K2_GetComponentLocation` (`Actor.RootComponent` (`ChildActorComponent.ChildActor` (`self.pickupable`)))) _returnvalue_2) -25.0 25.0) _returnvalue_2) (`GameplayStatics.GetWorldDeltaSeconds`) 10.0) false false)
          (`SceneComponent.K2_SetWorldLocation` (`self.dummyRoot`) (`KismetMathLibrary.VInterpTo` (`SceneComponent.K2_GetComponentLocation` (`self.dummyRoot`)) (+ (`KismetMathLibrary.ClampVectorSize` (- (`SceneComponent.K2_GetComponentLocation` (`Actor.RootComponent` (`ChildActorComponent.ChildActor` (`self.pickupable`)))) _returnvalue_2) -25.0 25.0) _returnvalue_2) (`GameplayStatics.GetWorldDeltaSeconds`) 10.0) false false)
          (else
            (`SceneComponent.K2_SetWorldLocation` _dummyroot_2 (`KismetMathLibrary.VInterpTo` (`SceneComponent.K2_GetComponentLocation` _dummyroot_2) (`SceneComponent.K2_GetComponentLocation` (`self.attachmentEnd`)) (`GameplayStatics.GetWorldDeltaSeconds`) 5.0) false false)
            (`SceneComponent.K2_SetWorldLocation` (`Actor.RootComponent` (`ChildActorComponent.ChildActor` (`self.pickupable`))) (`KismetMathLibrary.VInterpTo` (`SceneComponent.K2_GetComponentLocation` _dummyroot_2) (`SceneComponent.K2_GetComponentLocation` (`self.attachmentEnd`)) (`GameplayStatics.GetWorldDeltaSeconds`) 5.0) false false)))
        ;[1 1 1] Rotates plug
        (`|ExecutionSequence`
          (:`then_0`
            ;;[1 1 1] dummy relative rotation
            (set `self.dummyCurrentYrotation` (`KismetMathLibrary.FInterpTo` (`self.dummyCurrentYrotation`) (`KismetMathLibrary.SelectFloat` 90.0 0.0 (`self.isHeld`)) (`GameplayStatics.GetWorldDeltaSeconds`) 3.0))
            (`SceneComponent.K2_SetRelativeRotation` _plugdummy (`KismetMathLibrary.MakeRotator` 0.0 (`self.dummyCurrentYrotation`)) false false)
            (`SceneComponent.K2_SetWorldRotation` (`Actor.RootComponent` (`ChildActorComponent.ChildActor` (`self.pickupable`))) (`SceneComponent.K2_GetComponentRotation` _plugdummy) false false))
          (:`then_1`
            ;;[1 1 1] lookat logic
            (`SceneComponent.K2_SetWorldRotation` _dummyroot (`KismetMathLibrary.RInterpTo` (`SceneComponent.K2_GetComponentRotation` _dummyroot) (`KismetMathLibrary.SelectRotator` (`KismetMathLibrary.FindLookAtRotation` (`self.PreviousLocation`) (`SceneComponent.K2_GetComponentLocation` _dummyroot)) (struct :`Yaw` -90.0) (`self.isHeld`)) (`GameplayStatics.GetWorldDeltaSeconds`) 3.0) false false))
          (:`then_2`
            (if (!= _previouslocation _returnvalue_3 :`ErrorTolerance` 0.5)
              (set `self.PreviousLocation` (+ _previouslocation (/ (- _returnvalue_3 _previouslocation) 2.0)))))))
      (:`then_1`
        ;[1 1 1] Cahnges cable lenght
        (if (!= (`CableComponent.CableLength` (`self.Cable`)) _returnvalue)
          (set `CableComponent.CableLength` (`KismetMathLibrary.FInterpTo` (`CableComponent.CableLength` (`self.Cable`)) _returnvalue (`GameplayStatics.GetWorldDeltaSeconds`) 3.0) (`self.Cable`))))
      (:`then_2`
        ;[1 1 1] Detaches from hand if it's too far
        (if (> (`KismetMathLibrary.Vector_Distance` (`SceneComponent.K2_GetComponentLocation` (`self.DefaultSceneRoot`)) (`SceneComponent.K2_GetComponentLocation` (`Actor.RootComponent` (`ChildActorComponent.ChildActor` (`self.pickupable`))))) 40.0)
          (bind _asbp_pickupable (cast `/Game/Blueprints/newBridge/BP_Pickupable` (`ChildActorComponent.ChildActor` (`self.pickupable`))))
          (`UxtGrabTargetComponent.ForceEndGrab` (`/Game/Blueprints/newBridge/BP_Pickupable.UxtGenericManipulator` _asbp_pickupable))))
      (:`then_3`
        ;[1 1 1] Wiggle Timer
        (if (`self.canWiggle`)
          (bind _returnvalue_4 (`PrimitiveComponent.GetPhysicsLinearVelocity` (`self.plugDummy`) "None"))
          (if (and (== _returnvalue_4 (0.0 0.0 0.0)) (== (`self.isHeld`) false))
            (`/Engine/EditorBlueprintResources/StandardMacros.DoOnce` false :!label _label_4
              (:`Completed`
                (`KismetSystemLibrary.K2_SetTimer` null "Wiggle" 1.0 true)
                (goto _label_5 :!via `Reset`)))
            (else
              (`/Engine/EditorBlueprintResources/StandardMacros.DoOnce` false :!label _label_5
                (:`Completed`
                  (`KismetSystemLibrary.K2_PauseTimer` null "Wiggle")
                  (`KismetSystemLibrary.K2_ClearTimer` null "Wiggle")
                  (`ActorComponent.Deactivate` (`self.Beam`))
                  (set `self.wiggleCurrentTime` 0)
                  (goto _label_4 :!via `Reset`))))))))))

(fn `DeactivateIdleSparks`
  (`KismetSystemLibrary.K2_PauseTimer` null "TriggerIdleSparks")
  (`KismetSystemLibrary.K2_ClearTimer` null "TriggerIdleSparks"))

(fn `TriggerIdleSparks`
  (`ActorComponent.Activate` (`self.SparksIdle`) true)
  (`GameplayStatics.PlaySoundAtLocation` "/Game/Sounds/Bridge01/SC_LargeSpark.SC_LargeSpark" (`SceneComponent.K2_GetComponentLocation` (`self.SparksOnce`)) (struct) (`KismetMathLibrary.RandomFloatInRange` 0.2 0.4) (`KismetMathLibrary.RandomFloatInRange` 0.8 1.2) 0.0 "/Game/Sounds/DefaultAttenuationSettings.DefaultAttenuationSettings" null null))

(fn `UserConstructionScript`
  (`TimelineComponent.SetPlayRate` (`self.GrabFocusScaleTimeline`) 3.5))

(fn `Wiggle`
  (bind (_returnvalue_x _returnvalue_y) (`KismetMathLibrary.BreakVector` (`KismetMathLibrary.RandomUnitVector`)))
  (bind _beam (`self.Beam`))
  (bind _radialforce (`self.RadialForce`))
  (bind (_relativelocation_x _relativelocation_y _relativelocation_z) (`KismetMathLibrary.BreakVector` (`SceneComponent.RelativeLocation` _radialforce)))
  (set `self.wiggleCurrentTime` (+ (`self.wiggleCurrentTime`) 1))
  (`|ExecutionSequence`
    (:`then_0`
      ;[1 1 1] Beam FX
      (if (== (`self.wiggleCurrentTime`) 3)
        (`ActorComponent.Activate` (`self.Beam`) false)
        (`ParticleSystemComponent.SetBeamSourcePoint` _beam 0 (`SceneComponent.K2_GetComponentLocation` (`self.DefaultSceneRoot`)) 0)
        (`ParticleSystemComponent.SetBeamTargetPoint` _beam 0 (`SceneComponent.K2_GetComponentLocation` (`self.plugDummy`)) 0)
        (`FXSystemComponent.SetColorParameter` _beam "Beam_Colour" (struct :`G` 33.799957 :`B` 50.0 :`A` 1.0))
        (else
          (`ActorComponent.Deactivate` (`self.Beam`)))))
    (:`then_1`
      (if (== (`self.wiggleCurrentTime`) 4)
        (`SceneComponent.K2_SetRelativeLocation` _radialforce (`KismetMathLibrary.MakeVector` (* _returnvalue_x 3.0) (* _returnvalue_y 3.0) _relativelocation_z) false false)
        (`RadialForceComponent.FireImpulse` (`self.RadialForce`))
        (`ActorComponent.Activate` (`self.SparksOnce`) true)
        (`GameplayStatics.PlaySoundAtLocation` "/Game/Sounds/Bridge01/SC_LargeSpark.SC_LargeSpark" (`SceneComponent.K2_GetComponentLocation` (`self.SparksOnce`)) (struct) 1.0 1.0 0.0 "/Game/Sounds/DefaultAttenuationSettings.DefaultAttenuationSettings" null null)))))