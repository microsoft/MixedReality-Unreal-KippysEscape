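; BP_Pickupable is a grabbable Mixed Reality UX Tools actor that acts as the pickup for its parent BP_HangingCable.
; Its generic manipulator forwards grab and focus events to the cable, setting held state and playing an audio cue on grab.
; ActivateDeactivate enables pickup collision after a short delay, or disables it and force-ends any grab.
; The shadow and glint alignment functions contain only unconnected logic.
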(event `self.UxtGenericManipulator.OnBeginGrab`
  (params (Grabbable :type "UxtGrabTargetComponent Object Reference") (GrabPointer :type "UxtGrabPointerData Structure"))
  ;[1 1 1] Begin and end grab
  (bind _asbp_hanging_cable (cast `/Game/Blueprints/newBridge/BP_HangingCable` (`self.GetParentActor`)))
  (`/Game/Blueprints/newBridge/BP_HangingCable.ChangeHeldState` _asbp_hanging_cable true)
  (`AudioComponent.Play` (`self.AUD_Grab_Cue`) 0.0))

(event `self.UxtGenericManipulator.OnEnterGrabFocus`
  (params (Grabbable :type "UxtGrabTargetComponent Object Reference") (Pointer :type "UxtNearPointerComponent Object Reference"))
  ;[1 1 1] Grab Focus
  (bind _asbp_hanging_cable (cast `/Game/Blueprints/newBridge/BP_HangingCable` (`self.GetParentActor`)))
  (`/Game/Blueprints/newBridge/BP_HangingCable.EnterGrabFocus` _asbp_hanging_cable))

(event `self.UxtGenericManipulator.OnEndGrab`
  (params (Grabbable :type "UxtGrabTargetComponent Object Reference") (GrabPointer :type "UxtGrabPointerData Structure"))
  ;[1 1 1] Begin and end grab
  (bind _asbp_hanging_cable (cast `/Game/Blueprints/newBridge/BP_HangingCable` (`self.GetParentActor`)))
  (`/Game/Blueprints/newBridge/BP_HangingCable.ChangeHeldState` _asbp_hanging_cable false))

(event `self.UxtGenericManipulator.OnExitGrabFocus`
  (params (Grabbable :type "UxtGrabTargetComponent Object Reference") (Pointer :type "UxtNearPointerComponent Object Reference"))
  ;[1 1 1] Grab Focus
  (bind _asbp_hanging_cable (cast `/Game/Blueprints/newBridge/BP_HangingCable` (`self.GetParentActor`)))
  (`/Game/Blueprints/newBridge/BP_HangingCable.ExitGrabFocus` _asbp_hanging_cable))

(event `ActivateDeactivate`
  (params (Active :type Boolean))
  (if Active
    (`KismetSystemLibrary.Delay` 1.5)
    (`PrimitiveComponent.SetCollisionEnabled` (`self.Pickup`) "QueryAndPhysics")
    (else
      (`PrimitiveComponent.SetCollisionEnabled` (`self.Pickup`) "NoCollision")
      (`UxtGrabTargetComponent.ForceEndGrab` (`self.UxtGenericManipulator`)))))

(fn `AlignGlintEffect`)

(fn `AlignShadow`)

(fn `IsGrabFocusable`
  (params (Primitive :type "PrimitiveComponent Object Reference"))
  (returns (ReturnValue :type Boolean))
  (return true))

(fn `UserConstructionScript`)