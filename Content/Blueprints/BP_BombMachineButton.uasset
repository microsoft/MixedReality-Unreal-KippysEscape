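; Pressable bomb machine button built on UxtPressableButton, with visual and audio feedback for gaze, focus and presses.
; BeginPlay caches the dynamic material's base color and attaches a spawned outline effect actor that receives active, gaze, focus and press flags.
; Button events play sounds, drive a scale timeline and refresh the color from button state, brightened when focused and gray when disabled.
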(event `self.ReceiveBeginPlay`
  (bind _movingvisuals (`self.MovingVisuals`))
  (bind _interactiveeffect (`self.interactiveEffect`))
  (bind _movingvisuals_2 (`self.MovingVisuals`))
  (bind _interactiveeffect_2 (`self.interactiveEffect`))
  (`|ExecutionSequence`
    (:`then_0`
      ;[1 1 1] Create a dynamic material instance so we can update it to reflect button state
      (bind _returnvalue (`PrimitiveComponent.CreateDynamicMaterialInstance` _movingvisuals 0 (`PrimitiveComponent.GetMaterial` _movingvisuals 0) "None"))
      ;[1 1 1] Store initial base color
      (bind _returnvalue_2 (`MaterialInstanceDynamic.K2_GetVectorParameterValue` _returnvalue "Base Color"))
      (set `self.BaseColor` _returnvalue_2))
    (:`then_1`
      ;[0.3 0.3 0.3] Spawn interactive object effect BP
      (bind _returnvalue_3 (`|SpawnActorFromClass` "/Game/Blueprints/BP_InteractiveObjectsEffect_Outline.BP_InteractiveObjectsEffect_Outline_C" (`KismetMathLibrary.MakeTransform` (`SceneComponent.K2_GetComponentLocation` _movingvisuals_2) (`SceneComponent.K2_GetComponentRotation` _movingvisuals_2)) "Undefined" "OverrideRootScale" null null))
      (set `self.interactiveEffect` _returnvalue_3)
      (`self.K2_AttachToComponent` _interactiveeffect_2 (`self.MovingVisuals`) "None" "KeepWorld" "KeepWorld" "KeepWorld" true)
      (`StaticMeshComponent.SetStaticMesh` (`/Game/Blueprints/BP_InteractiveObjectsEffect_Outline.outlineMesh` _interactiveeffect_2) "/Game/Art/BombMachine/SM_BombMachine_Switch_Outline.SM_BombMachine_Switch_Outline")
      (set `/Game/Blueprints/BP_InteractiveObjectsEffect_Outline.thicknessActiveTarget` (* 0.35 0.9) _interactiveeffect)
      (set `/Game/Blueprints/BP_InteractiveObjectsEffect_Outline.thicknessFocusTarget` (* 0.55 0.9) _interactiveeffect))))

(event `ActivateDeactivateAffordance`
  (params (Active :type Boolean))
  (set `/Game/Blueprints/BP_InteractiveObjectsEffect_Outline.isActive` Active (`self.interactiveEffect`)))

(event `/Game/Framework/BP_GazeTriggerInterface.OnGazeBegin`
  ;[1 1 1] gaze
  (set `/Game/Blueprints/BP_InteractiveObjectsEffect_Outline.isLookedAt` true (`self.interactiveEffect`)))

(event `ScaleUp`
  ;[1 1 1] Interactive Scaling
  (bind (_direction _scale) (`Timeline|GrabFocusScaleTimeline` :!label _label)
    (:`Update`
      (`SceneComponent.SetRelativeScale3D` (`self.MovingVisuals`) (`KismetMathLibrary.Conv_DoubleToVector` (`KismetMathLibrary.Lerp` 1.0 1.15 _scale))))))

(event `ScaleDown`
  ;[1 1 1] Interactive Scaling
  (goto _label :!via `Reverse`))

(event `/Game/Framework/BP_GazeTriggerInterface.OnGazeEnd`
  ;[1 1 1] gaze
  (set `/Game/Blueprints/BP_InteractiveObjectsEffect_Outline.isLookedAt` false (`self.interactiveEffect`)))

(event `self.UxtPressableButton.OnBeginFocus`
  (params (Button :type "UxtPressableButtonComponent Object Reference") (Pointer :type "UxtPointerComponent Object Reference") (bWasAlreadyFocused :type Boolean))
  ;[1 1 1] begin focus
  (if (not bWasAlreadyFocused)
    (`self.UpdateButtonColor`)
    (set `/Game/Blueprints/BP_InteractiveObjectsEffect_Outline.grabFocus` true (`self.interactiveEffect`))
    (`self.ScaleUp`)))

(event `self.UxtPressableButton.OnButtonPressed`
  (params (Button :type "UxtPressableButtonComponent Object Reference") (Pointer :type "UxtPointerComponent Object Reference"))
  ;[1 1 1] Play sound on press
  (`GameplayStatics.PlaySoundAtLocation` (`self.PressedSound`) (`SceneComponent.K2_GetComponentLocation` (`self.MovingVisuals`)) (struct) 1.0 1.0 0.0 "/Game/Sounds/DefaultAttenuationSettings.DefaultAttenuationSettings" null null)
  (set `/Game/Blueprints/BP_InteractiveObjectsEffect_Outline.isGrabbed` true (`self.interactiveEffect`))
  (`self.ScaleDown`))

(event `self.UxtPressableButton.OnButtonEnabled`
  (params (Button :type "UxtPressableButtonComponent Object Reference"))
  (`self.UpdateButtonColor`))

(event `self.UxtPressableButton.OnEndFocus`
  (params (Button :type "UxtPressableButtonComponent Object Reference") (Pointer :type "UxtPointerComponent Object Reference") (bIsStillFocused :type Boolean))
  ;[1 1 1] begin focus
  (if (not bIsStillFocused)
    (`self.UpdateButtonColor`)
    (set `/Game/Blueprints/BP_InteractiveObjectsEffect_Outline.grabFocus` false (`self.interactiveEffect`))
    (`self.ScaleDown`)))

(event `self.UxtPressableButton.OnButtonReleased`
  (params (Button :type "UxtPressableButtonComponent Object Reference") (Pointer :type "UxtPointerComponent Object Reference"))
  ;[1 1 1] Play sound on release
  (`GameplayStatics.PlaySoundAtLocation` (`self.ReleasedSound`) (`SceneComponent.K2_GetComponentLocation` (`self.MovingVisuals`)) (struct) 1.0 1.0 0.0 "/Game/Sounds/DefaultAttenuationSettings.DefaultAttenuationSettings" null null)
  (set `/Game/Blueprints/BP_InteractiveObjectsEffect_Outline.isGrabbed` false (`self.interactiveEffect`))
  (`self.ScaleUp`))

(event `self.UxtPressableButton.OnButtonDisabled`
  (params (Button :type "UxtPressableButtonComponent Object Reference"))
  (`self.UpdateButtonColor`))

(fn `UpdateButtonColor`
  (switch `EUxtButtonState` (`UxtPressableButtonComponent.GetState` (`self.UxtPressableButton`))
    (:`Default`
      ;[1 1 1] Set original base color
      (`MeshComponent.SetVectorParameterValueOnMaterials` (`self.MovingVisuals`) "Base Color" (`KismetMathLibrary.Conv_LinearColorToVector` (`self.BaseColor`))))
    (:`Disabled`
      ;[1 1 1] Gray out button when disabled
      (`MeshComponent.SetVectorParameterValueOnMaterials` (`self.MovingVisuals`) "Base Color" (`KismetMathLibrary.Conv_LinearColorToVector` (struct :`R` 0.25 :`G` 0.25 :`B` 0.25 :`A` 1.0))))
    (:`Focused`
      ;[1 1 1] Lighten base color when focused
      (`MeshComponent.SetVectorParameterValueOnMaterials` (`self.MovingVisuals`) "Base Color" (`KismetMathLibrary.Conv_LinearColorToVector` (* (`self.BaseColor`) 2.0))))))

(fn `UserConstructionScript`
  (`TimelineComponent.SetPlayRate` (`self.GrabFocusScaleTimeline`) 3.5))