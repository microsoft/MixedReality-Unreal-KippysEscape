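; Hand-grabbable (UXT) red, green or blue puzzle gem that starts inactive-colored until activated, then can be fitted into its matching BP_GemSocket.
; GemColor selects mesh, dynamic materials and socket.
; Tick hovers active, unheld gems over plinths and drives hum and emissive by socket distance.
; InsertGem locks manipulation, animates the gem into place and triggers BP_Island02 emissive; gaze, grab, hint and respawn events add feedback, while hand-proximity scaling is unwired.
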(event `self.ReceiveTick`
  (params (DeltaSeconds :type "Float (single-precision)"))
  (bind _gemloop (`self.GemLoop`))
  (bind _returnvalue (and (`self.Active`) (`self.OverlappingPlinth`) (not (`self.Held`))))
  (`|ExecutionSequence`
    (:`then_0`
      ;[0.06274 0.3176 1] Check if gem should be hovering
      (if (xor _returnvalue (`self.Hovering`))
        (bind _output_get (set `self.Hovering` _returnvalue))
        (if _output_get
          (`self.StartHover`)
          (else
            (`self.StopHover`)))))
    (:`then_1`
      ;[0.1146 0.1146 0.1146 0.339] Make gem humming audio louder and pitch up as it gets closer to the socket
      (if (`self.Inserted`)
        ;;[0 0 0] Fade out loop
        (`AudioComponent.FadeOut` (`self.GemLoop`) 1.0 0.0 "Linear")
        (elif (`self.Active`)
          (bind _output_get_2 (set `self.DistanceFromSocket` (`KismetMathLibrary.Vector_Distance` (`SceneComponent.K2_GetComponentLocation` (`self.GemMesh`)) (`self.SocketLocation`))))
          (if (< _output_get_2 (`self.LoopAudioStartDistance`))
            ;[0 0 0] Making audio smoother for gem loop
            (if (not (`AudioComponent.IsPlaying` (`self.GemLoop`)))
              (`AudioComponent.Play` (`self.GemLoop`) 0.0))
            (bind _returnvalue_2 (- 1.0 (`KismetMathLibrary.NormalizeToRange` _output_get_2 0.0 (`self.LoopAudioStartDistance`))))
            (`AudioComponent.SetVolumeMultiplier` _gemloop _returnvalue_2)
            (`AudioComponent.SetPitchMultiplier` _gemloop (+ 1.0 (/ _returnvalue_2 4.0)))
            ;[0.1085 0.5519 1 0.358] Modify gem emissive & light intensity based on distance from socket
            (`MeshComponent.SetScalarParameterValueOnMaterials` (`self.GemMesh`) "Emissive_master" (`KismetMathLibrary.FClamp` (* _returnvalue_2 7.5) 1.5 100000000.0))
            (else
              (`AudioComponent.FadeOut` (`self.GemLoop`) 1.0 0.0 "Linear")
              (`MeshComponent.SetScalarParameterValueOnMaterials` (`self.GemMesh`) "Emissive_master" 1.5))))))
    (:`then_2`
      (`self.AlignGlintEffect`)
      (`self.AlignShadow`))
    (:`then_3`)))

(event `self.ReceiveBeginPlay`
  (bind _interactiveeffect (`self.interactiveEffect`))
  (bind _gemmesh (`self.GemMesh`))
  ;[1 0.6939 0 0.499] Grab socket location that the gem belongs to for hum audio
  (`|ExecutionSequence`
    (:`then_0`
      (bind _outactors (`GameplayStatics.GetAllActorsOfClass` "/Game/Blueprints/BP_GemSocket.BP_GemSocket_C"))
      (for _array_element _outactors
        (if (== (`self.GemColor`) (`/Game/Blueprints/BP_GemSocket.GemColor` _array_element))
          (bind _socketlocation (`/Game/Blueprints/BP_GemSocket.Get Socket Location` _array_element))
          (set `self.SocketLocation` _socketlocation))))
    (:`then_1`
      ;;[0.13 0.7579 1 0.394] Spawn interactive object effect BP
      (bind _returnvalue (`|SpawnActorFromClass` "/Game/Blueprints/BP_InteractiveObjectsEffect_Outline.BP_InteractiveObjectsEffect_Outline_C" (`KismetMathLibrary.MakeTransform` (`SceneComponent.K2_GetComponentLocation` _gemmesh) (`SceneComponent.K2_GetComponentRotation` _gemmesh)) "Undefined" "OverrideRootScale" null null))
      (set `self.interactiveEffect` _returnvalue)
      (`self.K2_AttachToComponent` _interactiveeffect (`self.GemMesh`) "None" "KeepWorld" "KeepWorld" "KeepWorld" true)
      (`StaticMeshComponent.SetStaticMesh` (`/Game/Blueprints/BP_InteractiveObjectsEffect_Outline.outlineMesh` _interactiveeffect) (select `/Game/Blueprints/Enums/E_GemColor` (`self.GemColor`) :`NewEnumerator0` "/Game/Art/Gems/SM_Gem_Trillion.SM_Gem_Trillion" :`NewEnumerator1` "/Game/Art/Gems/SM_Gem_Emerald.SM_Gem_Emerald" :`NewEnumerator2` "/Game/Art/Gems/SM_Gem_Radiant.SM_Gem_Radiant" :!type "StaticMesh Object Reference")))))

(event `ActivateGem`
  (params (Delay :type "Float (double-precision)"))
  (bind _materialinstanceinner (`self.MaterialInstanceInner`))
  (bind _materialinstanceouter (`self.MaterialInstanceOuter`))
  ;[0 1 0.08557 0.316] Activate Gem - change colour saturation
  (`KismetSystemLibrary.Delay` Delay)
  (set `self.Active` true)
  (set `/Game/Blueprints/BP_InteractiveObjectsEffect_Outline.isActive` true (`self.interactiveEffect`))
  (bind (_direction _gemactivatealpha) (`Timeline|GemActivation`)
    (:`Update`
      (`|ExecutionSequence`
        (:`then_0`
          (`|ExecutionSequence`
            (:`then_0`
              (bind _returnvalue (`KismetMathLibrary.LinearColorLerp` (`self.InactiveColor`) (`self.ActiveGemColor`) _gemactivatealpha))
              (`MaterialInstanceDynamic.SetVectorParameterValue` _materialinstanceouter "BC_gem" _returnvalue))
            (:`then_1`
              (bind _returnvalue_2 (`KismetMathLibrary.LinearColorLerp` (`self.InactiveColor`) (`self.ActiveGemEdgeColor`) _gemactivatealpha))
              (`MaterialInstanceDynamic.SetVectorParameterValue` _materialinstanceouter "BC_edges" _returnvalue_2))))
        (:`then_1`
          (`|ExecutionSequence`
            (:`then_0`
              (`MaterialInstanceDynamic.SetVectorParameterValue` _materialinstanceinner "BC_gem" _returnvalue))
            (:`then_1`
              (`MaterialInstanceDynamic.SetVectorParameterValue` _materialinstanceinner "BC_edges" _returnvalue_2))))
        (:`then_2`
          (`MaterialInstanceDynamic.SetVectorParameterValue` (`self.MaterialInstanceShadow`) "CausticsColor" _returnvalue))))))

(event `StartHover`
  (bind (_returnvalue_x _returnvalue_y _returnvalue_z) (`KismetMathLibrary.BreakVector` (`SceneComponent.GetUpVector` (`self.GemMesh`))))
  (bind (_returnvalue_location _returnvalue_rotation _returnvalue_scale) (`KismetMathLibrary.BreakTransform` (`SceneComponent.K2_GetComponentToWorld` (`self.GemMesh`))))
  (bind (_returnvalue_x_2 _returnvalue_y_2 _returnvalue_z_2) (`KismetMathLibrary.BreakVector` (`SceneComponent.GetUpVector` (`self.GemMesh`))))
  ;[0.06274 0.3176 1] Gem Start Hover
  (`AudioComponent.Play` (`self.GemHoverLoop`) 0.0)
  (`PrimitiveComponent.SetSimulatePhysics` (`self.GemMesh`) false)
  ;[0.06274 0.3176 1] Move to plinth center Timeline
  (bind (_direction _lerptoplinthcenteralpha) (`Timeline|MoveGemToCenter` :!via `PlayFromStart` :!label _label)
    (:`Update`
      (`SceneComponent.K2_SetWorldTransform` (`self.GemMesh`) (`KismetMathLibrary.MakeTransform` (`KismetMathLibrary.VLerp` _returnvalue_location (`self.PlinthHoverLocation`) _lerptoplinthcenteralpha) (`KismetMathLibrary.RLerp` _returnvalue_rotation (`KismetMathLibrary.MakeRotator` 0.0 0.0 (+ _returnvalue_z_2 (stale _rotation))) _lerptoplinthcenteralpha true) _returnvalue_scale) false false))
    (:`Finished`
      ;[0.06274 0.3176 1] Hover and rotate loop
      (bind (_direction_2 _zoffset _rotation) (`Timeline|GemHoverUpDown` :!label _label_2)
        (:`Update`
          (`SceneComponent.K2_SetWorldLocation` (`self.GemMesh`) (+ (`self.PlinthHoverLocation`) (`KismetMathLibrary.MakeVector` 0.0 0.0 _zoffset)) false false)
          (`SceneComponent.K2_SetWorldRotation` (`self.GemMesh`) (`KismetMathLibrary.MakeRotator` _returnvalue_x _returnvalue_y (+ _returnvalue_z _rotation)) false false))))))

(event `StopHover`
  (bind _gemmesh (`self.GemMesh`))
  ;[0.06274 0.3176 1] GemStopHover
  (if (`self.Held`)
    (`PrimitiveComponent.SetSimulatePhysics` _gemmesh false)
    (else
      (`PrimitiveComponent.SetSimulatePhysics` _gemmesh true)))
  (`AudioComponent.Stop` (`self.GemHoverLoop`))
  (`|ExecutionSequence`
    (:`then_0`
      (goto _label :!via `Stop`))
    (:`then_1`
      (goto _label_2 :!via `Stop`))))

(event `self.UxtGenericManipulator.OnEnterGrabFocus`
  (params (Grabbable :type "UxtGrabTargetComponent Object Reference") (Pointer :type "UxtNearPointerComponent Object Reference"))
  ;[1 0 0.1939 0.352] Grab Focus
  (set `/Game/Blueprints/BP_InteractiveObjectsEffect_Outline.grabFocus` true (`self.interactiveEffect`))
  (if (`self.Active`)
    (`self.ScaleUp`)))

(event `Respawn`
  (bind _gemmesh (`self.GemMesh`))
  ;[0 0.526 1 0.415] Respawn after dropped off side
  (`SceneComponent.K2_SetWorldLocation` _gemmesh (`self.SpawnLocation`) false false)
  (`SceneComponent.K2_SetWorldRotation` _gemmesh (`KismetMathLibrary.RandomRotator` false) false false)
  (`SceneComponent.K2_SetWorldRotation` :`self` (`self.SmokeParticles`))
  ;;[1 1 1 1 15] Remove momentum
  (`PrimitiveComponent.SetSimulatePhysics` _gemmesh false)
  (`PrimitiveComponent.SetSimulatePhysics` _gemmesh true)
  (`AudioComponent.Play` (`self.GemRespawn`) 0.0)
  (`ActorComponent.Activate` (`self.SmokeParticles`) false))

(event `ScaleUp`
  ;[1 0.8443 0 0.342] Interactive Scaling
  (bind (_direction _scale) (`Timeline|GrabFocusScaleTimeline` :!label _label_3)
    (:`Update`
      (`SceneComponent.SetRelativeScale3D` (`self.GemMesh`) (`KismetMathLibrary.Conv_DoubleToVector` (`KismetMathLibrary.Lerp` 1.0 1.125 _scale))))))

(event `ScaleDown`
  ;[1 0.8443 0 0.342] Interactive Scaling
  (goto _label_3 :!via `Reverse`))

(event `self.UxtGenericManipulator.OnExitGrabFocus`
  (params (Grabbable :type "UxtGrabTargetComponent Object Reference") (Pointer :type "UxtNearPointerComponent Object Reference"))
  ;[1 0 0.1939 0.352] Grab Focus
  (set `/Game/Blueprints/BP_InteractiveObjectsEffect_Outline.grabFocus` false (`self.interactiveEffect`))
  (`self.ScaleDown`))

(event `/Game/Framework/BP_GazeTriggerInterface.OnGazeBegin`
  ;[0.1057 0.17 0.3438 0.352] Gaze detection
  (`ActorComponent.Activate` (`self.ParticleSystem`) false)
  (`MeshComponent.SetScalarParameterValueOnMaterials` (`self.GemMesh`) "Glint" 1.0)
  (set `/Game/Blueprints/BP_InteractiveObjectsEffect_Outline.isLookedAt` true (`self.interactiveEffect`)))

(event `self.UxtGenericManipulator.OnBeginGrab`
  (params (Grabbable :type "UxtGrabTargetComponent Object Reference") (GrabPointer :type "UxtGrabPointerData Structure"))
  ;[1 0.1564 0 0.363] Begin and end grab
  (if (not (`self.Inserted`))
    (set `self.Held` true)
    (`PrimitiveComponent.SetSimulatePhysics` (`self.GemMesh`) false)
    (`/Game/Blueprints/BP_GlowHintComponent.DeactivateParticleSystem` (`self.BP_GlowHintComponent`))
    (set `/Game/Blueprints/BP_InteractiveObjectsEffect_Outline.isGrabbed` true (`self.interactiveEffect`))
    (`self.ScaleDown`)
    (`AudioComponent.Play` (`self.Gem_Grab`) 0.0)))

(event `/Game/Framework/BP_GazeTriggerInterface.OnGazeEnd`
  ;[0.1057 0.17 0.3438 0.352] Gaze detection
  (`ActorComponent.Deactivate` (`self.ParticleSystem`))
  (`MeshComponent.SetScalarParameterValueOnMaterials` (`self.GemMesh`) "Glint" 0.0)
  (set `/Game/Blueprints/BP_InteractiveObjectsEffect_Outline.isLookedAt` false (`self.interactiveEffect`)))

(event `self.UxtGenericManipulator.OnEndGrab`
  (params (Grabbable :type "UxtGrabTargetComponent Object Reference") (GrabPointer :type "UxtGrabPointerData Structure"))
  ;[1 0.1564 0 0.363] Begin and end grab
  (if (not (`self.Inserted`))
    (set `self.Held` false)
    (`PrimitiveComponent.SetSimulatePhysics` (`self.GemMesh`) true)
    (set `/Game/Blueprints/BP_InteractiveObjectsEffect_Outline.isGrabbed` false (`self.interactiveEffect`))
    (`AudioComponent.Play` (`self.Gem_Release`) 0.0)))

(event `self.ActivateHint`
  (bind _bp_glowhintcomponent (`self.BP_GlowHintComponent`))
  ;[0 0 0] Activate/Deactivate hint effect
  (if (and (not (`self.Inserted`)) (`self.Active`) (not (`self.Held`)))
    (`/Game/Blueprints/BP_GlowHintComponent.ActivateOutliner` _bp_glowhintcomponent (`self.GemMesh`))
    (`/Game/Blueprints/BP_GlowHintComponent.ActivateParticleSystem` _bp_glowhintcomponent)))

(event `self.DeactivateHint`
  (bind _bp_glowhintcomponent (`self.BP_GlowHintComponent`))
  ;[0 0 0] Activate/Deactivate hint effect
  (`/Game/Blueprints/BP_GlowHintComponent.DeactivateOutliner` _bp_glowhintcomponent (`self.GemMesh`))
  (`/Game/Blueprints/BP_GlowHintComponent.DeactivateParticleSystem` _bp_glowhintcomponent))

(event `Event InsertGem`
  (bind _returnvalue (+ (`self.SocketLocation`) (* (`KismetMathLibrary.GetForwardVector` (`self.SocketRotation`)) (`self.DistanceBeforeInsert`))))
  ;[1 0 0] Needs Cleanup
  (if (not (`self.AnimationTriggered`))
    (set `self.Inserted` true)
    (set `/Game/Blueprints/BP_InteractiveObjectsEffect_Outline.isActive` false (`self.interactiveEffect`))
    (`self.DeactivateHint`)
    (`UxtGrabTargetComponent.ForceEndGrab` (`self.UxtGenericManipulator`))
    (set `UxtGenericManipulatorComponent.ManipulationModes` 0 (`self.UxtGenericManipulator`))
    ;;[0 1 0.1757] Anim play speed
    (`TimelineComponent.SetPlayRate` (`self.Align`) 5.0)
    (`TimelineComponent.SetPlayRate` (`self.Movein`) 5.0)
    (set `self.AnimationTriggered` true)
    ;;[0.3694 1 0.6763] Disable physics
    (`PrimitiveComponent.SetSimulatePhysics` (`self.GemMesh`) false)
    (set `self.StartPosition` (`SceneComponent.K2_GetComponentLocation` (`self.GemMesh`)))
    (set `self.StartRotation` (`SceneComponent.K2_GetComponentRotation` (`self.GemMesh`)))
    ;;[1 0.3884 0.2584 0.504] Gem ANIMATION - spin and landing
    (bind (_direction _newtrack_0) (`Timeline|Align`)
      (:`Update`
        (`SceneComponent.K2_SetWorldLocationAndRotation` (`self.GemMesh`) (`KismetMathLibrary.VLerp` (`self.StartPosition`) _returnvalue _newtrack_0) (`KismetMathLibrary.RLerp` (`self.StartRotation`) (`self.SocketRotation`) _newtrack_0) false false))
      (:`Finished`
        (`AudioComponent.Play` (`self.GemMoveIn`) 0.0)
        (bind (_direction_2 _newtrack_0_2) (`Timeline|Movein` :!via `PlayFromStart`)
          (:`Update`
            (`SceneComponent.K2_SetWorldLocation` (`self.GemMesh`) (`KismetMathLibrary.VLerp` _returnvalue (+ (`self.SocketLocation`) (* (`KismetMathLibrary.GetForwardVector` (`self.SocketRotation`)) 0.1)) _newtrack_0_2) false false))
          (:`Finished`
            (`AudioComponent.Play` (`self.GemSnap`) 0.0)
            ;[0.8916 0.2746 1 0.384] EmissiveEvents
            (switch `/Game/Blueprints/Enums/E_GemColor` (`self.GemColor`)
              (:`NewEnumerator0`
                (bind _returnvalue_2 (`GameplayStatics.GetActorOfClass` "/Game/Blueprints/Islands/BP_Island02.BP_Island02_C"))
                (`/Game/Blueprints/Islands/BP_Island02.RedGemEmissive` _returnvalue_2))
              (:`NewEnumerator1`
                (bind _returnvalue_3 (`GameplayStatics.GetActorOfClass` "/Game/Blueprints/Islands/BP_Island02.BP_Island02_C"))
                (`/Game/Blueprints/Islands/BP_Island02.GreenGemEmissive` _returnvalue_3))
              (:`NewEnumerator2`
                (bind _returnvalue_4 (`GameplayStatics.GetActorOfClass` "/Game/Blueprints/Islands/BP_Island02.BP_Island02_C"))
                (`/Game/Blueprints/Islands/BP_Island02.BlueGemEmissive` _returnvalue_4)))))))))

(fn `AlignGlintEffect`
  (`SceneComponent.K2_SetWorldRotation` (`self.Source_GlintEffect`) (`KismetMathLibrary.FindLookAtRotation` (`SceneComponent.K2_GetComponentLocation` (`self.Source_GlintEffect`)) (`SceneComponent.K2_GetComponentLocation` (`PlayerCameraManager.TransformComponent` (`GameplayStatics.GetPlayerCameraManager` 0)))) false false)
  (return))

(fn `AlignShadow`)

(fn `IsGrabFocusable`
  (params (Primitive :type "PrimitiveComponent Object Reference"))
  (returns (ReturnValue :type Boolean))
  (return false))

(fn `ScaleInputOnDistance`
  (params (GemMesh :type "SceneComponent Object Reference") (ScaleAmmount :type "Float (double-precision)") (StartScale :type "Vector Structure") (DistanceBeforeScalingStarts :type "Float (double-precision)"))
  (bind _returnvalue (`SceneComponent.K2_GetComponentLocation` GemMesh))
  (bind _returnvalue_2 (`SceneComponent.K2_GetComponentLocation` GemMesh))
  (bind _returnvalue_3 (`KismetMathLibrary.VLerp` StartScale (* StartScale ScaleAmmount) (`self.DistanceFromHand`)))
  (if (`HeadMountedDisplayFunctionLibrary.IsHeadMountedDisplayConnected`)
    ;[0.1039 0.7373 1 0.394] Get distance from closest UXT Hand
    (bind (_outorientation _outposition) (`UxtHandTrackingFunctionLibrary.GetHandJointState` "Left" "IndexTip"))
    (bind (_outorientation_2 _outposition_2) (`UxtHandTrackingFunctionLibrary.GetHandJointState` "Right" "IndexTip"))
    (bind _returnvalue_4 (`KismetMathLibrary.MapRangeClamped` (`KismetMathLibrary.Vector_Distance` _returnvalue_2 _outposition) DistanceBeforeScalingStarts 0.0 0.0 1.0))
    (bind _returnvalue_5 (`KismetMathLibrary.MapRangeClamped` (`KismetMathLibrary.Vector_Distance` _returnvalue_2 _outposition_2) DistanceBeforeScalingStarts 0.0 0.0 1.0))
    (if (< _returnvalue_4 _returnvalue_5)
      (set `self.DistanceFromHand` _returnvalue_5)
      (else
        (set `self.DistanceFromHand` _returnvalue_4)))
    (`SceneComponent.SetWorldScale3D` GemMesh _returnvalue_3)
    (else
      ;[0 1 0.5136 0.332] Get distance from closest simulated UXT hand (Editor only)
      (bind _returnvalue_6 (`GameplayStatics.GetActorOfClass` "/Script/UXToolsInputSimulation.UxtInputSimulationActor"))
      (bind _returnvalue_7 (`KismetMathLibrary.MapRangeClamped` (`KismetMathLibrary.Vector_Distance` _returnvalue (`SceneComponent.K2_GetComponentLocation` (`UxtInputSimulationActor.RightHand` _returnvalue_6))) DistanceBeforeScalingStarts 0.0 0.0 1.0))
      (bind _returnvalue_8 (`KismetMathLibrary.MapRangeClamped` (`KismetMathLibrary.Vector_Distance` _returnvalue (`SceneComponent.K2_GetComponentLocation` (`UxtInputSimulationActor.LeftHand` _returnvalue_6))) DistanceBeforeScalingStarts 0.0 0.0 1.0))
      (if (< _returnvalue_7 _returnvalue_8)
        (set `self.DistanceFromHand` _returnvalue_8)
        (else
          (set `self.DistanceFromHand` _returnvalue_7)))
      (`SceneComponent.SetWorldScale3D` GemMesh _returnvalue_3))))

(fn `SetOverlappingPlinth`
  (params (Overlapping :type Boolean) (PlinthHoverLocation :type "Vector Structure"))
  (set `self.OverlappingPlinth` Overlapping)
  (set `self.PlinthHoverLocation` PlinthHoverLocation))

(fn `UserConstructionScript`
  (bind _inactivecolor (`self.InactiveColor`))
  (`|ExecutionSequence`
    (:`then_0`
      ;[1 0.7085 0 0.53] Set respawn to original location
      (set `self.SpawnLocation` (+ (`SceneComponent.K2_GetComponentLocation` (`self.GemMesh`)) (0.0 0.0 8.0))))
    (:`then_1`
      ;[1 0.5787 0 0.499] Record original scale
      (set `self.GemStartScale` (`SceneComponent.K2_GetComponentScale` (`self.GemMesh`))))
    (:`then_2`
      ;[0.343 0.9701 1 0.488] Set static meshs
      (`StaticMeshComponent.SetStaticMesh` (`self.GemMesh`) (select `/Game/Blueprints/Enums/E_GemColor` (`self.GemColor`) :`NewEnumerator0` "/Game/Art/Gems/SM_Gem_Trillion.SM_Gem_Trillion" :`NewEnumerator1` "/Game/Art/Gems/SM_Gem_Emerald.SM_Gem_Emerald" :`NewEnumerator2` "/Game/Art/Gems/SM_Gem_Radiant.SM_Gem_Radiant" :!type "StaticMesh Object Reference")))
    (:`then_3`
      (`|ExecutionSequence`
        (:`then_0`
          ;[0.2304 0.3524 1 0.295] Outer Material Setup
          (bind _returnvalue (`KismetMaterialLibrary.CreateDynamicMaterialInstance` (select `/Game/Blueprints/Enums/E_GemColor` (`self.GemColor`) :`NewEnumerator0` "/Game/Art/Gems/MI_Gem_Trillion_out.MI_Gem_Trillion_out" :`NewEnumerator1` "/Game/Art/Gems/MI_Gem_Emerald_out.MI_Gem_Emerald_out" :`NewEnumerator2` "/Game/Art/Gems/MI_Gem_Radiant_out.MI_Gem_Radiant_out" :!type "MaterialInterface Object Reference") "OuterMat"))
          (bind _output_get (set `self.MaterialInstanceOuter` _returnvalue))
          (`|ExecutionSequence`
            (:`then_0`
              (bind _returnvalue_2 (`MaterialInstanceDynamic.K2_GetVectorParameterValue` _output_get "BC_gem"))
              (set `self.ActiveGemColor` _returnvalue_2)
              (`MaterialInstanceDynamic.SetVectorParameterValue` _output_get "BC_gem" (`self.InactiveColor`)))
            (:`then_1`
              (bind _returnvalue_3 (`MaterialInstanceDynamic.K2_GetVectorParameterValue` _output_get "BC_edges"))
              (set `self.ActiveGemEdgeColor` _returnvalue_3)
              (`MaterialInstanceDynamic.SetVectorParameterValue` _output_get "BC_edges" (`self.InactiveColor`)))
            (:`then_2`
              (`PrimitiveComponent.SetMaterial` (`self.GemMesh`) (select `/Game/Blueprints/Enums/E_GemColor` (`self.GemColor`) :`NewEnumerator0` 1 :`NewEnumerator1` 1) (`self.MaterialInstanceOuter`)))))
        (:`then_1`
          ;[0.1713 0.7989 1 0.514] Inner Material Setup
          (bind _returnvalue_4 (`KismetMaterialLibrary.CreateDynamicMaterialInstance` (select `/Game/Blueprints/Enums/E_GemColor` (`self.GemColor`) :`NewEnumerator0` "/Game/Art/Gems/MI_Gem_Trillion_out.MI_Gem_Trillion_out" :`NewEnumerator1` "/Game/Art/Gems/MI_Gem_Emerald_out.MI_Gem_Emerald_out" :`NewEnumerator2` "/Game/Art/Gems/MI_Gem_Radiant_out.MI_Gem_Radiant_out" :!type "MaterialInterface Object Reference") "InnerMat"))
          (bind _output_get_2 (set `self.MaterialInstanceInner` _returnvalue_4))
          (`|ExecutionSequence`
            (:`then_0`
              (`MaterialInstanceDynamic.SetVectorParameterValue` _output_get_2 "BC_gem" _inactivecolor))
            (:`then_1`
              (`MaterialInstanceDynamic.SetVectorParameterValue` _output_get_2 "BC_edges" _inactivecolor))
            (:`then_2`
              (`PrimitiveComponent.SetMaterial` (`self.GemMesh`) (select `/Game/Blueprints/Enums/E_GemColor` (`self.GemColor`) :`NewEnumerator2` 1) (`self.MaterialInstanceInner`)))))
        (:`then_2`
          ;[0.1839 0.4844 0.1405 0.269] Shadow Material Setup
          (bind _returnvalue_5 (`KismetMaterialLibrary.CreateDynamicMaterialInstance` (select `/Game/Blueprints/Enums/E_GemColor` (`self.GemColor`) :`NewEnumerator0` "/Game/Art/Gems/MI_RedGemShadow.MI_RedGemShadow" :`NewEnumerator1` "/Game/Art/Gems/MI_GreenGemShadow.MI_GreenGemShadow" :`NewEnumerator2` "/Game/Art/Gems/MI_BlueGemShadow.MI_BlueGemShadow" :!type "MaterialInterface Object Reference") "DecalShadowMat"))
          (bind _output_get_3 (set `self.MaterialInstanceShadow` _returnvalue_5))
          (`MaterialInstanceDynamic.SetVectorParameterValue` _output_get_3 "CausticsColor" (`self.InactiveColor`)))
        (:`then_3`
          ;[0.2257 0.7778 1 0.514] Smoke color setup
          (`FXSystemComponent.SetColorParameter` (`self.SmokeParticles`) "Particle_Colour" (select `/Game/Blueprints/Enums/E_GemColor` (`self.GemColor`) :`NewEnumerator0` (make `LinearColor` 1.0 0.25 0.25 1.0) :`NewEnumerator1` (make `LinearColor` 0.25 1.0 0.32 1.0) :`NewEnumerator2` (make `LinearColor` 0.25 0.5 1.0 1.0))))))
    (:`then_4`
      ;[0.2158 0.7779 1 0.509] Set particle system param
      (`FXSystemComponent.SetActorParameter` (`self.ParticleSystem`) "VertSurfaceActor" self))
    (:`then_5`
      ;[0.3659 0.5525 1 0.431] Set timeline rate
      (`TimelineComponent.SetPlayRate` (`self.GrabFocusScaleTimeline`) 3.5))))