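; Decorative floating block for hand-tracked interaction that bobs, spins and gets nudged away from the user's hand.
; A seeded stream randomizes its rotation, spin direction, bob speed and bob direction.
; On UXT grab focus, a timeline pushes it away from the nearer index fingertip, then returns it to its start location.
; A short delay throttles repeated pushes, and the fifth locks input until the timeline finishes.
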(event `self.ReceiveBeginPlay`
  (bind _stream (`self.stream`))
  (bind _returnvalue (/ (`self.offsetAmount`) 2.0))
  (bind _returnvalue_2 (/ (`self.offsetAmount`) 2.0))
  (if (`self.active`)
    (`|ExecutionSequence`
      (:`then_0`
        ;[1 1 1] Idle motion
        (`TimelineComponent.SetPlayRate` (`self.floatingMotion`) (`KismetMathLibrary.RandomFloatInRangeFromStream` 0.02 (`self.speed`) _stream))
        (set `self.invertDirection` (`KismetMathLibrary.RandomBoolFromStream` _stream))
        (bind (_direction _lerp) (`Timeline|floatingMotion` :!via `PlayFromStart`)
          (:`Update`
            (`SceneComponent.K2_SetRelativeLocation` (`self.FloatingBlock`) (`KismetMathLibrary.SelectVector` (`KismetMathLibrary.VLerp` _returnvalue_2 (* _returnvalue_2 -1.0) _lerp) (`KismetMathLibrary.VLerp` (* _returnvalue -1.0) _returnvalue _lerp) (`self.invertDirection`)) false false))))
      (:`then_1`
        (set `self.initialLocation` (`SceneComponent.K2_GetComponentLocation` (`self.Scene`)))))))

(event `self.ReceiveTick`
  (params (DeltaSeconds :type "Float (single-precision)"))
  (bind _returnvalue (`SceneComponent.K2_GetComponentLocation` (`self.Scene`)))
  (bind _returnvalue_2 (/ (`self.offsetAmount`) 2.0))
  ;[1 1 1] debug
  (if (`self.debugLocation`)
    (`KismetSystemLibrary.DrawDebugSphere` (+ _returnvalue _returnvalue_2) 0.2 12 (struct :`R` 1.0 :`G` 1.0 :`B` 1.0 :`A` 1.0) 0.0 0.1)
    (`KismetSystemLibrary.DrawDebugSphere` (+ _returnvalue (* _returnvalue_2 -1.0)) 0.2 12 (struct :`R` 1.0 :`G` 1.0 :`B` 1.0 :`A` 1.0) 0.0 0.1)))

(event `self.UxtGrabTarget.OnEnterGrabFocus`
  (params (Grabbable :type "UxtGrabTargetComponent Object Reference") (Pointer :type "UxtNearPointerComponent Object Reference"))
  (bind _locationpriorwobble (`self.locationPriorWobble`))
  (bind _returnvalue (`SceneComponent.K2_GetComponentLocation` (`self.Scene`)))
  (bind _returnvalue_2 (`SceneComponent.K2_GetComponentLocation` (`self.Scene`)))
  (bind _returnvalue_3 (+ _locationpriorwobble (* (* (`KismetMathLibrary.Normal` (`self.wobbleDirection`)) -1.0) (`self.wobbleAmount`))))
  ;[1 1 1] Hands interaction
  (if (`self.active`)
    ;;[1 1 1] lets timeline finish when you trigger the wobble 5 times in a row
    (if (`self.canWobble`)
      (set `self.interactionsCounter` (+ (`self.interactionsCounter`) 1))
      (if (!= (`self.interactionsCounter`) 5)
        (set `self.canWobble` false) ; decreases interaction frequency allowed
        (`KismetSystemLibrary.Delay` 0.33)
        (set `self.canWobble` true)
        (else
          (set `self.canWobble` false) ; allows interaction logic to reset
        ))
      (`|ExecutionSequence`
        (:`then_0`
          ;;[1 1 1] gets distance of the closer hand
          (bind (_outorientation _outposition) (`UxtHandTrackingFunctionLibrary.GetHandJointState` "Left" "IndexIntermediate"))
          (bind (_outorientation_2 _outposition_2) (`UxtHandTrackingFunctionLibrary.GetHandJointState` "Right" "IndexIntermediate"))
          (set `self.leftHandCloser` (< (`KismetMathLibrary.Vector_Distance` _outposition _returnvalue_2) (`KismetMathLibrary.Vector_Distance` _outposition_2 _returnvalue_2))))
        (:`then_1`
          ;;[1 1 1] sets variables needed
          ;;;[1 1 1] calculates direction
          (if (`self.leftHandCloser`)
            (bind (_outorientation_3 _outposition_3) (`UxtHandTrackingFunctionLibrary.GetHandJointState` "Left" "IndexTip"))
            (set `self.wobbleDirection` (`KismetMathLibrary.GetDirectionUnitVector` _returnvalue _outposition_3))
            (else
              (bind (_outorientation_4 _outposition_4) (`UxtHandTrackingFunctionLibrary.GetHandJointState` "Right" "IndexTip"))
              (set `self.wobbleDirection` (`KismetMathLibrary.GetDirectionUnitVector` _returnvalue _outposition_4))))
          (set `self.locationPriorWobble` (`SceneComponent.K2_GetComponentLocation` (`self.Scene`)))
          (set `self.wobbleAmount` (`KismetMathLibrary.RandomFloatInRange` 0.75 1.5))
          (set `self.goBackToOriginalLoc` false))
        (:`then_2`
          ;;[1 1 1] Animates block
          (bind (_direction _lerp) (`Timeline|Timeline_0` :!via `PlayFromStart`)
            (:`Update`
              (`SceneComponent.K2_SetWorldLocation` (`self.Scene`) (`KismetMathLibrary.SelectVector` (`KismetMathLibrary.VLerp` (`self.initialLocation`) _returnvalue_3 _lerp) (`KismetMathLibrary.VLerp` _locationpriorwobble _returnvalue_3 _lerp) (`self.goBackToOriginalLoc`)) false false))
            (:`Finished`
              ;;[1 1 1] reset
              (set `self.canWobble` true)
              (set `self.interactionsCounter` 0))
            (:`pushCompletedEvent`
              (set `self.goBackToOriginalLoc` true))))))))

(fn `UserConstructionScript`
  (bind _randomxyrotation (`self.randomXYrotation`))
  (bind _stream (`self.stream`))
  (bind _rotationspeed (`self.rotationSpeed`))
  (`SceneComponent.K2_SetWorldRotation` (`self.FloatingBlock`) (`KismetMathLibrary.MakeRotator` (`KismetMathLibrary.SelectFloat` (`KismetMathLibrary.RandomFloatInRangeFromStream` 0.0 360.0 _stream) 0.0 _randomxyrotation) (`KismetMathLibrary.SelectFloat` (`KismetMathLibrary.RandomFloatInRangeFromStream` 0.0 360.0 _stream) 0.0 _randomxyrotation) (`KismetMathLibrary.RandomFloatInRangeFromStream` 0.0 360.0 _stream)) false false)
  (set `RotatingMovementComponent.RotationRate` (`KismetMathLibrary.MakeRotator` 0.0 0.0 (`KismetMathLibrary.SelectFloat` _rotationspeed (* _rotationspeed -1.0) (`KismetMathLibrary.RandomBoolFromStream` _stream))) (`self.RotatingMovement`)))