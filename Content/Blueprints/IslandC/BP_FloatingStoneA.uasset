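; Three-piece floating stone prop for IslandC that animates in and out on toggle and reacts to hands and bombs.
; While active, the first stone bobs on a timeline and the others chase its sockets with interpolation, the third also spinning.
; UXT grab focus nudges it away from the nearer hand, with throttled repeats, and nearby BP_Bomb explosions push it by distance.
; Deactivation snapshots current transforms to reverse smoothly to rest.
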(event `ActivationToggle`
  (params (active :type Boolean))
  (bind _floatingstonea_1 (`self.FloatingStoneA_1`))
  (bind _floatingstonea_2 (`self.FloatingStoneA_2`))
  (bind _floatingstonea_3 (`self.FloatingStoneA_3`))
  ;[1 1 1] Activate
  (if active
    (bind (_direction _lerp) (`Timeline|ActivationAnim` :!via `PlayFromStart` :!label _label)
      (:`Update`
        (`|ExecutionSequence`
          (:`then_0`
            (`SceneComponent.K2_SetRelativeLocation` (`self.FloatingStoneA_2`) (`KismetMathLibrary.VLerp` (`self.floatingStoneA2_deactiveRloc`) (`self.floatingStoneA2_activeRloc`) _lerp) false false)
            (`SceneComponent.SetRelativeScale3D` (`self.FloatingStoneA_3`) (`KismetMathLibrary.VLerp` (`self.floatingStoneA3_deactiveRscale`) (`self.floatingStoneA3_activeRscale`) _lerp)))
          (:`then_1`
            ;[1 1 1] Deactivation
            (if (not active)
              (`SceneComponent.K2_SetRelativeRotation` (`self.FloatingStoneA_1`) (`KismetMathLibrary.RLerp` (struct) (`self.floatingStoneA1_currentRotation`) _lerp true) false false)
              (`SceneComponent.K2_SetRelativeRotation` (`self.FloatingStoneA_2`) (`KismetMathLibrary.RLerp` (struct) (`self.floatingStoneA2_currentRotation`) _lerp true) false false)
              (`SceneComponent.K2_SetRelativeRotation` (`self.FloatingStoneA_3`) (`KismetMathLibrary.RLerp` (struct) (`self.floatingStoneA3_currentRotation`) _lerp true) false false)
              (`SceneComponent.K2_SetRelativeLocation` (`self.FloatingStoneA_1`) (`KismetMathLibrary.VLerp` (0.0 0.0 0.0) (`self.floatingStoneA1_currentLoc`) _lerp) false false)
              (`SceneComponent.K2_SetRelativeLocation` (`self.FloatingStoneA_3`) (`KismetMathLibrary.VLerp` (2.030877 0.0 0.0) (`self.floatingStoneA3_currentLoc`) _lerp) false false)))))
      (:`Finished`
        (if active
          (`self.StartIdle`)
          (set `self.activated` true)
          (set `self.initialLocationInteraction` (`SceneComponent.K2_GetComponentLocation` (`self.InteractionMotion`))))))
    (else
      (set `self.activated` false)
      (`self.Stop`)
      (set `self.floatingStoneA1_currentRotation` (`SceneComponent.RelativeRotation` _floatingstonea_1))
      (set `self.floatingStoneA2_currentRotation` (`SceneComponent.RelativeRotation` _floatingstonea_2))
      (set `self.floatingStoneA3_currentRotation` (`SceneComponent.RelativeRotation` _floatingstonea_3))
      (set `self.floatingStoneA1_currentLoc` (`SceneComponent.RelativeLocation` _floatingstonea_1))
      (set `self.floatingStoneA3_currentLoc` (`SceneComponent.RelativeLocation` _floatingstonea_3))
      (set `self.floatingStoneA2_activeRloc` (`SceneComponent.RelativeLocation` _floatingstonea_2))
      (goto _label :!via `ReverseFromEnd`))))

(event `StartIdle`
  ;[1 1 1] idle anim master
  (`TimelineComponent.SetPlayRate` (`self.IdleAnim`) 0.5)
  (bind (_direction _lerp) (`Timeline|IdleAnim` :!via `PlayFromStart` :!label _label_2)
    (:`Update`
      (`SceneComponent.K2_SetRelativeLocation` (`self.FloatingStoneA_1`) (`KismetMathLibrary.VLerp` (0.0 0.0 0.0) (`self.idleOffsetAmount`) _lerp) false false))))

(event `Stop`
  ;[1 1 1] idle anim master
  (goto _label_2 :!via `Stop`))

(event `self.ReceiveTick`
  (params (DeltaSeconds :type "Float (single-precision)"))
  (bind _floatingstonea_2 (`self.FloatingStoneA_2`))
  (bind _floatingstonea_3 (`self.FloatingStoneA_3`))
  (bind _floatingstonea_3_2 (`self.FloatingStoneA_3`))
  (bind _floatingstonea_2_2 (`self.FloatingStoneA_2`))
  (bind _relativelocation (`SceneComponent.RelativeLocation` _floatingstonea_3))
  (bind (_relativerotation_roll _relativerotation_pitch _relativerotation_yaw) (`KismetMathLibrary.BreakRotator` (`SceneComponent.RelativeRotation` _floatingstonea_3_2)))
  (bind _relativelocation_2 (`SceneComponent.RelativeLocation` _floatingstonea_2))
  (bind _returnvalue (`KismetMathLibrary.InverseTransformLocation` (`SceneComponent.K2_GetComponentToWorld` (`self.DefaultSceneRoot`)) (`SceneComponent.GetSocketLocation` (`self.FloatingStoneA_1`) "A2")))
  (bind _returnvalue_2 (`KismetMathLibrary.InverseTransformLocation` (`SceneComponent.K2_GetComponentToWorld` (`self.DefaultSceneRoot`)) (`SceneComponent.GetSocketLocation` (`self.FloatingStoneA_1`) "A3")))
  (bind (_returnvalue_x _returnvalue_y _returnvalue_z) (`KismetMathLibrary.BreakVector` (`KismetMathLibrary.VInterpTo` _relativelocation _returnvalue_2 (`GameplayStatics.GetWorldDeltaSeconds`) 3.25)))
  (if (`self.activated`)
    ;[1 1 1] blocks follow
    (`|ExecutionSequence`
      (:`then_0`)
      (:`then_1`
        ;;[1 1 1] block 2
        (`SceneComponent.K2_SetRelativeRotation` _floatingstonea_2_2 (`KismetMathLibrary.RInterpTo` (`SceneComponent.RelativeRotation` _floatingstonea_2_2) (`SceneComponent.RelativeRotation` (`self.FloatingStoneA_1`)) (`GameplayStatics.GetWorldDeltaSeconds`) 1.5) false false)
        (if (not (== _relativelocation_2 _returnvalue :`ErrorTolerance` 0.02))
          (`SceneComponent.K2_SetRelativeLocation` _floatingstonea_2 (`KismetMathLibrary.VInterpTo` _relativelocation_2 _returnvalue (`GameplayStatics.GetWorldDeltaSeconds`) 1.5) false false)))
      (:`then_2`
        ;;[1 1 1] block 3
        (`SceneComponent.K2_SetRelativeRotation` _floatingstonea_3_2 (`KismetMathLibrary.MakeRotator` _relativerotation_roll _relativerotation_pitch (+ _relativerotation_yaw -0.1)) false false)
        (if (not (== _relativelocation _returnvalue_2 :`ErrorTolerance` 0.01))
          (`SceneComponent.K2_SetRelativeLocation` _floatingstonea_3 (`KismetMathLibrary.MakeVector` _returnvalue_x _returnvalue_y _returnvalue_z) false false))))))

(event `self.UxtGrabTarget.OnEnterGrabFocus`
  (params (Grabbable :type "UxtGrabTargetComponent Object Reference") (Pointer :type "UxtNearPointerComponent Object Reference"))
  (bind _locationpriorwobble (`self.locationPriorWobble`))
  (bind _returnvalue (`SceneComponent.K2_GetComponentLocation` (`self.InteractionMotion`)))
  (bind _returnvalue_2 (`SceneComponent.K2_GetComponentLocation` (`self.InteractionMotion`)))
  (bind _returnvalue_3 (+ _locationpriorwobble (* (* (`KismetMathLibrary.Normal` (`self.wobbleDirection`)) -1.0) (`self.wobbleAmount`))))
  ;[1 1 1] Hands interaction
  (if (`self.activated`)
    ;;[1 1 1] lets timeline finish when you trigger the wobble 5 times in a row
    (if (`self.canWobble`)
      (set `self.interactionsCounter` (+ (`self.interactionsCounter`) 1))
      (if (!= (`self.interactionsCounter`) 4)
        (set `self.canWobble` false) ; decreases interaction frequency allowed
        (`KismetSystemLibrary.Delay` 0.33)
        (set `self.canWobble` true)
        (else
          (set `self.canWobble` false) ; allows interaction logic to reset
        ))
      (`|ExecutionSequence`
        (:`then_0`
          ;;[1 1 1] gets distance of the closer hand
          (bind (_outorientation _outposition) (`UxtHandTrackingFunctionLibrary.GetHandJointState` "Left" "IndexIntermediate"))
          (bind (_outorientation_2 _outposition_2) (`UxtHandTrackingFunctionLibrary.GetHandJointState` "Right" "IndexIntermediate"))
          (set `self.leftHandCloser` (< (`KismetMathLibrary.Vector_Distance` _outposition _returnvalue_2) (`KismetMathLibrary.Vector_Distance` _outposition_2 _returnvalue_2))))
        (:`then_1`
          ;;[1 1 1] sets variables needed
          ;;;[1 1 1] calculates direction
          (if (`self.leftHandCloser`)
            (bind (_outorientation_3 _outposition_3) (`UxtHandTrackingFunctionLibrary.GetHandJointState` "Left" "IndexTip"))
            (set `self.wobbleDirection` (`KismetMathLibrary.GetDirectionUnitVector` _returnvalue _outposition_3))
            (else
              (bind (_outorientation_4 _outposition_4) (`UxtHandTrackingFunctionLibrary.GetHandJointState` "Right" "IndexTip"))
              (set `self.wobbleDirection` (`KismetMathLibrary.GetDirectionUnitVector` _returnvalue _outposition_4))))
          (set `self.locationPriorWobble` (`SceneComponent.K2_GetComponentLocation` (`self.InteractionMotion`)))
          (set `self.wobbleAmount` (`KismetMathLibrary.RandomFloatInRange` 0.25 0.75))
          (set `self.goBackToOriginalLoc` false))
        (:`then_2`
          ;;[1 1 1] Animates block
          (bind (_direction _lerp) (`Timeline|Timeline_0` :!via `PlayFromStart` :!label _label_3)
            (:`Update`
              (`SceneComponent.K2_SetWorldLocation` (`self.InteractionMotion`) (`KismetMathLibrary.SelectVector` (`KismetMathLibrary.VLerp` (`self.initialLocationInteraction`) _returnvalue_3 _lerp) (`KismetMathLibrary.VLerp` _locationpriorwobble _returnvalue_3 _lerp) (`self.goBackToOriginalLoc`)) false false))
            (:`Finished`
              ;;[1 1 1] reset
              (set `self.canWobble` true)
              (set `self.interactionsCounter` 0))
            (:`pushCompletedEvent`
              (set `self.goBackToOriginalLoc` true))))))))

(event `self.ReceiveBeginPlay`
  ;[1 1 1] Hands interaction
  (bind _returnvalue (`GameplayStatics.GetActorOfClass` "/Game/Blueprints/BP_Bomb.BP_Bomb_C"))
  (add `/Game/Blueprints/BP_Bomb.Explosion` _returnvalue (delegate `Explosion`)))

(event `Explosion`
  (params (bombLocation :type "Vector Structure"))
  (bind _returnvalue (`SceneComponent.K2_GetComponentLocation` (`self.InteractionMotion`)))
  (bind _returnvalue_2 (`KismetMathLibrary.Vector_Distance` bombLocation _returnvalue))
  ;[1 1 1] Hands interaction
  (if (< _returnvalue_2 30.0)
    (set `self.wobbleDirection` (* (`KismetMathLibrary.GetDirectionUnitVector` bombLocation _returnvalue) -1.0))
    (set `self.locationPriorWobble` (`SceneComponent.K2_GetComponentLocation` (`self.InteractionMotion`)))
    (set `self.wobbleAmount` (`KismetMathLibrary.Lerp` 1.0 6.0 (- 1.0 (`KismetMathLibrary.MapRangeClamped` (`KismetMathLibrary.FClamp` _returnvalue_2 0.0 30.0) 0.0 30.0 0.0 1.0))))
    (set `self.goBackToOriginalLoc` false)
    (goto _label_3 :!via `PlayFromStart`)))

(fn `UserConstructionScript`)