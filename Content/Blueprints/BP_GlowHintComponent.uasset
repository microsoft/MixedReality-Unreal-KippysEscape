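; Glow hint component that highlights a target mesh with a post-process outline and an attached glow particle effect, each toggled separately.
; The outliner functions store the mesh and start a looping timer that fades MPC_Outliner's global OffOn parameter, enabling custom depth until fade-out completes.
; The particle functions attach PS_Glow_v02 to that stored mesh, then deactivate it and destroy it after a short delay.
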(event `DestroyEmitter`
  (`KismetSystemLibrary.Delay` 1.5)
  (`self.K2_DestroyComponent` (`self.emitter`)))

(fn `ActivateOutliner`
  (params (TargetMesh :type "StaticMeshComponent Object Reference"))
  (set `self.targetMesh` TargetMesh)
  (if (not (`self.outlinerActive`))
    (set `self.outlinerActive` true)
    (`PrimitiveComponent.SetRenderCustomDepth` (`self.targetMesh`) true)
    (`KismetSystemLibrary.K2_PauseTimer` null "UpdatePPmaterial")
    (`KismetSystemLibrary.K2_ClearTimer` null "UpdatePPmaterial")
    (`KismetSystemLibrary.K2_SetTimer` null "UpdatePPmaterial" (`GameplayStatics.GetWorldDeltaSeconds`) true)))

(fn `ActivateParticleSystem`
  (if (not (`self.particleSystemActive`))
    (set `self.particleSystemActive` true)
    (bind _returnvalue (`GameplayStatics.SpawnEmitterAttached` "/Game/Effects/Glow/PS_Glow_v02.PS_Glow_v02" (`self.targetMesh`) "None" (`self.emitterOffset`) (struct) (`self.emitterScale`) "SnapToTarget"))
    (set `self.emitter` _returnvalue)))

(fn `DeactivateOutliner`
  (params (TargetMesh :type "StaticMeshComponent Object Reference"))
  (set `self.targetMesh` TargetMesh)
  (if (`self.outlinerActive`)
    (`KismetSystemLibrary.K2_PauseTimer` null "UpdatePPmaterial")
    (`KismetSystemLibrary.K2_ClearTimer` null "UpdatePPmaterial")
    (`KismetSystemLibrary.K2_SetTimer` null "UpdatePPmaterial" (`GameplayStatics.GetWorldDeltaSeconds`) true)
    (set `self.outlinerActive` false)))

(fn `DeactivateParticleSystem`
  (if (`self.particleSystemActive`)
    (`self.Deactivate` (`self.emitter`))
    (`self.DestroyEmitter`)
    (set `self.particleSystemActive` false)))

(fn `UpdatePPmaterial`
  (bind _returnvalue (`GameplayStatics.GetWorldDeltaSeconds`))
  (bind _returnvalue_2 (`KismetMathLibrary.FInterpTo_Constant` (`self.Outliner_OnOff_Lerp`) 0.0 _returnvalue 0.75))
  (bind _returnvalue_3 (`KismetMathLibrary.FInterpTo_Constant` (`self.Outliner_OnOff_Lerp`) 1.0 _returnvalue 0.5))
  ;[1 1 1] Update material collection parameter (used in the post process)
  (if (`self.outlinerActive`)
    (set `self.Outliner_OnOff_Lerp` _returnvalue_3)
    (`KismetMaterialLibrary.SetScalarParameterValue` "/Game/Materials/PostProcess/Outliner/MPC_Outliner.MPC_Outliner" "OffOn" _returnvalue_3)
    ;[1 1 1] stops function when value reaches target
    (if (`KismetMathLibrary.NearlyEqual_FloatFloat` (`self.Outliner_OnOff_Lerp`) 1.0)
      (`KismetSystemLibrary.K2_PauseTimer` null "UpdatePPmaterial" :!label _label)
      (`KismetSystemLibrary.K2_ClearTimer` null "UpdatePPmaterial"))
    (else
      (set `self.Outliner_OnOff_Lerp` _returnvalue_2)
      (`KismetMaterialLibrary.SetScalarParameterValue` "/Game/Materials/PostProcess/Outliner/MPC_Outliner.MPC_Outliner" "OffOn" _returnvalue_2)
      (if (`KismetMathLibrary.NearlyEqual_FloatFloat` (`self.Outliner_OnOff_Lerp`))
        (`PrimitiveComponent.SetRenderCustomDepth` (`self.targetMesh`) false)
        (goto _label)))))