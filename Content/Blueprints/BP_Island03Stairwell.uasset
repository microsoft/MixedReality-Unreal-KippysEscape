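; Island 03 stairwell Blueprint with rubble piles that bombs clear.
; BombDetonate tests the bomb mesh against trigger areas: successive hits in the main area clear right then left rubble, setting RubbleCleared once both are gone.
; Two optional piles have their own triggers; clearing any pile hides it with a crumble sound and particles.
; The construction script gives six rock meshes one shared dynamic material with darkened colour and emissive sphere mask.
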(event `BombDetonate`
  (params (BombMeshRef :type "StaticMeshComponent Object Reference"))
  (set `self.BombRef` BombMeshRef)
  (`|ExecutionSequence`
    (:`then_0`
      (if (`PrimitiveComponent.IsOverlappingComponent` (`self.DetonateArea`) (`self.BombRef`))
        (if (not (`self.RightRubbleCleared`))
          (`GameplayStatics.PlaySoundAtLocation` "/Game/Sounds/Rubble/SC_RubbleCrumble.SC_RubbleCrumble" (`SceneComponent.K2_GetComponentLocation` (`self.RightRubble_GRP`)) (struct) 1.0 1.0 0.0 "/Game/Sounds/DefaultAttenuationSettings.DefaultAttenuationSettings" null null)
          (`SceneComponent.SetVisibility` (`self.RightRubble_GRP`) false true)
          (`ActorComponent.Activate` (`self.P_RubbleRight`) false)
          (`ActorComponent.Activate` (`self.P_RubbleRight2`) false)
          (set `self.RightRubbleCleared` true)
          (else
            (`GameplayStatics.PlaySoundAtLocation` "/Game/Sounds/Rubble/SC_RubbleCrumble.SC_RubbleCrumble" (`SceneComponent.K2_GetComponentLocation` (`self.LeftRubble_GRP`)) (struct) 1.0 1.0 0.0 "/Game/Sounds/DefaultAttenuationSettings.DefaultAttenuationSettings" null null)
            (`SceneComponent.SetVisibility` (`self.LeftRubble_GRP`) false true)
            (`ActorComponent.Activate` (`self.P_RubbleLeft`) false)
            (set `self.LeftRubbleCleared` true)))
        (if (and (`self.LeftRubbleCleared`) (`self.RightRubbleCleared`))
          (set `self.RubbleCleared` true))))
    (:`then_1`
      (`|ExecutionSequence`
        (:`then_0`
          (if (`PrimitiveComponent.IsOverlappingComponent` (`self.OptionalRubbleLeftTrigger`) (`self.BombRef`))
            (`GameplayStatics.PlaySoundAtLocation` "/Game/Sounds/Rubble/SC_RubbleCrumble.SC_RubbleCrumble" (`SceneComponent.K2_GetComponentLocation` (`self.OptionalRubbleLeft_GRP`)) (struct) 1.0 1.0 0.0 "/Game/Sounds/DefaultAttenuationSettings.DefaultAttenuationSettings" null null)
            (`SceneComponent.SetVisibility` (`self.OptionalRubbleLeft_GRP`) false true)
            (`ActorComponent.Activate` (`self.P_OptionalRubbleLeft`) false)))
        (:`then_1`
          (if (`PrimitiveComponent.IsOverlappingComponent` (`self.OptionalRubbleRightTrigger`) (`self.BombRef`))
            (`GameplayStatics.PlaySoundAtLocation` "/Game/Sounds/Rubble/SC_RubbleCrumble.SC_RubbleCrumble" (`SceneComponent.K2_GetComponentLocation` (`self.OptionalRubbleRight_GRP`)) (struct) 1.0 1.0 0.0 "/Game/Sounds/DefaultAttenuationSettings.DefaultAttenuationSettings" null null)
            (`SceneComponent.SetVisibility` (`self.OptionalRubbleRight_GRP`) false true)
            (`ActorComponent.Activate` (`self.P_OptionalRubbleRight`) false)))))))

(fn `UserConstructionScript`
  (bind _returnvalue (`PrimitiveComponent.CreateDynamicMaterialInstance` (`self.SM_rocks`) 0 "/Game/Art/Rock/MI_rock.MI_rock" "None"))
  (bind _output_get (set `self.RockMat` _returnvalue))
  (`MaterialInstanceDynamic.SetScalarParameterValue` _output_get "UseEmissiveSphereMaskBool" 1.0)
  (`MaterialInstanceDynamic.SetScalarParameterValue` _output_get "BaseColourMultiplier" 0.2)
  (for _array_element (`|MakeArray` (`self.SM_rocks`) (`self.SM_rocks2`) (`self.SM_rocks3`) (`self.SM_rocks4`) (`self.SM_rocks5`) (`self.SM_rocks6`))
    (`PrimitiveComponent.SetMaterial` _array_element 0 (`self.RockMat`))))