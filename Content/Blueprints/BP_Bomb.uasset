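; Grabbable UXT bomb that arms when grabbed and explodes after a countdown, reporting the blast to the Island03 stairwell.
; A timeline drives emissive flashing, beeps and the explosion, after which the same actor resets hidden at its spawn point following a cooldown.
; Grab toggles physics and stops rotation, while gaze and grab focus feed a spawned outline effect actor, with focus also scaling the mesh.
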(event `self.ReceiveBeginPlay`
  (bind _bombmesh (`self.BombMesh`))
  (bind _interactiveeffect (`self.interactiveEffect`))
  (bind _interactiveeffect_2 (`self.interactiveEffect`))
  (`|ExecutionSequence`
    (:`then_0`
      ;[1 0.2817 0.1317 0.41] Delay bomb setup to ensure refs are set
      (`KismetSystemLibrary.Delay` 0.25)
      (`self.ArmBomb` true)
      (`self.WakeBomb` true)
      (bind _returnvalue (`GameplayStatics.GetActorOfClass` "/Game/Blueprints/BP_Island03Stairwell.BP_Island03Stairwell_C"))
      (set `self.StairRef` _returnvalue))
    (:`then_1`
      ;[1 1 1] Spawn interactive object effect BP
      (bind _returnvalue_2 (`|SpawnActorFromClass` "/Game/Blueprints/BP_InteractiveObjectsEffect_Outline.BP_InteractiveObjectsEffect_Outline_C" (`KismetMathLibrary.MakeTransform` (`SceneComponent.K2_GetComponentLocation` _bombmesh) (`SceneComponent.K2_GetComponentRotation` _bombmesh)) "Undefined" "OverrideRootScale" null null))
      (set `self.interactiveEffect` _returnvalue_2)
      (`self.K2_AttachToComponent` _interactiveeffect (`self.BombMesh`) "None" "KeepWorld" "KeepWorld" "KeepWorld" true)
      (`StaticMeshComponent.SetStaticMesh` (`/Game/Blueprints/BP_InteractiveObjectsEffect_Outline.outlineMesh` _interactiveeffect) "/Game/Art/BombMachine/SM_BombMachine_Explosive_Outline.SM_BombMachine_Explosive_Outline")
      (set `/Game/Blueprints/BP_InteractiveObjectsEffect_Outline.thicknessActiveTarget` 0.35 _interactiveeffect_2)
      (set `/Game/Blueprints/BP_InteractiveObjectsEffect_Outline.thicknessFocusTarget` 0.6 _interactiveeffect_2)
      (set `/Game/Blueprints/BP_InteractiveObjectsEffect_Outline.interpSpeedDisappear` 100.0 _interactiveeffect_2))))

(event `ArmBomb`
  (params (ResetBomb :type Boolean))
  (bind _bombmesh (`self.BombMesh`))
  (bind _rotatingmovement (`self.RotatingMovement`))
  (if ResetBomb
    ;[1 0.675 0 0.556] Reset bomb to base position
    (`ActorComponent.Activate` _rotatingmovement false)
    (set `RotatingMovementComponent.RotationRate` (`KismetMathLibrary.MakeRotator` (`KismetMathLibrary.RandomFloatInRange` 10.0 20.0) (`KismetMathLibrary.RandomFloatInRange` 25.0 50.0) (`KismetMathLibrary.RandomFloatInRange` 20.0 50.0)) _rotatingmovement)
    (`SceneComponent.K2_SetWorldLocation` _bombmesh (`self.SpawnLocation`) false false)
    (`PrimitiveComponent.SetEnableGravity` _bombmesh false)
    (`PrimitiveComponent.SetSimulatePhysics` _bombmesh false)
    (set `self.BombArmedToBlow` false)
    (elif (`self.IsBombAsleep`)
      (set `self.BombAlreadyExists` true)
      (if (not (`self.BombArmedToBlow`))
        (set `self.BombArmedToBlow` true)
        ;[1 0 0.005617 0.384] Bomb Flash countdown
        (bind (_direction _bomblights) (`Timeline|BombCountdown` :`NewTime` 4.7 :!via `PlayFromStart` :!label _label)
          (:`Update`
            (`MaterialInstanceDynamic.SetScalarParameterValue` (`self.BombMat`) "EmissiveIntensity" _bomblights))
          (:`Beep`
            (`AudioComponent.Play` (`self.Beep`) 0.0))
          (:`Explosion`
            (`AudioComponent.Play` (`self.GDC2020_Demo_Explosion`) 0.0)
            (`self.Explosion` (`SceneComponent.K2_GetComponentLocation` (`self.BombMesh`)))
            (set `/Game/Blueprints/BP_InteractiveObjectsEffect_Outline.isActive` false (`self.interactiveEffect`)) ; Turn off affordance effect
            ;[1 0.8086 0 0.29] Set explosion location to check on locks after reset
            (`/Game/Blueprints/BP_Island03Stairwell.BombDetonate` (`self.StairRef`) (`self.BombMesh`))
            ;[1 0.4592 0 0.389] Fire particles
            (`ActorComponent.Activate` (`self.ExplosionParticles`) true)
            (`SceneComponent.SetVisibility` (`self.BombMesh`) false false)
            ;[1 0.8396 0 0.264] Reset bomb to starting position
            (`UxtGrabTargetComponent.ForceEndGrab` (`self.UxtGenericManipulator`))
            ;[1 0 0.03369 0.321] Reset bool to spawn new bomb on button press
            (`KismetSystemLibrary.Delay` (`self.BombResetCooldownTime`))
            (`self.ArmBomb` true)
            (`self.WakeBomb` true)
            (set `self.BombAlreadyExists` false)))))))

(event `BombFallOfMap`
  (set `self.BombArmedToBlow` true)
  (goto _label :!via `SetNewTime`))

(event `WakeBomb`
  (params (Sleep :type Boolean))
  (bind _returnvalue (not Sleep))
  ;[0.4003 0.8283 1 0.405] Hide Bomb Until Needed
  (`SceneComponent.SetVisibility` (`self.BombMesh`) _returnvalue true)
  (set `self.IsBombAsleep` _returnvalue)
  (set `/Game/Blueprints/BP_InteractiveObjectsEffect_Outline.isActive` _returnvalue (`self.interactiveEffect`)))

(event `self.UxtGenericManipulator.OnBeginGrab`
  (params (Grabbable :type "UxtGrabTargetComponent Object Reference") (GrabPointer :type "UxtGrabPointerData Structure"))
  (bind _bombmesh (`self.BombMesh`))
  (bind _rotatingmovement (`self.RotatingMovement`))
  (set `/Game/Blueprints/BP_InteractiveObjectsEffect_Outline.isGrabbed` true (`self.interactiveEffect`))
  (`self.ScaleDown`)
  ;[0.3694 1 0.6763] Disable physics
  (`PrimitiveComponent.SetEnableGravity` _bombmesh false)
  (`PrimitiveComponent.SetSimulatePhysics` _bombmesh false)
  ;[0.5284 0.6322 1 0.394] StopBombRotating
  (set `self.IsBombHeld?` true)
  (set `RotatingMovementComponent.RotationRate` (struct) _rotatingmovement)
  (`ActorComponent.Deactivate` _rotatingmovement)
  (`SceneComponent.K2_SetWorldRotation` _bombmesh (`SceneComponent.K2_GetComponentRotation` _bombmesh) false false)
  ;[1 0.5438 0] Arm bomb on grab
  (`self.ArmBomb` false)
  ;[0 0 0] AUD - play metal grab sfx
  (`AudioComponent.Play` (`self.AUD_Grab_Cue`) 0.0))

(event `self.UxtGenericManipulator.OnEndGrab`
  (params (Grabbable :type "UxtGrabTargetComponent Object Reference") (GrabPointer :type "UxtGrabPointerData Structure"))
  (bind _bombmesh (`self.BombMesh`))
  (set `/Game/Blueprints/BP_InteractiveObjectsEffect_Outline.isGrabbed` false (`self.interactiveEffect`))
  ;[0.3755 1 0.6848] EnablePhysics
  (`PrimitiveComponent.SetEnableGravity` _bombmesh true)
  (`PrimitiveComponent.SetSimulatePhysics` _bombmesh true)
  (set `self.IsBombHeld?` false))

(event `/Game/Framework/BP_GazeTriggerInterface.OnGazeBegin`
  ;[1 1 1] Gaze
  (set `/Game/Blueprints/BP_InteractiveObjectsEffect_Outline.isLookedAt` true (`self.interactiveEffect`)))

(event `self.UxtGenericManipulator.OnEnterGrabFocus`
  (params (Grabbable :type "UxtGrabTargetComponent Object Reference") (Pointer :type "UxtNearPointerComponent Object Reference"))
  ;[1 1 1] Grab Focus
  (set `/Game/Blueprints/BP_InteractiveObjectsEffect_Outline.grabFocus` true (`self.interactiveEffect`))
  (`self.ScaleUp`))

(event `ScaleUp`
  ;[1 1 1] Interactive Scaling
  (bind (_direction _scale) (`Timeline|GrabFocusScaleTimeline` :!label _label_2)
    (:`Update`
      (`SceneComponent.SetRelativeScale3D` (`self.BombMesh`) (`KismetMathLibrary.Conv_DoubleToVector` (`KismetMathLibrary.Lerp` 1.0 1.15 _scale))))))

(event `ScaleDown`
  ;[1 1 1] Interactive Scaling
  (goto _label_2 :!via `Reverse`))

(event `self.UxtGenericManipulator.OnExitGrabFocus`
  (params (Grabbable :type "UxtGrabTargetComponent Object Reference") (Pointer :type "UxtNearPointerComponent Object Reference"))
  ;[1 1 1] Grab Focus
  (set `/Game/Blueprints/BP_InteractiveObjectsEffect_Outline.grabFocus` false (`self.interactiveEffect`))
  (`self.ScaleDown`))

(event `/Game/Framework/BP_GazeTriggerInterface.OnGazeEnd`
  ;[1 1 1] Gaze
  (set `/Game/Blueprints/BP_InteractiveObjectsEffect_Outline.isLookedAt` false (`self.interactiveEffect`)))

(fn `IsGrabFocusable`
  (params (Primitive :type "PrimitiveComponent Object Reference"))
  (returns (ReturnValue :type Boolean))
  (return false))

(fn `UserConstructionScript`
  (bind _returnvalue (`PrimitiveComponent.CreateDynamicMaterialInstance` (`self.BombMesh`) 0 "/Game/Art/BombMachine/MI_BombMachine.MI_BombMachine" "None"))
  (set `self.BombMat` _returnvalue)
  (`TimelineComponent.SetPlayRate` (`self.GrabFocusScaleTimeline`) 3.5))