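; A plinth that, while active, acts as a hover point for gems of its matching colour.
; Activation sets it active after a delay; each Tick it then searches HoverSphere for a matching gem and passes it the sphere's centre as hover location.
; Any gem leaving the sphere is told the overlap has ended.
; The sphere-mask emissive power-up and its dynamic material are disabled to reduce draw calls.
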(event `ActivatePlinth`
  (params (Delay :type "Float (double-precision)") (SpheremaskOrigin :type "Vector Structure"))
  ;[1 1 1] Activate - Set Active and Light Up
  (`KismetSystemLibrary.Delay` Delay)
  (set `self.Active` true)
  (`self.PlinthEmissiveLinesPowerUp` SpheremaskOrigin))

(event `self.ReceiveTick`
  (params (DeltaSeconds :type "Float (single-precision)"))
  ;[1 1 1] Tell gem overlapping
  (if (`self.Active`)
    (bind (_overlapping _overlappinggem) (`self.IsGemOverlapping`))
    (if _overlapping
      (`/Game/Blueprints/BP_Gem.SetOverlappingPlinth` _overlappinggem true (`KismetSystemLibrary.GetComponentBounds` (`self.HoverSphere`))))))

(event `self.HoverSphere.OnComponentEndOverlap`
  (params (OverlappedComponent :type "PrimitiveComponent Object Reference") (OtherActor :type "Actor Object Reference") (OtherComp :type "PrimitiveComponent Object Reference") (OtherBodyIndex :type Integer))
  ;[1 1 1] Tell Gem Overlap Finished
  (bind _asbp_gem (cast `/Game/Blueprints/BP_Gem` OtherActor))
  (`/Game/Blueprints/BP_Gem.SetOverlappingPlinth` _asbp_gem false (`KismetSystemLibrary.GetComponentBounds` (`self.HoverSphere`))))

(event `PlinthEmissiveLinesPowerUp`
  (params (SpheremaskOrigin :type "Vector Structure"))
  ;[0 0.9622 1 0.587] Power up emissive lines (disabled to reduce draw calls)
)

(fn `Deactivate`
  (set `self.Active` false)
  (return))

(fn `IsGemOverlapping`
  (returns (Overlapping :type Boolean) (OverlappingGem :type "/Game/Blueprints/BP_Gem Object Reference"))
  (for _array_element (`PrimitiveComponent.GetOverlappingActors` (`self.HoverSphere`) "/Game/Blueprints/BP_Gem.BP_Gem_C")
    (bind _asbp_gem (cast `/Game/Blueprints/BP_Gem` _array_element))
    (if (`|EnumEquality` (`self.GemColour`) (`/Game/Blueprints/BP_Gem.GemColor` _asbp_gem))
      (return true _asbp_gem)))
  (return false null))

(fn `UserConstructionScript`)