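; Island 02 actor that powers up glowing emissive lines on its island and rock ramp meshes, plus red, green and blue gem sockets.
; The construction script creates dynamic material instances, enables sphere masking and caches mask positions from marker components.
; The power-up event plays a sound and uses a timeline to drive mask radius, hardness, intensity and colour.
; Each gem event animates its own sub-mask on the island material only.
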(event `EmissiveLinesPowerUp`
  (bind _rampmat (`self.RampMat`))
  (bind _islandmat (`self.IslandMat`))
  (bind _returnvalue (`KismetMathLibrary.Conv_VectorToLinearColor` (`self.MainMaskPosition`)))
  ;[0 0.9622 1 0.587] Power up emissive lines
  (`GameplayStatics.PlaySoundAtLocation` "/Game/Sounds/Island/SC_IslandPowerUp.SC_IslandPowerUp" (`SceneComponent.K2_GetComponentLocation` (`self.MainEmissiveSphereMask`)) (struct) 1.0 1.0 0.0 "/Game/Sounds/DefaultAttenuationSettings.DefaultAttenuationSettings" null null)
  (bind (_direction _sphereradius _hardness _emissivestrength _emissivecolour) (`Timeline|ExpandSphereMask` :!via `PlayFromStart`)
    (:`Update`
      (`MaterialInstanceDynamic.SetVectorParameterValue` _rampmat "MainSphereMaskLocation" _returnvalue)
      (`MaterialInstanceDynamic.SetScalarParameterValue` _rampmat "MainSphereMaskRadius" _sphereradius)
      (`MaterialInstanceDynamic.SetScalarParameterValue` _rampmat "MainSphereMaskHardness" _hardness)
      (`MaterialInstanceDynamic.SetScalarParameterValue` _rampmat "EmissiveIntensity" _emissivestrength)
      (`MaterialInstanceDynamic.SetVectorParameterValue` _rampmat "EmissiveColour" _emissivecolour)
      (`MaterialInstanceDynamic.SetVectorParameterValue` _islandmat "MainSphereMaskLocation" _returnvalue)
      (`MaterialInstanceDynamic.SetScalarParameterValue` _islandmat "MainSphereMaskRadius" _sphereradius)
      (`MaterialInstanceDynamic.SetScalarParameterValue` _islandmat "MainSphereMaskHardness" _hardness)
      (`MaterialInstanceDynamic.SetScalarParameterValue` _islandmat "EmissiveIntensity" _emissivestrength)
      (`MaterialInstanceDynamic.SetVectorParameterValue` _islandmat "EmissiveColour" _emissivecolour))))

(event `RedGemEmissive`
  (bind _islandmat (`self.IslandMat`))
  ;[0 1 0.3469 0.243] Power up eachgem Socket
  (bind (_direction _sphereradius _hardness) (`Timeline|Timeline_3` :!via `PlayFromStart`)
    (:`Update`
      (`MaterialInstanceDynamic.SetVectorParameterValue` _islandmat "SubSphereMaskLocation1" (`KismetMathLibrary.Conv_VectorToLinearColor` (`self.RedMaskPosition`)))
      (`MaterialInstanceDynamic.SetScalarParameterValue` _islandmat "SubSphereMaskRadius1" _sphereradius)
      (`MaterialInstanceDynamic.SetScalarParameterValue` _islandmat "SubSphereMaskHardness1" _hardness))))

(event `GreenGemEmissive`
  (bind _islandmat (`self.IslandMat`))
  ;[0 1 0.3469 0.243] Power up eachgem Socket
  (bind (_direction _sphereradius _hardness) (`Timeline|Timeline_2` :!via `PlayFromStart`)
    (:`Update`
      (`MaterialInstanceDynamic.SetVectorParameterValue` _islandmat "SubSphereMaskLocation2" (`KismetMathLibrary.Conv_VectorToLinearColor` (`self.GreenMaskPosition`)))
      (`MaterialInstanceDynamic.SetScalarParameterValue` _islandmat "SubSphereMaskRadius2" _sphereradius)
      (`MaterialInstanceDynamic.SetScalarParameterValue` _islandmat "SubSphereMaskHardness2" _hardness))))

(event `BlueGemEmissive`
  (bind _islandmat (`self.IslandMat`))
  ;[0 1 0.3469 0.243] Power up eachgem Socket
  (bind (_direction _sphereradius _hardness) (`Timeline|Timeline_0` :!via `PlayFromStart`)
    (:`Update`
      (`MaterialInstanceDynamic.SetVectorParameterValue` _islandmat "SubSphereMaskLocation3" (`KismetMathLibrary.Conv_VectorToLinearColor` (`self.BlueMaskPosition`)))
      (`MaterialInstanceDynamic.SetScalarParameterValue` _islandmat "SubSphereMaskRadius3" _sphereradius)
      (`MaterialInstanceDynamic.SetScalarParameterValue` _islandmat "SubSphereMaskHardness3" _hardness))))

(fn `UserConstructionScript`
  (`|ExecutionSequence`
    (:`then_0`
      ;[0 1 0.9055 0.426] Setup dynamic mat instances
      (bind _returnvalue (`PrimitiveComponent.CreateDynamicMaterialInstance` (`self.SM_IslandB`) 0 "/Game/Art/IslandB/MI_Island.MI_Island" "None"))
      (set `self.IslandMat` _returnvalue)
      (bind _returnvalue_2 (`PrimitiveComponent.CreateDynamicMaterialInstance` (`self.SM_RockRamp`) 0 "/Game/Art/IslandB/MI_Rock.MI_Rock" "None"))
      (bind _output_get (set `self.RampMat` _returnvalue_2))
      ;[0 1 0.9075 0.413] Set both materials to use mask
      (`MaterialInstanceDynamic.SetScalarParameterValue` _output_get "UseEmissiveSphereMaskBool" 1.0)
      (`MaterialInstanceDynamic.SetScalarParameterValue` (`self.IslandMat`) "UseEmissiveSphereMaskBool" 1.0))
    (:`then_1`
      ;[1 0.7013 0 0.415] Get Main Mask postion
      (set `self.MainMaskPosition` (`SceneComponent.K2_GetComponentLocation` (`self.MainEmissiveSphereMask`)))
      ;[1 0.6135 0 0.478] GetSubMasks
      (set `self.RedMaskPosition` (`SceneComponent.K2_GetComponentLocation` (`self.RedEmissiveSphere`)))
      (set `self.GreenMaskPosition` (`SceneComponent.K2_GetComponentLocation` (`self.GreenEmissiveSphere`)))
      (set `self.BlueMaskPosition` (`SceneComponent.K2_GetComponentLocation` (`self.BlueEmissiveSphere`))))))