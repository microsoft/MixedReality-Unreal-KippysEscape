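; Island 03 actor that powers its emissive lines on or off through ToggleIslandGlow.
; The construction script creates dynamic materials, sharing one stone instance across props, and caches start transforms.
; One timeline drives sphere-mask glow parameters, raises floating stones, pillars and the bomb island, and triggers BP_BombFactoryV2's hover through an event track.
; Enabling plays a sound; disabling reverses the timeline after a delay; both notify floating-stone child actors.
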(event `ToggleIslandGlow`
  (params (Enabled :type Boolean))
  (bind _bombislandmat (`self.BombIslandMat`))
  (bind _blocksmat (`self.BlocksMat`))
  (bind _stonemat (`self.StoneMat`))
  ;[0.09399 0.8702 1 0.588] Turn island Emissive lines on
  (if Enabled
    (`|ExecutionSequence`
      (:`then_0`
        (`GameplayStatics.PlaySoundAtLocation` "/Game/Sounds/Island/SC_IslandPowerUp.SC_IslandPowerUp" (`SceneComponent.K2_GetComponentLocation` (`self.Sphere`)) (struct) 1.0 1.0 0.0 "/Game/Sounds/DefaultAttenuationSettings.DefaultAttenuationSettings" null null)
        (bind (_direction _sphereradius _hardness _emissivestrength _movepillarsup _bombfactoryriseup _emissivecolour) (`Timeline|EmissiveLinesLightUp` :!via `PlayFromStart` :!label _label)
          (:`Update`
            (`MaterialInstanceDynamic.SetVectorParameterValue` _blocksmat "MainSphereMaskLocation" (`KismetMathLibrary.Conv_VectorToLinearColor` (`self.SphereMaskLoc`)))
            (`MaterialInstanceDynamic.SetScalarParameterValue` _blocksmat "MainSphereMaskRadius" _sphereradius)
            (`MaterialInstanceDynamic.SetScalarParameterValue` _blocksmat "MainSphereMaskHardness" _hardness)
            (`MaterialInstanceDynamic.SetScalarParameterValue` _blocksmat "EmissiveIntensity" _emissivestrength)
            (`MaterialInstanceDynamic.SetVectorParameterValue` _blocksmat "EmissiveColour" _emissivecolour)
            (`MaterialInstanceDynamic.SetVectorParameterValue` _stonemat "MainSphereMaskLocation" _emissivecolour)
            (`MaterialInstanceDynamic.SetScalarParameterValue` _stonemat "MainSphereMaskRadius" _sphereradius)
            (`MaterialInstanceDynamic.SetScalarParameterValue` _stonemat "MainSphereMaskHardness" _hardness)
            (`MaterialInstanceDynamic.SetScalarParameterValue` _stonemat "EmissiveIntensity" _emissivestrength)
            (`MaterialInstanceDynamic.SetVectorParameterValue` _stonemat "EmissiveColour" _emissivecolour)
            ;[1 1 1] makes floating stone rise up
            (`SceneComponent.K2_SetRelativeLocationAndRotation` (`self.FloatingStoneA`) (`KismetMathLibrary.VLerp` (`self.FloatingStoneA_StartLoc`) (`self.FloatingStoneA_EndLoc`) _movepillarsup) (`KismetMathLibrary.RLerp` (`self.FloatingStoneA_StartRot`) (`self.FloatingStoneA_EndRot`) _movepillarsup) false false)
            (`SceneComponent.K2_SetRelativeLocationAndRotation` (`self.FloatingStoneB`) (`KismetMathLibrary.VLerp` (`self.FloatingStoneB_StartLoc`) (`self.FloatingStoneB_EndLoc`) _movepillarsup) (`KismetMathLibrary.RLerp` (`self.FloatingStoneB_StartRot`) (`self.FloatingStoneB_EndRot`) _movepillarsup) false false)
            ;[1 0.8167 0 0.232] Make pillars rise up
            (for (_array_element _array_index) (`self.Pillars`)
              (`SceneComponent.K2_SetRelativeLocation` _array_element (`KismetMathLibrary.VLerp` (`|GetArrayItem` (`self.PillarsStartLoc`) _array_index) (0.0 0.0 0.0) _movepillarsup) false false)
              ;[1 0.3335 0 0.441] Make bomb factory float up
              (`SceneComponent.K2_SetWorldTransform` (`self.BombIsland_GRP`) (`KismetMathLibrary.TLerp` (`self.BombIslandStartTransform`) (`SceneComponent.K2_GetComponentToWorld` (`self.BombIslandEndingPoint`)) _movepillarsup) false false)
              (`MaterialInstanceDynamic.SetVectorParameterValue` _bombislandmat "MainSphereMaskLocation" (`KismetMathLibrary.Conv_VectorToLinearColor` (`SceneComponent.K2_GetComponentLocation` (`self.BombIslandMask`))))
              (`MaterialInstanceDynamic.SetScalarParameterValue` _bombislandmat "MainSphereMaskRadius" (`KismetMathLibrary.Lerp` 0.0 35.0 _bombfactoryriseup))
              (`MaterialInstanceDynamic.SetScalarParameterValue` _bombislandmat "MainSphereMaskHardness" 25.0)
              (`MaterialInstanceDynamic.SetScalarParameterValue` _bombislandmat "EmissiveIntensity" (`KismetMathLibrary.Lerp` 0.0 3.0 _bombfactoryriseup))
              (`MaterialInstanceDynamic.SetVectorParameterValue` _bombislandmat "EmissiveColour" _emissivecolour)))
          (:`FireBombFactory`
            ;[1 0.8695 0 0.308] Activate bomb machine and spline cable
            (bind _returnvalue (`GameplayStatics.GetActorOfClass` "/Game/Blueprints/BP_BombFactoryV2.BP_BombFactoryV2_C"))
            (`/Game/Blueprints/BP_BombFactoryV2.BombMachineHover` _returnvalue))))
      (:`then_1`
        ;;[0.2011 0.7042 1 0.561] Updates states of FlotingStones child BPs
        (`|ExecutionSequence` :!label _label_2
          (:`then_0`
            (bind _asbp_floating_stone_a (cast `/Game/Blueprints/IslandC/BP_FloatingStoneA` (`ChildActorComponent.ChildActor` (`self.FloatingStoneA`))))
            (`/Game/Blueprints/IslandC/BP_FloatingStoneA.ActivationToggle` _asbp_floating_stone_a Enabled))
          (:`then_1`
            (bind _asbp_floating_stone_b (cast `/Game/Blueprints/IslandC/BP_FloatingStoneB` (`ChildActorComponent.ChildActor` (`self.FloatingStoneB`))))
            (`/Game/Blueprints/IslandC/BP_FloatingStoneB.ActivationToggle` _asbp_floating_stone_b Enabled)))))
    (else
      (`KismetSystemLibrary.Delay` 1.5)
      (`|ExecutionSequence`
        (:`then_0`
          (goto _label :!via `Reverse`))
        (:`then_1`
          (goto _label_2))))))

(fn `UserConstructionScript`
  (bind _stonemat (`self.StoneMat`))
  (bind _array (`|MakeArray` (`self.SM_IslandC_PillarLeft`) (`self.SM_IslandC_PillarRight`) (`self.SM_IslandC_PillarLeft2`) (`self.SM_IslandC_PillarRight2`)))
  (`|ExecutionSequence`
    (:`then_0`
      ;[0.2249 0.4679 1 0.337] Setup main blocks emissive mat
      (bind _returnvalue (`PrimitiveComponent.CreateDynamicMaterialInstance` (`self.SM_IslandC_MainIsland`) 0 "/Game/Art/IslandC/MI_Island.MI_Island" "None"))
      (set `self.BlocksMat` _returnvalue)
      (bind _returnvalue_2 (`PrimitiveComponent.CreateDynamicMaterialInstance` (`self.SM_IslandC_BombIsland`) 0 "/Game/Art/IslandC/MI_Island.MI_Island" "None"))
      (set `self.BombIslandMat` _returnvalue_2)
      ;[0.1946 0.2477 0.3958 0.431] Setup remaining assets emissive mats
      (bind _returnvalue_3 (`PrimitiveComponent.CreateDynamicMaterialInstance` (`self.SM_IslandC_PillarLeft`) 0 "/Game/Art/IslandC/MI_Stone.MI_Stone" "None"))
      (bind _output_get (set `self.StoneMat` _returnvalue_3))
      (for _array_element (`|MakeArray` (`self.SM_IslandC_TowerRight`) (`self.SM_IslandC_TowerLeft`) (`self.SM_IslandC_PillarBase`) (`self.SM_IslandC_PillarLeft`) (`self.SM_IslandC_PillarBase1`) (`self.SM_IslandC_PillarRight`) (`self.SM_IslandC_PillarBase2`) (`self.SM_IslandC_PillarLeft2`) (`self.SM_IslandC_PillarBase3`) (`self.SM_IslandC_PillarRight2`))
        (`PrimitiveComponent.SetMaterial` _array_element 0 _output_get))
      (`|ExecutionSequence`
        (:`then_0`
          (`|ExecutionSequence`
            (:`then_0`
              (bind _asbp_floating_stone_a (cast `/Game/Blueprints/IslandC/BP_FloatingStoneA` (`ChildActorComponent.ChildActor` (`self.FloatingStoneA`))))
              (`PrimitiveComponent.SetMaterial` (`/Game/Blueprints/IslandC/BP_FloatingStoneA.FloatingStoneA_1` _asbp_floating_stone_a) 0 _stonemat)
              (`PrimitiveComponent.SetMaterial` (`/Game/Blueprints/IslandC/BP_FloatingStoneA.FloatingStoneA_2` _asbp_floating_stone_a) 0 _stonemat)
              (`PrimitiveComponent.SetMaterial` (`/Game/Blueprints/IslandC/BP_FloatingStoneA.FloatingStoneA_3` _asbp_floating_stone_a) 0 _stonemat))
            (:`then_1`
              (bind _asbp_floating_stone_b (cast `/Game/Blueprints/IslandC/BP_FloatingStoneB` (`ChildActorComponent.ChildActor` (`self.FloatingStoneB`))))
              (`PrimitiveComponent.SetMaterial` (`/Game/Blueprints/IslandC/BP_FloatingStoneB.FloatingStoneB_1` _asbp_floating_stone_b) 0 _stonemat)
              (`PrimitiveComponent.SetMaterial` (`/Game/Blueprints/IslandC/BP_FloatingStoneB.FloatingStoneB_2` _asbp_floating_stone_b) 0 _stonemat)
              (`PrimitiveComponent.SetMaterial` (`/Game/Blueprints/IslandC/BP_FloatingStoneB.FloatingStoneB_3` _asbp_floating_stone_b) 0 _stonemat))))
        (:`then_1`
          ;[1 0.9217 0 0.337] SetupSphere mask location
          (set `self.SphereMaskLoc` (`SceneComponent.K2_GetComponentLocation` (`self.Sphere`)))
          ;[1 0.7982 0 0.373] Get Pillars relative locations
          (set `self.Pillars` _array)
          (for (_array_element_2 _array_index) _array
            (`KismetArrayLibrary.Array_Set` (`self.PillarsStartLoc`) _array_index (`SceneComponent.RelativeLocation` _array_element_2) true)))))
    (:`then_1`
      (`|ExecutionSequence`
        (:`then_0`
          ;[0.03311 0.147 0.1559] Setup Floating block refs
          (bind _asbp_floater_block (cast `/Game/Blueprints/BP_floaterBlock` (`ChildActorComponent.ChildActor` (`self.FloatingStoneA`))))
          (`StaticMeshComponent.SetStaticMesh` (`/Game/Blueprints/BP_floaterBlock.FloatingBlock` _asbp_floater_block) "/Game/Art/IslandC/SM_IslandC_FloatingStoneB.SM_IslandC_FloatingStoneB"))
        (:`then_1`
          (bind _asbp_floater_block_2 (cast `/Game/Blueprints/BP_floaterBlock` (`ChildActorComponent.ChildActor` (`self.FloatingStoneA`))))
          (`StaticMeshComponent.SetStaticMesh` (`/Game/Blueprints/BP_floaterBlock.FloatingBlock` _asbp_floater_block_2) "/Game/Art/IslandC/SM_IslandC_FloatingStoneB.SM_IslandC_FloatingStoneB"))
        (:`then_2`
          ;[1 0.7394 0 0.41] Setup Bomb island ending position
          (set `self.BombIslandStartTransform` (`SceneComponent.K2_GetComponentToWorld` (`self.BombIsland_GRP`))))))))