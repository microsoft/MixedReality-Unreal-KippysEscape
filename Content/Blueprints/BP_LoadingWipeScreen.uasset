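; Loading-screen wipe actor that covers or reveals the player's view with a black cube.
; On BeginPlay it attaches its pivot to the player camera manager and marks the wipe as active.
; ActivateBlackWipe runs a timeline lerping the cube between its construction-time position and 200 units below, reversed to hide the screen and forward to reveal it.
; An IsActive flag blocks repeat triggers, and the cube is hidden once a reveal finishes.
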(event `self.ReceiveBeginPlay`
  ;[1 0.6842 0 0.337] On start parent the BP to the player camera and set it to active
  (`SceneComponent.K2_AttachToComponent` (`self.OriginPivot`) (`PlayerCameraManager.TransformComponent` (`GameplayStatics.GetPlayerCameraManager` 0)) "None" "KeepRelative" "KeepRelative" "KeepRelative" true)
  (set `self.isActive?` true))

(event `ActivateBlackWipe`
  (params (HideScreen :type Boolean))
  (bind _blackwipecubelocation (`self.BlackWipeCubeLocation`))
  ;[1 1 1] HideMeansMoveUp ^
  (if HideScreen
    (if (not (`self.isActive?`))
      (set `self.isActive?` true)
      (`SceneComponent.SetHiddenInGame` (`self.BlackWipeCube`) false false)
      (bind (_direction _lerpcubezpos) (`Timeline|WipeScreen` :!via `ReverseFromEnd` :!label _label)
        (:`Update`
          (`SceneComponent.K2_SetRelativeLocation` (`self.BlackWipeCube`) (`KismetMathLibrary.VLerp` _blackwipecubelocation (- _blackwipecubelocation (0.0 0.0 200.0)) _lerpcubezpos) false false))
        (:`Finished`
          (if (not HideScreen)
            (`SceneComponent.SetHiddenInGame` (`self.BlackWipeCube`) true false)))))
    (elif (`self.isActive?`)
      (set `self.isActive?` false)
      (goto _label :!via `PlayFromStart`))))

(fn `UserConstructionScript`
  (set `self.BlackWipeCubeLocation` (`SceneComponent.RelativeLocation` (`self.BlackWipeCube`))))