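; BP_GlowHint is a timed hint that makes the current state's interactables glow, with only Gem Placement (BP_Gem meshes) handled so far.
; OnGameStateChanged clears previous targets, enables custom depth on new ones, then switches the glow on and off using placeholder delays.
; Activation attaches glow particles to each target, later removed on deactivation.
; Tick eases MPC_Outliner's "OffOn" parameter to fade the post-process outline in and out.
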(event `self.ReceiveBeginPlay`)

(event `Event OnGameStateChanged`
  (params (NewState :type "/Game/Framework/StateMachine/EGameState Enum" :default "NewEnumerator9"))
  ;[1 1 1] Bind to game state change events
  (`|ExecutionSequence`
    (:`then_0`
      ;;[1 1 1] Reset Array
      (for _array_element (`self.Interactables`)
        (`PrimitiveComponent.SetRenderCustomDepth` _array_element false))
      (`KismetArrayLibrary.Array_Clear` (`self.Interactables`))
      (`KismetArrayLibrary.Array_Clear` (`self.Interactables_Actors`)))
    (:`then_1`
      (`self.UpdateArray` NewState)
      ;[1 0 0] Add logic to properly fire these events
      (`KismetSystemLibrary.Delay` 4.0)
      (`self.ActivateEffect`)
      (`KismetSystemLibrary.Delay` 7.0)
      (`self.DeactivateGlow`))))

(event `ActivateEffect`
  ;[1 1 1] Activation
  (set `self.Active` true)
  (for _array_element (`self.Interactables`)
    (bind _returnvalue (`GameplayStatics.SpawnEmitterAttached` "/Game/Effects/Glow/PS_Glow_v02.PS_Glow_v02" _array_element "None" (`self.emitterOffset`) (struct) (`self.emitterScale`)))
    (`KismetArrayLibrary.Array_Add` (`self.Emitter`) _returnvalue)))

(event `self.ReceiveTick`
  (params (DeltaSeconds :type "Float (single-precision)"))
  (bind _returnvalue (`KismetMathLibrary.FInterpTo_Constant` (`self.OnOff`) 0.0 DeltaSeconds 1.5))
  (bind _returnvalue_2 (`KismetMathLibrary.FInterpTo_Constant` (`self.OnOff`) 1.0 DeltaSeconds 0.5))
  ;[1 1 1] Update Post Process Material
  (if (`self.Active`)
    (set `self.OnOff` _returnvalue_2)
    (`KismetMaterialLibrary.SetScalarParameterValue` "/Game/Materials/PostProcess/Outliner/MPC_Outliner.MPC_Outliner" "OffOn" _returnvalue_2)
    (else
      (set `self.OnOff` _returnvalue)
      (`KismetMaterialLibrary.SetScalarParameterValue` "/Game/Materials/PostProcess/Outliner/MPC_Outliner.MPC_Outliner" "OffOn" _returnvalue))))

(event `DeactivateGlow`
  (bind _emitter (`self.Emitter`))
  ;[1 1 1] Deactivation
  (set `self.Active` false)
  (for _array_element (`self.Emitter`)
    (`ActorComponent.Deactivate` _array_element))
  (`KismetSystemLibrary.Delay` 1.0)
  (for _array_element_2 _emitter
    (`ActorComponent.K2_DestroyComponent` _array_element_2))
  (`KismetArrayLibrary.Array_Clear` _emitter))

(fn `UpdateArray`
  (params (newState :type "/Game/Framework/StateMachine/EGameState Enum" :default "NewEnumerator9"))
  (switch `/Game/Framework/StateMachine/EGameState` newState
    (:`NewEnumerator4`
      ;[1 1 1] Stores current Interactable objects
      (bind _outactors (`GameplayStatics.GetAllActorsOfClass` "/Game/Blueprints/BP_Gem.BP_Gem_C"))
      (for _array_element _outactors
        (`KismetArrayLibrary.Array_Add` (`self.Interactables`) (`/Game/Blueprints/BP_Gem.GemMesh` _array_element)))
      ;[1 1 1] PS scale and offset from pivot point
      (set `self.emitterScale` (1.5 1.5 1.5))
      (set `self.emitterOffset` (0.0 0.0 0.0))
      (for _array_element_2 (`self.Interactables`)
        (`PrimitiveComponent.SetRenderCustomDepth` _array_element_2 true)))))

(fn `UserConstructionScript`)