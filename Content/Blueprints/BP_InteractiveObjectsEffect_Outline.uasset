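; Outline highlight effect for interactive objects, responding to gaze, hand proximity and grabbing.
; Each Tick derives an Off, Active or Grabbing state from externally set flags and the nearer index fingertip's distance.
; A dynamic material interpolates thickness, tints by proximity, pulses until grab focus, and shrinks away when grabbed or inactive, hiding the mesh at zero.
; Entering Active triggers a brief thicker, brighter flash and gaze audio cue via DoOnce.
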(event `self.ReceiveTick`
  (params (DeltaSeconds :type "Float (single-precision)"))
  (bind _colourbase (`self.colourBase`))
  (bind _dynamicmaterial (`self.dynamicMaterial`))
  (bind _dynamicmaterial_2 (`self.dynamicMaterial`))
  (bind _returnvalue (`SceneComponent.K2_GetComponentLocation` (`self.DefaultSceneRoot`)))
  (if (`self.isActive`)
    (`|ExecutionSequence`
      (:`then_0`
        ;[1 1 1] gets distance of the closer hand
        (bind (_outorientation _outposition) (`UxtHandTrackingFunctionLibrary.GetHandJointState` "Left" "IndexTip"))
        (bind (_outorientation_2 _outposition_2) (`UxtHandTrackingFunctionLibrary.GetHandJointState` "Right" "IndexTip"))
        (bind _returnvalue_2 (`KismetMathLibrary.Vector_Distance` _outposition _returnvalue))
        (bind _returnvalue_3 (`KismetMathLibrary.Vector_Distance` _outposition_2 _returnvalue))
        (set `self.closerHandDistance` (`KismetMathLibrary.FClamp` (`KismetMathLibrary.SelectFloat` _returnvalue_2 _returnvalue_3 (< _returnvalue_2 _returnvalue_3)) 3.0 (+ (`self.activateEffectDistance`) 5.0))))
      (:`then_1`
        ;[1 1 1] State control
        (`|ExecutionSequence`
          (:`then_0`
            (if (< (`self.closerHandDistance`) (`self.activateEffectDistance`))
              (set `self.handIsClose` true)
              (else
                (set `self.handIsClose` false))))
          (:`then_1`
            (if (`self.isGrabbed`)
              (set `self.effectState` "NewEnumerator4")
              (elif (or (`self.isLookedAt`) (`self.handIsClose`))
                (set `self.effectState` "NewEnumerator1")
                (`/Engine/EditorBlueprintResources/StandardMacros.DoOnce` false :!label _label
                  (:`Completed`
                    (set `self.initialGlance` true)
                    ;[0 0 0 0.604] GCVRS - Gaze audio
                    (if (not (`AudioComponent.IsPlaying` (`self.AUD_Gaze_Cue`)))
                      (`AudioComponent.Play` (`self.AUD_Gaze_Cue`) 0.0))
                    (`KismetSystemLibrary.Delay` 0.33)
                    (set `self.initialGlance` false)))
                (else
                  (set `self.effectState` "NewEnumerator0")
                  (goto _label :!via `Reset`)))))))
      (:`then_2`
        ;[1 1 1] otline behavior
        (`|ExecutionSequence`
          (:`then_0`
            (switch `/Game/Blueprints/Enums/E_InteractiveObjectsState` (`self.effectState`)
              (:`NewEnumerator0`
                (set `self.outlineScale` (`KismetMathLibrary.FInterpTo` (`self.outlineScale`) 0.0 (`GameplayStatics.GetWorldDeltaSeconds`) (`self.interpSpeed`)) :!label _label_2)
                (`MaterialInstanceDynamic.SetScalarParameterValue` (`self.dynamicMaterial`) "Scale" (`self.outlineScale`)))
              (:`NewEnumerator1`
                (if (`self.grabFocus`)
                  (set `self.outlineScale` (`KismetMathLibrary.FInterpTo` (`self.outlineScale`) (`self.thicknessFocusTarget`) (`GameplayStatics.GetWorldDeltaSeconds`) (`self.interpSpeed`)))
                  (`MaterialInstanceDynamic.SetScalarParameterValue` _dynamicmaterial_2 "Scale" (`self.outlineScale`))
                  (`MaterialInstanceDynamic.SetScalarParameterValue` _dynamicmaterial_2 "Pulse" 0.0)
                  (`MaterialInstanceDynamic.SetVectorParameterValue` (`self.dynamicMaterial`) "Colour" (* (`self.colourCanBeHeald`) 2.0))
                  (else
                    (`MaterialInstanceDynamic.SetVectorParameterValue` (`self.dynamicMaterial`) "Colour" (`KismetMathLibrary.LinearColorLerp` (`KismetMathLibrary.SelectColor` (* _colourbase 3.0) _colourbase (`self.initialGlance`)) (`self.colourCanBeHeald`) (- 1.0 (`KismetMathLibrary.MapRangeClamped` (`self.closerHandDistance`) 4.0 12.5 0.25 1.0))))
                    (set `self.outlineScale` (`KismetMathLibrary.FInterpTo` (`self.outlineScale`) (`KismetMathLibrary.SelectFloat` (* (`self.thicknessFocusTarget`) 1.5) (`self.thicknessActiveTarget`) (`self.initialGlance`)) (`GameplayStatics.GetWorldDeltaSeconds`) (`self.interpSpeed`)))
                    (`MaterialInstanceDynamic.SetScalarParameterValue` _dynamicmaterial "Scale" (`self.outlineScale`))
                    (`MaterialInstanceDynamic.SetScalarParameterValue` _dynamicmaterial "Pulse" 1.0))))
              (:`NewEnumerator4`
                (goto _label_2))))
          (:`then_1`
            ;;[1 1 1] hides effect when not active
            (if (== (`self.outlineScale`) 0.0) :!label _label_3
              (`SceneComponent.SetHiddenInGame` (`self.outlineMesh`) true false)
              (else
                (`SceneComponent.SetHiddenInGame` (`self.outlineMesh`) false false)))))))
    (else
      (set `self.outlineScale` (`KismetMathLibrary.FInterpTo` (`self.outlineScale`) 0.0 (`GameplayStatics.GetWorldDeltaSeconds`) (`self.interpSpeedDisappear`)))
      (`MaterialInstanceDynamic.SetScalarParameterValue` (`self.dynamicMaterial`) "Scale" (`self.outlineScale`))
      (goto _label_3))))

(fn `UserConstructionScript`
  (bind _outlinemesh (`self.outlineMesh`))
  (`|ExecutionSequence`
    (:`then_0`
      (`SceneComponent.SetRelativeScale3D` (`self.scene_generalScale`) (`self.generalScale`)))
    (:`then_1`
      (bind _returnvalue (`PrimitiveComponent.CreateDynamicMaterialInstance` _outlinemesh 0 "/Game/Effects/ObjectInteraction/MI_ObjectInteractionOutline.MI_ObjectInteractionOutline" "None"))
      (bind _output_get (set `self.dynamicMaterial` _returnvalue))
      (`PrimitiveComponent.CreateDynamicMaterialInstance` _outlinemesh 1 _output_get "None"))))