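; A grabbable edge handle affordance, apparently for content placement, that animates in response to UX Tools grab focus and grab events.
; On BeginPlay it spawns and attaches an interactive outline effect using the guide mesh, then forwards focus and grab state to it.
; Tick spins the guide: faster on focus, stopped while grabbed, slowly after release.
; A reversible timeline scales guide and arrows, turns arrows and drives their materials, alongside rotate and grab sounds.
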(event `self.ReceiveBeginPlay`
  (bind _interactiveeffect (`self.interactiveEffect`))
  (bind _rotatorguide002 (`self.RotatorGuide002`))
  (bind _rotatorguide002_2 (`self.RotatorGuide002`))
  (bind _interactiveeffect_2 (`self.interactiveEffect`))
  ;[1 1 1] Spawn interactive object effect BP
  (bind _returnvalue (`|SpawnActorFromClass` "/Game/Blueprints/BP_InteractiveObjectsEffect_Outline.BP_InteractiveObjectsEffect_Outline_C" (`KismetMathLibrary.MakeTransform` (`SceneComponent.K2_GetComponentLocation` _rotatorguide002_2) (`SceneComponent.K2_GetComponentRotation` _rotatorguide002_2) (`SceneComponent.K2_GetComponentScale` _rotatorguide002_2)) "Undefined" "OverrideRootScale" self null))
  (set `self.interactiveEffect` _returnvalue)
  (`self.K2_AttachToComponent` _interactiveeffect _rotatorguide002 "None" "KeepWorld" "KeepWorld" "KeepWorld" true)
  (`StaticMeshComponent.SetStaticMesh` (`/Game/Blueprints/BP_InteractiveObjectsEffect_Outline.outlineMesh` _interactiveeffect) (`StaticMeshComponent.StaticMesh` _rotatorguide002))
  (set `/Game/Blueprints/BP_InteractiveObjectsEffect_Outline.isActive` true _interactiveeffect_2)
  (set `/Game/Blueprints/BP_InteractiveObjectsEffect_Outline.thicknessActiveTarget` 0.5 _interactiveeffect_2)
  (set `/Game/Blueprints/BP_InteractiveObjectsEffect_Outline.thicknessFocusTarget` 1.25 _interactiveeffect_2)
  (set `/Game/Blueprints/BP_InteractiveObjectsEffect_Outline.activateEffectDistance` 40.0 _interactiveeffect_2))

(event `self.UxtGrabTarget.OnBeginGrab`
  (params (Grabbable :type "UxtGrabTargetComponent Object Reference") (GrabPointer :type "UxtGrabPointerData Structure"))
  (`self.ScaleDown`)
  (set `/Game/Blueprints/BP_InteractiveObjectsEffect_Outline.isGrabbed` true (`self.interactiveEffect`))
  (set `self.deltaRotation` (struct))
  ;[0 0 0] AUD
  (`AudioComponent.FadeOut` (`self.AUD_Rotate_SFX`) 0.2 0.0 "Linear")
  (`AudioComponent.Play` (`self.AUD_Grab_SFX`) 0.0))

(event `self.UxtGrabTarget.OnEnterGrabFocus`
  (params (Grabbable :type "UxtGrabTargetComponent Object Reference") (Pointer :type "UxtNearPointerComponent Object Reference"))
  (`self.ScaleUp`)
  (set `/Game/Blueprints/BP_InteractiveObjectsEffect_Outline.grabFocus` true (`self.interactiveEffect`)))

(event `self.UxtGrabTarget.OnEndGrab`
  (params (Grabbable :type "UxtGrabTargetComponent Object Reference") (GrabPointer :type "UxtGrabPointerData Structure"))
  (set `/Game/Blueprints/BP_InteractiveObjectsEffect_Outline.isGrabbed` false (`self.interactiveEffect`))
  (set `self.deltaRotation` (struct :`Yaw` 0.25)))

(event `self.UxtGrabTarget.OnExitGrabFocus`
  (params (Grabbable :type "UxtGrabTargetComponent Object Reference") (Pointer :type "UxtNearPointerComponent Object Reference"))
  (`self.ScaleDown`)
  (set `/Game/Blueprints/BP_InteractiveObjectsEffect_Outline.grabFocus` false (`self.interactiveEffect`)))

(event `ScaleUp`
  (bind _sm_handlearrows (`self.SM_HandleArrows`))
  ;[0 0 0 0.779] AUD
  (if (not (`AudioComponent.IsPlaying` (`self.AUD_Rotate_SFX`)))
    (`AudioComponent.FadeIn` (`self.AUD_Rotate_SFX`) 0.25 1.0 0.0 "Linear"))
  (set `self.deltaRotation` (struct :`Yaw` 2.0))
  (bind (_direction _scale _rotation) (`Timeline|ScaleAnim` :!label _label)
    (:`Update`
      (`SceneComponent.SetRelativeScale3D` (`self.RotatorGuide002`) (`KismetMathLibrary.Conv_DoubleToVector` (`KismetMathLibrary.Lerp` 0.04 0.045 _scale)))
      (`SceneComponent.K2_AddRelativeRotation` _sm_handlearrows (`KismetMathLibrary.MakeRotator` 0.0 0.0 (`KismetMathLibrary.Lerp` 0.0 5.0 _rotation)) false false)
      (`SceneComponent.SetRelativeScale3D` _sm_handlearrows (`KismetMathLibrary.VLerp` (200.0 200.0 200.0) (225.0 225.0 225.0) _scale))
      (`MeshComponent.SetScalarParameterValueOnMaterials` (`self.SM_HandleArrows`) "scale" (`KismetMathLibrary.Lerp` 0.1 0.2 _scale)))))

(event `ScaleDown`
  ;[0 0 0 0.779] AUD
  (`AudioComponent.FadeOut` (`self.AUD_Rotate_SFX`) 0.25 0.0 "Linear")
  (set `self.deltaRotation` (struct :`Yaw` 0.25))
  (goto _label :!via `Reverse`))

(event `self.ReceiveTick`
  (params (DeltaSeconds :type "Float (single-precision)"))
  (`SceneComponent.K2_AddRelativeRotation` (`self.RotatorGuide002`) (`self.deltaRotation`) false false))

(fn `UserConstructionScript`
  (`TimelineComponent.SetPlayRate` (`self.ScaleAnim`) 3.5))