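; Mixed-reality player pawn that detects what the user looks at and can be repositioned relative to a transform.
; Each tick it line-traces a custom object type along HMD eye gaze, falling back to head pose without a headset.
; Hit actors implementing BP_GazeTriggerInterface receive gaze begin, ongoing and end messages, tracked via LastHitActor.
; TeleportPlayerRelativeTo offsets the pawn using head pose, keeps only yaw, then resets HMD tracking if connected.
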(event `self.ReceiveTick`
  (params (DeltaSeconds :type "Float (single-precision)"))
  (bind (_returnvalue_location _returnvalue_rotation) (`KismetMathLibrary.BreakTransform` (`UxtFunctionLibrary.GetHeadPose`)))
  (bind _returnvalue_location_2 (`KismetMathLibrary.BreakTransform` (`UxtFunctionLibrary.GetHeadPose`)))
  ;[1 1 1] User gaze ray on tick
  (bind _returnvalue (`HeadMountedDisplayFunctionLibrary.GetTrackingToWorldTransform`))
  (bind _outgazedata (`EyeTrackerFunctionLibrary.GetGazeData`))
  (bind _outhit (`KismetSystemLibrary.LineTraceSingleForObjects` (select `bool` (`HeadMountedDisplayFunctionLibrary.IsHeadMountedDisplayConnected`) :`false` _returnvalue_location_2 :`true` (`KismetMathLibrary.TransformLocation` _returnvalue (break `EyeTrackerGazeData` _outgazedata))) (select `bool` (`HeadMountedDisplayFunctionLibrary.IsHeadMountedDisplayConnected`) :`false` (* (`KismetMathLibrary.GetForwardVector` _returnvalue_rotation) (`self.GazeRayLength`)) :`true` (`KismetMathLibrary.TransformDirection` _returnvalue (+ (break `EyeTrackerGazeData` _outgazedata) (* (`.GazeDirection` (break `EyeTrackerGazeData` _outgazedata)) (`self.GazeRayLength`))))) (`|MakeArray` "ObjectTypeQuery7" :!type "EObjectTypeQuery Enum")))
  (if (`GameplayStatics.BreakHitResult` _outhit)
    (if (`KismetSystemLibrary.DoesImplementInterface` (`.HitActor` (`GameplayStatics.BreakHitResult` _outhit)) "/Game/Framework/BP_GazeTriggerInterface.BP_GazeTriggerInterface_C")
      (if (!= (`self.LastHitActor`) (`.HitActor` (`GameplayStatics.BreakHitResult` _outhit)))
        (message `/Game/Framework/BP_GazeTriggerInterface.OnGazeBegin` (`.HitActor` (`GameplayStatics.BreakHitResult` _outhit)))
        (set `self.LastHitActor` (`.HitActor` (`GameplayStatics.BreakHitResult` _outhit)))
        (else
          (message `/Game/Framework/BP_GazeTriggerInterface.OnGaze` (`.HitActor` (`GameplayStatics.BreakHitResult` _outhit)))))
      (else
        (bind _lasthitactor (`self.LastHitActor` :!label _label)
          (:`then`
            (message `/Game/Framework/BP_GazeTriggerInterface.OnGazeEnd` _lasthitactor)
            (set `self.LastHitActor` null))
          (:`else`))))
    (else
      (goto _label))))

(fn `TeleportPlayerRelativeTo`
  (params (RelativeTransform :type "Transform Structure"))
  (bind (_returnvalue_location _returnvalue_rotation _returnvalue_scale) (`KismetMathLibrary.BreakTransform` (`UxtFunctionLibrary.GetHeadPose`)))
  (bind _returnvalue (`KismetMathLibrary.MakeRelativeTransform` (`KismetMathLibrary.MakeTransform` _returnvalue_location _returnvalue_rotation _returnvalue_scale) RelativeTransform))
  (`self.K2_SetActorLocationAndRotation` (.location _returnvalue) (`KismetMathLibrary.MakeRotator` 0.0 0.0 (.yaw (.rotation _returnvalue))))
  (if (`HeadMountedDisplayFunctionLibrary.IsHeadMountedDisplayConnected`)
    (`HeadMountedDisplayFunctionLibrary.ResetOrientationAndPosition` 0.0)))

(fn `UserConstructionScript`)