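; Mixed reality placement proxy: a manipulable level miniature that the player positions before the content is anchored.
; UXT grab events lock rotation to yaw, drive a focus material timeline and toggle the bounds idle state, whose scale Tick interpolates.
; Releasing the child BP_PlayButton creates an anchor at the proxy transform via BP_MRGameMode, teleports the pawn relative to ProxyOrigin and resets the actor transform.
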(event `self.UxtBoundsControl.OnManipulationStarted`
  (params (Manipulator :type "UxtBoundsControlComponent Object Reference") (AffordanceInfo :type "UxtBoundsControlAffordanceInfo Structure (by ref)") (GrabbedComponent :type "UxtGrabTargetComponent Object Reference"))
  ;[1 1 1] Interactivity
  (`self.stopBoundsIdle`))

(event `self.ReceiveBeginPlay`
  (`|ExecutionSequence`
    (:`then_0`
      (bind _asbp_play_button (cast `/Game/Blueprints/BP_PlayButton` (`ChildActorComponent.ChildActor` (`self.ChildActor`))))
      (bind _output_get (set `self.Button` _asbp_play_button))
      (add `/Game/Blueprints/BP_PlayButton.EventDisp_ButtonReleased` _output_get (delegate `AnchorContent`)))
    (:`then_1`
      (`self.startBoundsIdle`))))

(event `startBoundsIdle`
  ;[1 1 1] Interactivity
  ;;[1 1 1] Bounds idle anim
  (set `self.boundsIdleState` true)
  (bind (_direction _lerp) (`Timeline|BoundsIdleAnim` :!label _label)
    (:`Update`
      (set `self.animatedIdleScale` (`KismetMathLibrary.MakeVector` 0.875 0.875 0.875)))))

(event `self.UxtBoundsControl.OnManipulationEnded`
  (params (Manipulator :type "UxtBoundsControlComponent Object Reference") (AffordanceInfo :type "UxtBoundsControlAffordanceInfo Structure (by ref)") (GrabbedComponent :type "UxtGrabTargetComponent Object Reference"))
  ;[1 1 1] Interactivity
  (`self.startBoundsIdle`))

(event `stopBoundsIdle`
  ;[1 1 1] Interactivity
  ;;[1 1 1] Bounds idle anim
  (set `self.boundsIdleState` false)
  (goto _label :!via `Stop`))

(event `AnchorContent`
  (`KismetMaterialLibrary.SetScalarParameterValue` "/Game/Materials/PostProcess/Outliner/MPC_Outliner.MPC_Outliner" "contentPlacement")
  (`|ExecutionSequence`
    (:`then_0`
      ;[1 1 1] Create Content Anchor
      (bind _asbp_mrgame_mode (cast `/Game/Framework/BP_MRGameMode` (`GameplayStatics.GetGameMode`)))
      (bind _success (`/Game/Framework/BP_MRGameMode.Create Anchor` _asbp_mrgame_mode (`SceneComponent.K2_GetComponentToWorld` (`self.LevelProxy`)) (`self.PinID`)))
      (if _success
        (`KismetSystemLibrary.PrintString` "Level anchor pin creation succeeded")
        (else
          (`KismetSystemLibrary.PrintString` "Level anchor pin creation failed")))
      (set `self.ContentPlaced` true))
    (:`then_1`
      ;[1 1 1] Teleport pawn to appropriate level position
      (bind _asbp_mrpawn (cast `/Game/Framework/BP_MRPawn` (`GameplayStatics.GetPlayerPawn` 0)))
      (`/Game/Framework/BP_MRPawn.TeleportPlayerRelativeTo` _asbp_mrpawn (`SceneComponent.K2_GetComponentToWorld` (`self.ProxyOrigin`)))
      (`self.K2_SetActorTransform` (`KismetMathLibrary.MakeTransform` (0.0 0.0 0.0))))))

(event `self.UxtGenericManipulator.OnEnterGrabFocus`
  (params (Grabbable :type "UxtGrabTargetComponent Object Reference") (Pointer :type "UxtNearPointerComponent Object Reference"))
  (bind _dynamicmaterialislands (`self.dynamicMaterialislands`))
  ;[1 1 1] Interactivity
  ;;[1 1 1] focus animation
  (bind (_direction _scale _colour) (`Timeline|FocusAnim` :!label _label_2)
    (:`Update`
      (`MaterialInstanceDynamic.SetScalarParameterValue` _dynamicmaterialislands "scale" (`KismetMathLibrary.Lerp` 0.0 0.5 _scale))
      (`MaterialInstanceDynamic.SetVectorParameterValue` _dynamicmaterialislands "Colour" (`KismetMathLibrary.LinearColorLerp` (struct :`R` 0.019608 :`G` 0.043137 :`B` 0.07451 :`A` 1.0) (struct :`R` 0.025634 :`G` 0.092773 :`B` 0.182292 :`A` 1.0) _colour)))))

(event `self.UxtGenericManipulator.OnUpdateGrab`
  (params (Grabbable :type "UxtGrabTargetComponent Object Reference") (GrabPointer :type "UxtGrabPointerData Structure"))
  (bind (_returnvalue_roll _returnvalue_pitch _returnvalue_yaw) (`KismetMathLibrary.BreakRotator` (`SceneComponent.K2_GetComponentRotation` (`self.LevelProxy`))))
  ;[1 1 1] Lock XY axis on 2 handed rotation
  (`SceneComponent.K2_SetWorldRotation` (`self.LevelProxy`) (`KismetMathLibrary.MakeRotator` 0.0 0.0 _returnvalue_yaw) false false))

(event `self.UxtGenericManipulator.OnExitGrabFocus`
  (params (Grabbable :type "UxtGrabTargetComponent Object Reference") (Pointer :type "UxtNearPointerComponent Object Reference"))
  ;[1 1 1] Interactivity
  (goto _label_2 :!via `Reverse`))

(event `self.UxtGenericManipulator.OnBeginGrab`
  (params (Grabbable :type "UxtGrabTargetComponent Object Reference") (GrabPointer :type "UxtGrabPointerData Structure"))
  ;[1 1 1] Interactivity
  (`self.stopBoundsIdle`)
  (goto _label_2 :!via `Reverse`))

(event `self.UxtGenericManipulator.OnEndGrab`
  (params (Grabbable :type "UxtGrabTargetComponent Object Reference") (GrabPointer :type "UxtGrabPointerData Structure"))
  ;[1 1 1] Interactivity
  (`self.startBoundsIdle`)
  (goto _label_2))

(event `self.ReceiveTick`
  (params (DeltaSeconds :type "Float (single-precision)"))
  (bind _boundsidlestate (`self.boundsIdleState`))
  ;[1 1 1] Interactivity
  ;;[1 1 1] Update bounds scale
  (set `self.lerpBoundsScale` (`KismetMathLibrary.FInterpTo` (`self.lerpBoundsScale`) (`KismetMathLibrary.SelectFloat` 0.0 1.0 _boundsidlestate) (`GameplayStatics.GetWorldDeltaSeconds`) (`KismetMathLibrary.SelectFloat` 1.0 5.0 _boundsidlestate)))
  (`SceneComponent.SetRelativeScale3D` (`self.Bounds`) (`KismetMathLibrary.VLerp` (`self.animatedIdleScale`) (`KismetMathLibrary.MakeVector` 0.825 0.825 0.825) (`self.lerpBoundsScale`))))

(fn `UserConstructionScript`
  (bind _returnvalue (`PrimitiveComponent.CreateDynamicMaterialInstance` (`self.Bounds`) 0 "/Game/Art/ProxyGeo/MI_ProxyGeo_v3_Bounds.MI_ProxyGeo_v3_Bounds" "None"))
  (set `self.dynamicMaterialBounds` _returnvalue)
  (bind _returnvalue_2 (`PrimitiveComponent.CreateDynamicMaterialInstance` (`self.LevelProxy`) 0 "/Game/Art/ProxyGeo/M_ProxyGeo_v4.M_ProxyGeo_v4" "None"))
  (set `self.dynamicMaterialislands` _returnvalue_2)
  (`TimelineComponent.SetPlayRate` (`self.FocusAnim`) 2.0))