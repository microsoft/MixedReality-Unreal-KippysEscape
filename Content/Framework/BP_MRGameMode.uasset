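; Mixed reality game mode that creates, saves and loads named spatial anchors through the Windows Mixed Reality anchor store.
; CreateAnchor checks that the store is ready, removes all current AR pins, then pins the given transform under the ID and saves it.
; After saving, it reloads the pin via TryLoadAnchor, which searches the stored pins for a matching ID and returns success with the pin.
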(fn `Create Anchor`
  (params (ContentTransform :type "Transform Structure") (AnchorID :type String))
  (returns (Success :type Boolean) (Anchor :type "WMRARPin Object Reference"))
  (locals (RemoveExisting :type Boolean) (ID :type String))
  (set `local.ID` AnchorID)
  (if (`HoloLensARFunctionLibrary.IsWMRAnchorStoreReady`)
    (`self.RemoveExistingAnchors`)
    (bind _returnvalue (`HoloLensARFunctionLibrary.CreateNamedARPin` (`KismetStringLibrary.Conv_StringToName` (`local.ID`)) ContentTransform))
    (bind _returnvalue_2 (`HoloLensARFunctionLibrary.SaveARPinToWMRAnchorStore` _returnvalue))
    (if _returnvalue_2
      (`KismetSystemLibrary.PrintString` "Anchor Saved" false)
      (bind (_success _loadedpin) (`self.TryLoadAnchor` (`local.ID`)))
      (return _success _loadedpin)
      (else
        (`KismetSystemLibrary.PrintString` "Error Anchor Not Saved" false)
        (return false null)))
    (else
      (`KismetSystemLibrary.PrintString` "Anchor store not ready" false)
      (return false null))))

(fn `RemoveExistingAnchors`
  (bind _returnvalue (`ARBlueprintLibrary.GetAllPins`))
  (for _array_element _returnvalue
    (`ARBlueprintLibrary.RemovePin` _array_element))
  (return))

(fn `TryLoadAnchor`
  (params (AnchorID :type String))
  (returns (Success :type Boolean) (LoadedPin :type "WMRARPin Object Reference"))
  (locals (Pin :type "WMRARPin Object Reference"))
  (bind _returnvalue (`HoloLensARFunctionLibrary.LoadWMRAnchorStoreARPins`))
  (for _array_element _returnvalue
    (if (`KismetStringLibrary.EqualEqual_StrStr` (`WMRARPin.GetAnchorId` _array_element) AnchorID)
      (set `local.Pin` _array_element)))
  (bind _pin (`local.Pin`)
    (:`then`
      (return true _pin))
    (:`else`
      (return false null))))

(fn `UserConstructionScript`)