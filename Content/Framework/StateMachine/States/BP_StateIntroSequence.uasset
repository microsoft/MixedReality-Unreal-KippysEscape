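; BP_StateIntroSequence is a state machine state that plays the intro sequence for the Astro character.
; On entry it unhides Astro with low gravity and fades in the level's ambient audio.
; Tick checks flag-gated steps: teleport to start, boot after a delay, move to the wave waypoint, wave, then switch to another state.
; Steps after boot wait on the animation Blueprint's locomotion state before firing.
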(fn `Init`
  (`parent.Init`)
  (bind _returnvalue (`GameplayStatics.GetActorOfClass` "/Script/Engine.AmbientSound"))
  (set `self.AmbientAudio` _returnvalue))

(fn `On Entry`
  (`parent.On Entry`)
  (`self.SetActorHiddenInGame` (`self.Astro`) false)
  (set `CharacterMovementComponent.GravityScale` 0.05 (`Character.CharacterMovement` (`self.Astro`)))
  (`AudioComponent.FadeIn` (`AmbientSound.AudioComponent` (`self.AmbientAudio`)) 2.0 1.0 0.0 "Linear"))

(fn `OnTick`
  (params (TimeInState :type "Float (double-precision)"))
  (`parent.OnTick` TimeInState)
  (`|ExecutionSequence`
    (:`then_0`
      (if (not (`self.AstroTeleported`))
        (set `self.AstroTeleported` true)
        (`/Game/Blueprints/Astro/BP_Astro.TeleportTo` (`self.Astro`) (`BlueprintMapLibrary.Map_Find` (`self.Waypoints`) "StartLocation"))
        (elif (and (> TimeInState 5.0) (not (`self.BootStarted`)))
          (`/Game/Blueprints/Astro/BP_Astro.EnableBoot` (`self.Astro`))
          (set `self.BootStarted` true))))
    (:`then_1`
      (if (and (`self.BootStarted`) (`|EnumEquality` (`/Game/Blueprints/Astro/ABP_Astro.LocomotionState` (`/Game/Blueprints/Astro/BP_Astro.ABP` (`self.Astro`))) "NewEnumerator0") (not (`self.HasCharacterReachedWaypoint` "CharacterWaveLocation")))
        (`self.MoveCharacterToWaypoint` "CharacterWaveLocation")))
    (:`then_2`
      (if (and (`self.HasCharacterReachedWaypoint` "CharacterWaveLocation") (not (`self.AstroWaved`)) (`|EnumEquality` (`/Game/Blueprints/Astro/ABP_Astro.LocomotionState` (`/Game/Blueprints/Astro/BP_Astro.ABP` (`self.Astro`))) "NewEnumerator0"))
        (`/Game/Blueprints/Astro/BP_Astro.Wave` (`self.Astro`) 4.0 false)
        (set `self.AstroWaved` true)))
    (:`then_3`
      (if (and (`self.AstroWaved`) (`|EnumEquality` (`/Game/Blueprints/Astro/ABP_Astro.LocomotionState` (`/Game/Blueprints/Astro/BP_Astro.ABP` (`self.Astro`))) "NewEnumerator0"))
        (`/Game/Framework/StateMachine/BP_StateManager.ChangeState` (`self.StateManager`) "NewEnumerator3")))))

(fn `UserConstructionScript`)