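; BP_StateRocketBlastOff is a game state machine state that runs the rocket launch sequence leading to game over.
; Init caches the level's BP_Rocket, and entering the state triggers the rocket's blast-off event and has Astro enter the rocket.
; Each state tick checks whether the rocket is in space, then has the StateManager switch to the game-over state.
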(fn `Init`
  (`parent.Init`)
  (bind _returnvalue (`GameplayStatics.GetActorOfClass` "/Game/Blueprints/BP_Rocket.BP_Rocket_C"))
  (set `self.Rocket` _returnvalue))

(fn `On Entry`
  (`parent.On Entry`)
  (`/Game/Blueprints/BP_Rocket.Event BlastOff` (`self.Rocket`))
  (`/Game/Blueprints/Astro/BP_Astro.EnterRocket` (`self.Astro`)))

(fn `OnExit`
  (`parent.OnExit`))

(fn `OnTick`
  (params (TimeInState :type "Float (double-precision)"))
  (`parent.OnTick` TimeInState)
  ;[1 1 1] Game over when rocket in space
  (if (`/Game/Blueprints/BP_Rocket.InSpace` (`self.Rocket`))
    (`/Game/Framework/StateMachine/BP_StateManager.ChangeState` (`self.StateManager`) "NewEnumerator10")))

(fn `UserConstructionScript`
  (`parent.UserConstructionScript`))