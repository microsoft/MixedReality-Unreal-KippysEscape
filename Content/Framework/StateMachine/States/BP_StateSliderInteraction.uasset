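; BP_StateSliderInteraction is a state machine state that runs the twin-slider interaction for deploying the island bridge.
; Init finds the sliders, bridge and temple island actors in the level; entry activates the sliders, powers up the island and lights the bridge.
; Each tick triggers a one-time slider highlight hint after a delay and changes state once the bridge is deployed.
; Exit clears the hints and disables Astro's pointing.
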(fn `Init`
  (`parent.Init`)
  (`|ExecutionSequence`
    (:`then_0`
      (bind _outactors (`GameplayStatics.GetAllActorsOfClass` "/Game/Blueprints/BP_TwinSlider.BP_TwinSlider_C"))
      (set `self.LaunchpadTwinSliders` _outactors))
    (:`then_1`
      (bind _returnvalue (`GameplayStatics.GetActorOfClass` "/Game/Blueprints/BP_Island03Bridge.BP_Island03Bridge_C"))
      (set `self.LaunchpadBridge` _returnvalue))
    (:`then_2`
      (bind _returnvalue_2 (`GameplayStatics.GetActorOfClass` "/Game/Blueprints/SM_Temple_Blueprint.SM_Temple_Blueprint_C"))
      (set `self.Island` _returnvalue_2))))

(fn `On Entry`
  (`parent.On Entry`)
  (`|ExecutionSequence`
    (:`then_0`
      (for _array_element (`self.LaunchpadTwinSliders`)
        (`/Game/Blueprints/BP_TwinSlider.ActivateSlider` _array_element)))
    (:`then_1`
      (`/Game/Blueprints/SM_Temple_Blueprint.PowerUp` (`self.Island`)))
    (:`then_2`
      (`/Game/Blueprints/BP_Island03Bridge.TurnBridgeEmissiveOn` (`self.LaunchpadBridge`)))))

(fn `OnExit`
  (`parent.OnExit`)
  (`/Game/Blueprints/Astro/BP_Astro.DisablePoint` (`self.Astro`))
  (for _array_element (`self.LaunchpadTwinSliders`)
    (`/Game/Blueprints/BP_TwinSlider.DeactivateHint` _array_element)))

(fn `OnTick`
  (params (TimeInState :type "Float (double-precision)"))
  (`parent.OnTick` TimeInState)
  (`|ExecutionSequence`
    (:`then_0`
      ;[1 1 1] Highlight hint
      (if (and (not (`self.HighlightHintActivated`)) (> TimeInState (`self.TimeUntilHighlightHint`)))
        (set `self.HighlightHintActivated` true)
        (for _array_element (`self.LaunchpadTwinSliders`)
          (`/Game/Blueprints/BP_TwinSlider.ActivateHint` _array_element))))
    (:`then_2`
      (if (`/Game/Blueprints/BP_Island03Bridge.Deployed` (`self.LaunchpadBridge`))
        (`/Game/Framework/StateMachine/BP_StateManager.ChangeState` (`self.StateManager`) "NewEnumerator7")))))

(fn `UserConstructionScript`
  (`parent.UserConstructionScript`))