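; State machine state for the gem island puzzle, where three colored gems must be placed in sockets while Astro accompanies.
; Init maps gems, sockets and plinths by color, and entry activates each set with staggered delays.
; Tick powers up the island when Astro arrives, fires timed hints, and moves Astro by waypoint according to time and gem progress.
; Once all gems are inserted, it extends the bridge and changes state.
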(fn `ActivateGemComponents`
  (params (GemColor :type "/Game/Blueprints/Enums/E_GemColor Enum" :default "NewEnumerator0") (Delay :type "Float (double-precision)"))
  (`|ExecutionSequence`
    (:`then_0`
      (`/Game/Blueprints/BP_Gem.ActivateGem` (`BlueprintMapLibrary.Map_Find` (`self.GemsMap`) GemColor) Delay))
    (:`then_1`
      (`/Game/Blueprints/BP_GemSocket.Activate` (`BlueprintMapLibrary.Map_Find` (`self.SocketMap`) GemColor) Delay))
    (:`then_2`
      (`/Game/Blueprints/BP_Plinth.ActivatePlinth` (`BlueprintMapLibrary.Map_Find` (`self.PlinthMap`) GemColor) Delay (`/Game/Blueprints/Islands/BP_Island02.MainMaskPosition` (`self.Island2Geo`))))))

(fn `ActivateHint`
  (params (GemColor :type "/Game/Blueprints/Enums/E_GemColor Enum" :default "NewEnumerator0"))
  (bind _value (`BlueprintMapLibrary.Map_Find` (`self.GemsMap`) GemColor))
  (if (not (`/Game/Blueprints/BP_Gem.Inserted` _value))
    (`/Game/Blueprints/BP_Gem.ActivateHint` _value)))

(fn `GetGemInserted`
  (params (Color :type "/Game/Blueprints/Enums/E_GemColor Enum" :default "NewEnumerator0"))
  (returns (Inserted :type Boolean))
  (bind (_value _returnvalue) (`BlueprintMapLibrary.Map_Find` (`self.SocketMap`) Color))
  (return (and (`/Game/Blueprints/BP_GemSocket.GemInserted` _value) _returnvalue)))

(fn `Init`
  (`parent.Init`)
  (`|ExecutionSequence`
    (:`then_0`
      (bind _outactors (`GameplayStatics.GetAllActorsOfClass` "/Game/Blueprints/BP_Gem.BP_Gem_C"))
      (set `self.GemsArray` _outactors)
      (for _array_element (`self.GemsArray`)
        (`BlueprintMapLibrary.Map_Add` (`self.GemsMap`) (`/Game/Blueprints/BP_Gem.GemColor` _array_element) _array_element)))
    (:`then_1`
      (bind _outactors_2 (`GameplayStatics.GetAllActorsOfClass` "/Game/Blueprints/BP_GemSocket.BP_GemSocket_C"))
      (bind _output_get (set `self.SocketArray` _outactors_2))
      (for _array_element_2 _output_get
        (`BlueprintMapLibrary.Map_Add` (`self.SocketMap`) (`/Game/Blueprints/BP_GemSocket.GemColor` _array_element_2) _array_element_2)))
    (:`then_2`
      (bind _returnvalue (`GameplayStatics.GetActorOfClass` "/Game/Blueprints/BP_Island02Bridge.BP_Island02Bridge_C"))
      (set `self.Island2Bridge` _returnvalue))
    (:`then_3`
      (bind _returnvalue_2 (`GameplayStatics.GetActorOfClass` "/Game/Blueprints/Islands/BP_Island02.BP_Island02_C"))
      (set `self.Island2Geo` _returnvalue_2))
    (:`then_4`
      (bind _outactors_3 (`GameplayStatics.GetAllActorsOfClass` "/Game/Blueprints/BP_Plinth.BP_Plinth_C"))
      (bind _output_get_2 (set `self.Plinths` _outactors_3))
      (for _array_element_3 _output_get_2
        (`BlueprintMapLibrary.Map_Add` (`self.PlinthMap`) (`/Game/Blueprints/BP_Plinth.GemColour` _array_element_3) _array_element_3)))))

(fn `On Entry`
  (locals (GemActivationIncrement :type "Float (double-precision)" :default 0.5) (SocketActivationIncement :type "Float (double-precision)") (PlinthActivationIncrement :type "Float (double-precision)"))
  (`parent.On Entry`)
  (`|ExecutionSequence`
    (:`then_0`
      ;[1 1 1] Move character to initial position
      (`self.MoveCharacterToWaypoint` "GemIslandStart"))
    (:`then_1`
      ;[1 1 1] Activate Gems, Sockets and Plinths
      (`self.ActivateGemComponents` "NewEnumerator2" 0.75)
      (`self.ActivateGemComponents` "NewEnumerator0" 2.0)
      (`self.ActivateGemComponents` "NewEnumerator1" 3.25))))

(fn `OnExit`
  (`parent.OnExit`)
  (bind _values (`BlueprintMapLibrary.Map_Values` (`self.GemsMap`)))
  (for _array_element _values
    (`/Game/Blueprints/BP_Gem.DeactivateHint` _array_element)))

(fn `OnTick`
  (params (TimeInState :type "Float (double-precision)"))
  (locals (InsertedGems :type Integer))
  (bind (_value _returnvalue) (`BlueprintMapLibrary.Map_Find` (`self.GemsMap`) "NewEnumerator0"))
  (`parent.OnTick` TimeInState)
  (`|ExecutionSequence`
    (:`then_0`
      ;[1 1 1] Character hint
      (if (and (not (`self.CharacterHintActivated`)) (> TimeInState (`self.TimeUntilCharacterHint`)))
        (set `self.CharacterHintActivated` true)
        (for _array_element (`self.GemsArray`)
          (if (not (`/Game/Blueprints/BP_Gem.Inserted` _array_element))
            (set `self.PointLocation` (`SceneComponent.K2_GetComponentLocation` (`/Game/Blueprints/BP_Gem.GemMesh` _array_element)))))
        (`/Game/Blueprints/Astro/BP_Astro.EnablePoint` (`self.Astro`) (`self.PointLocation`) 3.0)))
    (:`then_1`
      ;[1 1 1] Highlight hint
      (if (and (not (`self.HighlightHintActivated`)) (> TimeInState (`self.TimeUntilHighlightHint`)))
        (set `self.HighlightHintActivated` true)
        (`self.ActivateHint` "NewEnumerator0")
        (`self.ActivateHint` "NewEnumerator1")
        (`self.ActivateHint` "NewEnumerator2")))
    (:`then_2`
      ;[1 1 1] Astro Go To Red Gem
      (if (and (> TimeInState (`self.TimeUntilAstroInspectGem`)) _returnvalue (not (`/Game/Blueprints/BP_Gem.Inserted` _value)) (not (`/Game/Blueprints/BP_Gem.Held` _value)) (not (`self.CharacterMovedToGem`)) (not (`self.CharacterMovedToBridge`)))
        (set `self.CharacterMovedToGem` true)
        (`/Game/Blueprints/Astro/BP_Astro.PlayAudio` (`self.Astro`) "NewEnumerator1")
        (`self.MoveCharacterToWaypoint` "RedGem")))
    (:`then_3`
      ;[1 1 1] Astro Move to Bridge After 2 Gem Insert
      (if (not (`self.CharacterMovedToBridge`))
        (set `local.InsertedGems` 0)
        (for _array_element_2 (`self.GemsArray`)
          (if (`/Game/Blueprints/BP_Gem.Inserted` _array_element_2)
            (`/Engine/EditorBlueprintResources/StandardMacros.IncrementInt` (`local.InsertedGems`))))
        (if (> (`local.InsertedGems`) 1)
          (if (`self.GetGemInserted` "NewEnumerator1")
            (`self.MoveCharacterToWaypoint` "GemIslandExitBridge")
            (else
              (`self.MoveCharacterToWaypoint` "GemIslandWaitForGreenGem")))
          (set `self.CharacterMovedToBridge` true))))
    (:`then_4`
      ;[1 1 1] Advance state if all gems inserted
      (if (and (`self.GetGemInserted` "NewEnumerator0") (`self.GetGemInserted` "NewEnumerator1") (`self.GetGemInserted` "NewEnumerator2") (`self.CharacterMovedToBridge`))
        (`/Game/Blueprints/Astro/BP_Astro.DisablePoint` (`self.Astro`))
        (`/Game/Blueprints/Astro/BP_Astro.TriggerExpression` (`self.Astro`) "NewEnumerator7" 5.0)
        (`/Game/Blueprints/BP_Island02Bridge.ExtendBridge` (`self.Island2Bridge`))
        (`/Game/Framework/StateMachine/BP_StateManager.ChangeState` (`self.StateManager`) "NewEnumerator5")))
    (:`then_5`
      (if (and (not (`self.IslandPoweredUp`)) (`self.HasCharacterReachedWaypoint` "GemIslandStart"))
        (set `self.IslandPoweredUp` true)
        (`/Game/Blueprints/Islands/BP_Island02.EmissiveLinesPowerUp` (`self.Island2Geo`))))))

(fn `UserConstructionScript`
  (`parent.UserConstructionScript`))