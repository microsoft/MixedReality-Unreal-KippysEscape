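; State machine state that restores a saved AR anchor to position the level in a mixed reality game.
; On entry it starts an AR session, asks BP_MRGameMode to load the pin and moves BP_LevelPlacementProxy to it.
; Each tick it waits for the pin to track, re-applies its transform and switches to content adjustment.
; A missing pin or headset also leads to content adjustment, while a wrong game mode triggers the error state.
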(fn `On Entry`
  (`parent.On Entry`)
  (`|ExecutionSequence`
    (:`then_0`
      (`ARBlueprintLibrary.StartARSession` "/Game/Framework/ARSesh.ARSesh"))
    (:`then_1`
      (bind _returnvalue (`GameplayStatics.GetActorOfClass` "/Game/Framework/StateMachine/BP_StateManager.BP_StateManager_C"))
      (set `self.StateManager` _returnvalue))
    (:`then_2`
      (bind _returnvalue_2 (`GameplayStatics.GetActorOfClass` "/Game/Framework/BP_LevelPlacementProxy.BP_LevelPlacementProxy_C"))
      (set `self.LevelPlacementProxy` _returnvalue_2))
    (:`then_3`
      ;[1 1 1] Try Load Anchor
      (bind _asbp_mrgame_mode (cast `/Game/Framework/BP_MRGameMode` (`GameplayStatics.GetGameMode`))
        (:`then`
          (bind _output_get (set `self.GameMode` _asbp_mrgame_mode))
          (bind (_success _loadedpin) (`/Game/Framework/BP_MRGameMode.TryLoadAnchor` _output_get (`self.PinID`)))
          (if _success
            (bind _output_get_2 (set `self.Pin` _loadedpin))
            (`self.K2_SetActorTransform` (`self.LevelPlacementProxy`) (`ARPin.GetLocalToWorldTransform` _output_get_2) false false)
            (else
              (`KismetSystemLibrary.PrintString` "No pin found to anchor level." false) ; TODO: Need to move content placement proxy
              (`/Game/Framework/StateMachine/BP_StateManager.ChangeState` (`self.StateManager`) "NewEnumerator1") ; Go to content adjustment state
            )))
        (:`CastFailed`
          (`KismetSystemLibrary.PrintString` "Failed to get correct game mode." false)
          (`/Game/Framework/StateMachine/BP_StateManager.ChangeState` (`self.StateManager`) "NewEnumerator14") ; Go to error state
        )))))

(fn `OnTick`
  (params (TimeInState :type "Float (double-precision)"))
  (`parent.OnTick` TimeInState)
  (if (`HeadMountedDisplayFunctionLibrary.IsHeadMountedDisplayConnected`)
    (switch `EARTrackingState` (`ARPin.GetTrackingState` (`self.Pin`))
      (:`Tracking`
        (`self.K2_SetActorTransform` (`self.LevelPlacementProxy`) (`ARPin.GetLocalToWorldTransform` (`self.Pin`)) false false)
        (`/Game/Framework/StateMachine/BP_StateManager.ChangeState` (`self.StateManager`) "NewEnumerator1") ; Go to content adjust state
      ))
    (else
      (`/Game/Framework/StateMachine/BP_StateManager.ChangeState` (`self.StateManager`) "NewEnumerator1") ; Go to content adjust state
    )))

(fn `UserConstructionScript`)