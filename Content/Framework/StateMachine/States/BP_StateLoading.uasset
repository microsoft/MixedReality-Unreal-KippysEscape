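; Loading state for the game's state machine, holding until the four Island streaming levels are loaded.
; On Entry finds and caches the BP_StateManager actor in the world.
; OnTick polls each island's streaming level and, once all report loaded, has the manager initialize the game states and switch to another state.
; It only checks load status and does not request the streaming itself.
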(fn `On Entry`
  (`parent.On Entry`)
  (bind _returnvalue (`GameplayStatics.GetActorOfClass` "/Game/Framework/StateMachine/BP_StateManager.BP_StateManager_C"))
  (set `self.StateManager` _returnvalue))

(fn `OnExit`
  (`parent.OnExit`))

(fn `OnTick`
  (params (TimeInState :type "Float (double-precision)"))
  (`parent.OnTick` TimeInState)
  (if (and (`LevelStreaming.IsLevelLoaded` (`GameplayStatics.GetStreamingLevel` "Island_01")) (`LevelStreaming.IsLevelLoaded` (`GameplayStatics.GetStreamingLevel` "Island_02")) (`LevelStreaming.IsLevelLoaded` (`GameplayStatics.GetStreamingLevel` "Island_03")) (`LevelStreaming.IsLevelLoaded` (`GameplayStatics.GetStreamingLevel` "Island_04")))
    (`/Game/Framework/StateMachine/BP_StateManager.InitGameStates` (`self.StateManager`))
    (`/Game/Framework/StateMachine/BP_StateManager.ChangeState` (`self.StateManager`) "NewEnumerator2")))

(fn `UserConstructionScript`
  (`parent.UserConstructionScript`))