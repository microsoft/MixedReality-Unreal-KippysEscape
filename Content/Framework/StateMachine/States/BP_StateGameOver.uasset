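; State machine state for game over, offering the quit and reset buttons.
; On entry it finds the BP_QuitButton and BP_ResetButton actors in the level, unhides them and activates them.
; Each state tick it checks the reset button's pressed flag, then deactivates and hides both buttons and asks the StateManager to change state.
; The quit button's press is not handled here.
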(fn `Init`
  (`parent.Init`))

(fn `On Entry`
  (`parent.On Entry`)
  (`|ExecutionSequence`
    (:`then_0`
      (bind _returnvalue (`GameplayStatics.GetActorOfClass` "/Game/Blueprints/BP_QuitButton.BP_QuitButton_C"))
      (set `self.QuitButton` _returnvalue))
    (:`then_1`
      (bind _returnvalue_2 (`GameplayStatics.GetActorOfClass` "/Game/Blueprints/BP_ResetButton.BP_ResetButton_C"))
      (set `self.ResetButton` _returnvalue_2))
    (:`then_2`
      (`self.SetActorHiddenInGame` (`self.QuitButton`) false)
      (`self.SetActorHiddenInGame` (`self.ResetButton`) false)
      (`/Game/Blueprints/BP_QuitButton.Activate` (`self.QuitButton`))
      (`/Game/Blueprints/BP_ResetButton.Activate` (`self.ResetButton`)))))

(fn `OnExit`
  (`parent.OnExit`))

(fn `OnTick`
  (params (TimeInState :type "Float (double-precision)"))
  (`parent.OnTick` TimeInState)
  (if (`/Game/Blueprints/BP_ResetButton.PressedOnce` (`self.ResetButton`))
    (`/Game/Blueprints/BP_QuitButton.Deactivate` (`self.QuitButton`))
    (`self.SetActorHiddenInGame` (`self.QuitButton`) true)
    (`/Game/Blueprints/BP_ResetButton.Deactivate` (`self.ResetButton`))
    (`self.SetActorHiddenInGame` (`self.ResetButton`) true)
    (`/Game/Framework/StateMachine/BP_StateManager.ChangeState` (`self.StateManager`) "NewEnumerator16")))

(fn `UserConstructionScript`
  (`parent.UserConstructionScript`))