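; State machine state that waits for level content to be placed before the game moves on.
; On entry it looks up and caches the state manager and the level placement proxy actors.
; Each tick it polls the proxy's ContentPlaced flag and, once set, asks the manager to change to the next state.
; An alternative condition that also passes without a connected head-mounted display is present but unused.
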(fn `On Entry`
  (`parent.On Entry`)
  (`|ExecutionSequence`
    (:`then_0`
      (bind _returnvalue (`GameplayStatics.GetActorOfClass` "/Game/Framework/StateMachine/BP_StateManager.BP_StateManager_C"))
      (set `self.StateManager` _returnvalue))
    (:`then_1`
      (bind _returnvalue_2 (`GameplayStatics.GetActorOfClass` "/Game/Framework/BP_LevelPlacementProxy.BP_LevelPlacementProxy_C"))
      (set `self.LevelPlacementProxy` _returnvalue_2))))

(fn `OnExit`
  (`parent.OnExit`))

(fn `OnTick`
  (params (TimeInState :type "Float (double-precision)"))
  (`parent.OnTick` TimeInState)
  (if (`/Game/Framework/BP_LevelPlacementProxy.ContentPlaced` (`self.LevelPlacementProxy`))
    (`/Game/Framework/StateMachine/BP_StateManager.ChangeState` (`self.StateManager`) "NewEnumerator15")))

(fn `UserConstructionScript`)