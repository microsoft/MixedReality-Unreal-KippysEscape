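; Game state for the cable connection puzzle, where a hanging cable is plugged in to extend a bridge.
; On entry it starts the bridge sequence and moves the character to the bridge start.
; Tick escalates timed hints, first highlighting the plug with Astro audio, then having Astro point at the socket.
; Insertion clears hints and makes Astro react; full extension triggers a celebration and advances the state manager.
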(fn `Init`
  (`parent.Init`)
  (bind _returnvalue (`GameplayStatics.GetActorOfClass` "/Game/Blueprints/newBridge/BP_Bridge01.BP_Bridge01_C"))
  (set `self.CableBridge` _returnvalue)
  (bind _returnvalue_2 (`GameplayStatics.GetActorOfClass` "/Game/Blueprints/newBridge/BP_HangingCable.BP_HangingCable_C"))
  (set `self.Plug` _returnvalue_2))

(fn `On Entry`
  (`parent.On Entry`)
  (set `/Game/Blueprints/newBridge/BP_Bridge01.Active` true (`self.CableBridge`))
  (`/Game/Blueprints/newBridge/BP_Bridge01.InitialSequence` (`self.CableBridge`))
  (`self.MoveCharacterToWaypoint` "CableBridgeStart"))

(fn `OnExit`
  (`/Game/Blueprints/newBridge/BP_HangingCable.DeactivateHint` (`self.Plug`))
  (`/Game/Blueprints/Astro/BP_Astro.DisablePoint` (`self.Astro`)))

(fn `OnTick`
  (params (TimeInState :type "Float (double-precision)"))
  (locals (NewLocalVar_0 :type "Float (double-precision)" :default 0.0))
  (`parent.OnTick` TimeInState)
  (`|ExecutionSequence`
    (:`then_0`
      ;[1 1 1] Highlight Hint
      (if (and (not (`self.HighlightHintActivated`)) (> TimeInState (`self.TimeUntilHighlightHint`)))
        (set `self.HighlightHintActivated` true)
        (`/Game/Blueprints/newBridge/BP_HangingCable.ActivateHint` (`self.Plug`))
        (`/Game/Blueprints/Astro/BP_Astro.PlayAudio` (`self.Astro`) "NewEnumerator1")))
    (:`then_1`
      ;[1 1 1] Character Hint
      (if (and (not (`self.CharacterHintActivated`)) (> TimeInState (`self.TimeUntilCharacterHint`)))
        (set `self.CharacterHintActivated` true)
        (`/Game/Blueprints/Astro/BP_Astro.EnablePoint` (`self.Astro`) (`SceneComponent.K2_GetComponentLocation` (`/Game/Blueprints/newBridge/BP_Bridge01.plugOverlap` (`self.CableBridge`))) 5.0)))
    (:`then_2`
      ;[1 1 1] Toggle Astro Happy When Plugged In
      (if (and (`/Game/Blueprints/newBridge/BP_Bridge01.PlugInserted` (`self.CableBridge`)) (not (`self.PuzzleComplete`)))
        (set `self.PuzzleComplete` true)
        (`/Game/Blueprints/Astro/BP_Astro.DisablePoint` (`self.Astro`))
        (`/Game/Blueprints/Astro/BP_Astro.TriggerExpression` (`self.Astro`) "NewEnumerator1" 1.0)
        (`/Game/Blueprints/newBridge/BP_HangingCable.DeactivateHint` (`self.Plug`))))
    (:`then_3`
      ;[1 1 1] Astro Celebrate and Change State When Bridge Complete
      (if (`/Game/Blueprints/newBridge/BP_Bridge01.Extended` (`self.CableBridge`))
        (`/Game/Blueprints/Astro/BP_Astro.TriggerExpression` (`self.Astro`) "NewEnumerator7" 3.0)
        (`/Game/Framework/StateMachine/BP_StateManager.ChangeState` (`self.StateManager`) "NewEnumerator4")))))

(fn `UserConstructionScript`
  (`parent.UserConstructionScript`))