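; BP_ResetGame is a state in the game's state machine framework that restarts the match when entered.
; On entry it runs the parent logic, casts the current game mode to GameMode and calls RestartGame, doing nothing further if the cast fails.
; Init, exit and tick only forward to the parent state, with the tick passing zero instead of the actual time in state.
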(fn `Init`
  (`parent.Init`))

(fn `On Entry`
  (`parent.On Entry`)
  (bind _asgame_mode (cast `GameMode` (`GameplayStatics.GetGameMode`)))
  (`GameMode.RestartGame` _asgame_mode))

(fn `OnExit`
  (`parent.OnExit`))

(fn `OnTick`
  (params (TimeInState :type "Float (double-precision)"))
  (`parent.OnTick` 0.0))

(fn `UserConstructionScript`
  (`parent.UserConstructionScript`))