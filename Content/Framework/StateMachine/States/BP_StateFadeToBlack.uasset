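; BP_StateFadeToBlack is a state for the game's state machine that fades out ambient audio and waits for the camera fade to finish.
; On entry it caches the state manager, the first AmbientSound actor and the MR pawn, then fades that sound to silence.
; Each tick it polls the pawn's CameraFadeComplete flag and tells BP_StateManager to change state once it is true.
; The camera fade itself is not started here.
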(fn `Init`
  (`parent.Init`))

(fn `On Entry`
  (`parent.On Entry`)
  (bind _returnvalue (`GameplayStatics.GetActorOfClass` "/Game/Framework/StateMachine/BP_StateManager.BP_StateManager_C"))
  (set `self.StateManager` _returnvalue)
  (bind _returnvalue_2 (`GameplayStatics.GetActorOfClass` "/Script/Engine.AmbientSound"))
  (set `self.AmbientAudio` _returnvalue_2)
  (bind _asbp_mrpawn (cast `/Game/Framework/BP_MRPawn` (`GameplayStatics.GetPlayerPawn` 0)))
  (set `self.Pawn` _asbp_mrpawn)
  (`AudioComponent.FadeOut` (`AmbientSound.AudioComponent` (`self.AmbientAudio`)) 3.0 0.0 "Linear"))

(fn `OnExit`
  (`parent.OnExit`))

(fn `OnTick`
  (params (TimeInState :type "Float (double-precision)"))
  (`parent.OnTick` TimeInState)
  (if (`/Game/Framework/BP_MRPawn.CameraFadeComplete` (`self.Pawn`))
    (`/Game/Framework/StateMachine/BP_StateManager.ChangeState` (`self.StateManager`) "NewEnumerator10")))

(fn `UserConstructionScript`
  (`parent.UserConstructionScript`))