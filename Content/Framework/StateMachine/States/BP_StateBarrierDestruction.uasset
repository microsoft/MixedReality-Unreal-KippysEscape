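; State machine state for the bomb island segment, where a rubble barrier is cleared with help from a bomb dispenser.
; Init finds the barrier, dispenser and island actors; entry and exit toggle dispenser and island glow and move Astro between waypoints.
; Tick fires one-shot timed pointing hints and moves, sends Astro to partly cleared rubble, and changes state once all is cleared.
; The highlight hint only sets its flag.
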(fn `Init`
  (`parent.Init`)
  (`|ExecutionSequence`
    (:`then_0`
      (bind _returnvalue (`GameplayStatics.GetActorOfClass` "/Game/Blueprints/BP_Island03Stairwell.BP_Island03Stairwell_C"))
      (set `self.Barrier` _returnvalue))
    (:`then_1`
      (bind _returnvalue_2 (`GameplayStatics.GetActorOfClass` "/Game/Blueprints/BP_BombFactoryV2.BP_BombFactoryV2_C"))
      (set `self.BombDispenser` _returnvalue_2))
    (:`then_3`
      (bind _returnvalue_3 (`GameplayStatics.GetActorOfClass` "/Game/Blueprints/Islands/BP_Island03.BP_Island03_C"))
      (set `self.BombIslandGeo` _returnvalue_3))))

(fn `On Entry`
  (`parent.On Entry`)
  (`|ExecutionSequence`
    (:`then_0`
      (`/Game/Blueprints/BP_BombFactoryV2.ActivateDeactivate` (`self.BombDispenser`) true))
    (:`then_1`
      (`self.MoveCharacterToWaypoint` "BombIslandStart"))
    (:`then_2`
      (`/Game/Blueprints/Islands/BP_Island03.ToggleIslandGlow` (`self.BombIslandGeo`) true))))

(fn `OnExit`
  (bind _bombdispenser (`self.BombDispenser`))
  (`parent.OnExit`)
  (`self.MoveCharacterToWaypoint` "SliderBridgeStart")
  (`/Game/Blueprints/Astro/BP_Astro.DisablePoint` (`self.Astro`))
  (`/Game/Blueprints/Islands/BP_Island03.ToggleIslandGlow` (`self.BombIslandGeo`) false)
  (`/Game/Blueprints/BP_BombFactoryV2.ActivateDeactivate` _bombdispenser false)
  (set `/Game/Blueprints/BP_BombFactoryV2.Active` false _bombdispenser))

(fn `OnTick`
  (params (TimeInState :type "Float (double-precision)"))
  (`parent.OnTick` TimeInState)
  (`|ExecutionSequence`
    (:`then_0`
      ;[1 1 1] Character Hint
      (if (and (not (`self.CharacterHintActivated`)) (> TimeInState (`self.TimeUntilCharacterHint`)))
        (set `self.CharacterHintActivated` true)
        (`/Game/Blueprints/Astro/BP_Astro.EnablePoint` (`self.Astro`) (`SceneComponent.K2_GetComponentLocation` (`/Game/Blueprints/BP_BombFactoryV2.SpawnLocation` (`self.BombDispenser`))) 5.0)))
    (:`then_1`
      ;[1 1 1] Highlight hint
      (if (and (not (`self.HighlightHintActivated`)) (> TimeInState (`self.TimeUntilHighlightHint`)))
        (set `self.HighlightHintActivated` true)))
    (:`then_2`
      ;[1 1 1] Move to Bomb Machine
      (if (and (> TimeInState (`self.TimeUntilAstroMoveToBombMachine`)) (not (`self.AstroMovedToBombMachine`)))
        (set `self.AstroMovedToBombMachine` true)
        (`self.MoveCharacterToWaypoint` "BombDispenser")))
    (:`then_3`
      (if (and (or (`/Game/Blueprints/BP_Island03Stairwell.LeftRubbleCleared` (`self.Barrier`)) (`/Game/Blueprints/BP_Island03Stairwell.RightRubbleCleared` (`self.Barrier`))) (not (`self.AstroMoveToRubble`)))
        (set `self.AstroMoveToRubble` true)
        (`self.MoveCharacterToWaypoint` "RubblePile")))
    (:`then_4`
      (if (`/Game/Blueprints/BP_Island03Stairwell.RubbleCleared` (`self.Barrier`))
        (`/Game/Framework/StateMachine/BP_StateManager.ChangeState` (`self.StateManager`) "NewEnumerator6")))))

(fn `UserConstructionScript`
  (`parent.UserConstructionScript`))