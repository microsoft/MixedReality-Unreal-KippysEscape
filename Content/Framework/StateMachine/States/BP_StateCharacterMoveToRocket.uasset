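; State machine state that walks the Astro character to the rocket for a goodbye and boarding.
; On entry it sends Astro to the WaveGoodbye waypoint, opens the door of the rocket found during Init and triggers an expression.
; Each tick, gated on Astro's locomotion state, it retries that move, waves once on arrival, then heads to InRocket.
; Reaching InRocket hands over to the next state through the StateManager.
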(fn `Init`
  (`parent.Init`)
  (bind _returnvalue (`GameplayStatics.GetActorOfClass` "/Game/Blueprints/BP_Rocket.BP_Rocket_C"))
  (set `self.Rocket` _returnvalue))

(fn `On Entry`
  (`parent.On Entry`)
  (`self.MoveCharacterToWaypoint` "WaveGoodbye")
  (`/Game/Blueprints/BP_Rocket.OpenDoor` (`self.Rocket`))
  (`/Game/Blueprints/Astro/BP_Astro.TriggerExpression` (`self.Astro`) "NewEnumerator1" 100.0))

(fn `OnExit`
  (`parent.OnExit`))

(fn `OnTick`
  (params (TimeInState :type "Float (double-precision)"))
  (`parent.OnTick` TimeInState)
  (`|ExecutionSequence`
    (:`then_0`
      (if (and (`|EnumEquality` (`/Game/Blueprints/Astro/ABP_Astro.LocomotionState` (`/Game/Blueprints/Astro/BP_Astro.ABP` (`self.Astro`))) "NewEnumerator0") (not (`self.HasCharacterReachedWaypoint` "WaveGoodbye")))
        (`self.MoveCharacterToWaypoint` "WaveGoodbye")))
    (:`then_1`
      (if (and (`self.HasCharacterReachedWaypoint` "WaveGoodbye") (not (`self.AstroWaved`)) (`|EnumEquality` (`/Game/Blueprints/Astro/ABP_Astro.LocomotionState` (`/Game/Blueprints/Astro/BP_Astro.ABP` (`self.Astro`))) "NewEnumerator0"))
        (`/Game/Blueprints/Astro/BP_Astro.Wave` (`self.Astro`) 3.0 true)
        (set `self.AstroWaved` true)))
    (:`then_2`
      (if (and (`self.AstroWaved`) (`|EnumEquality` (`/Game/Blueprints/Astro/ABP_Astro.LocomotionState` (`/Game/Blueprints/Astro/BP_Astro.ABP` (`self.Astro`))) "NewEnumerator0"))
        (`self.MoveCharacterToWaypoint` "InRocket")))
    (:`then_3`
      (if (`self.HasCharacterReachedWaypoint` "InRocket")
        (`/Game/Framework/StateMachine/BP_StateManager.ChangeState` (`self.StateManager`) "NewEnumerator12")))))

(fn `UserConstructionScript`
  (`parent.UserConstructionScript`))