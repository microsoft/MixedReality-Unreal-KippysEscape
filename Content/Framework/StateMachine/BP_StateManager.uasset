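; State manager that spawns an actor per game phase, from anchor check through puzzle interactions to rocket blast-off, game over and reset.
; ChangeState exits the active state and diffs the new state's required streaming levels against those loaded.
; When levels differ, Tick runs a loading machine: black wipe, sequential unloads and loads, wipe back, then OnEntry.
; Otherwise entry is immediate; outside loading, Tick passes elapsed state time to the active state.
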(event `self.ReceiveBeginPlay`
  (`|ExecutionSequence`
    (:`then_0`
      (bind _returnvalue (`GameplayStatics.GetActorOfClass` "/Game/Blueprints/BP_LoadingWipeScreen.BP_LoadingWipeScreen_C"))
      (set `self.LoadingScreen` _returnvalue))
    (:`then_1`
      (`self.CreateState` "NewEnumerator15" "/Game/Framework/StateMachine/States/BP_StateLoading.BP_StateLoading_C")
      (`self.CreateState` "NewEnumerator0" "/Game/Framework/StateMachine/States/BP_StateCheckForAnchor.BP_StateCheckForAnchor_C")
      (`self.CreateState` "NewEnumerator1" "/Game/Framework/StateMachine/States/BP_StateContentPlacement.BP_StateContentPlacement_C")
      (`self.CreateState` "NewEnumerator2" "/Game/Framework/StateMachine/States/BP_StateIntroSequence.BP_StateIntroSequence_C")
      (`self.CreateState` "NewEnumerator3" "/Game/Framework/StateMachine/States/BP_StateCableConnection.BP_StateCableConnection_C")
      (`self.CreateState` "NewEnumerator4" "/Game/Framework/StateMachine/States/BP_StateGemPlacement.BP_StateGemPlacement_C")
      (`self.CreateState` "NewEnumerator5" "/Game/Framework/StateMachine/States/BP_StateBarrierDestruction.BP_StateBarrierDestruction_C")
      (`self.CreateState` "NewEnumerator6" "/Game/Framework/StateMachine/States/BP_StateSliderInteraction.BP_StateSliderInteraction_C")
      (`self.CreateState` "NewEnumerator7" "/Game/Framework/StateMachine/States/BP_StateCharacterMoveToRocket.BP_StateCharacterMoveToRocket_C")
      (`self.CreateState` "NewEnumerator12" "/Game/Framework/StateMachine/States/BP_StateRocketBlastOff.BP_StateRocketBlastOff_C")
      (`self.CreateState` "NewEnumerator8" "/Game/Framework/StateMachine/States/BP_StateFadeToBlack.BP_StateFadeToBlack_C")
      (`self.CreateState` "NewEnumerator10" "/Game/Framework/StateMachine/States/BP_StateGameOver.BP_StateGameOver_C")
      (`self.CreateState` "NewEnumerator16" "/Game/Framework/StateMachine/States/BP_ResetGame.BP_ResetGame_C"))
    (:`then_2`
      (`self.ChangeState` "NewEnumerator0"))))

(event `self.ReceiveTick`
  (params (DeltaSeconds :type "Float (single-precision)"))
  (switch `/Game/Framework/StateMachine/ELoadingState` (`self.LoadingState`)
    (:`NewEnumerator3`
      ;[1 1 1] State Tick
      (set `self.TimeInCurrentState` (+ DeltaSeconds (`self.TimeInCurrentState`)))
      (`/Game/Framework/StateMachine/BP_GameState.OnTick` (`self.ActiveState`) (`self.TimeInCurrentState`)))
    (:`NewEnumerator0`
      (`|ExecutionSequence`
        (:`then_0`
          ;[1 1 1] Camera fade before load
          (`/Engine/EditorBlueprintResources/StandardMacros.DoOnce` false :!label _label
            (:`Completed`
              (`/Game/Blueprints/BP_LoadingWipeScreen.ActivateBlackWipe` (`self.LoadingScreen`) true)
              (`KismetSystemLibrary.Delay` (`self.CameraFadeDuration`))
              (set `self.LoadingState` "NewEnumerator5"))))
        (:`then_1`
          (goto _label_2 :!via `Reset`))))
    (:`NewEnumerator5`
      ;[1 1 1] Unload each level
      (if (and (== (`self.CurrentlyUnloadingLevel`) "None") (> (`KismetArrayLibrary.Array_Length` (`self.LevelsToUnload`)) 0))
        (bind _output_get (set `self.CurrentlyUnloadingLevel` (`|GetArrayItem` (`self.LevelsToUnload`))))
        (`KismetArrayLibrary.Array_RemoveItem` (`self.CurrentLoadedLevels`) _output_get)
        (`KismetArrayLibrary.Array_Remove` (`self.LevelsToUnload`))
        (`KismetSystemLibrary.PrintString` (`KismetStringLibrary.Concat_StrStr` "Unloading Level: " (`KismetStringLibrary.Conv_NameToString` (`self.CurrentlyUnloadingLevel`))))
        (`GameplayStatics.UnloadStreamLevel` (`self.CurrentlyUnloadingLevel`) true)
        (elif (== (`self.CurrentlyUnloadingLevel`) "None")
          (set `self.LoadingState` "NewEnumerator1")
          (elif (not (`LevelStreaming.IsLevelLoaded` (`GameplayStatics.GetStreamingLevel` (`self.CurrentlyUnloadingLevel`))))
            (set `self.CurrentlyUnloadingLevel` "None")
            (if (<= (`KismetArrayLibrary.Array_Length` (`self.LevelsToUnload`)) 0)
              (set `self.LoadingState` "NewEnumerator1"))))))
    (:`NewEnumerator1`
      ;[1 1 1] Load each level
      (if (and (== (`self.CurrentlyLoadingLevel`) "None") (> (`KismetArrayLibrary.Array_Length` (`self.LevelsToLoad`)) 0))
        (bind _output_get_2 (set `self.CurrentlyLoadingLevel` (`|GetArrayItem` (`self.LevelsToLoad`))))
        (`KismetArrayLibrary.Array_Add` (`self.CurrentLoadedLevels`) _output_get_2)
        (`KismetArrayLibrary.Array_Remove` (`self.LevelsToLoad`))
        (`KismetSystemLibrary.PrintString` (`KismetStringLibrary.Concat_StrStr` "Loading Level: " (`KismetStringLibrary.Conv_NameToString` (`self.CurrentlyLoadingLevel`))))
        (`GameplayStatics.LoadStreamLevel` (`self.CurrentlyLoadingLevel`) true true)
        (elif (== (`self.CurrentlyLoadingLevel`) "None")
          (set `self.LoadingState` "NewEnumerator2")
          (elif (`LevelStreaming.IsLevelLoaded` (`GameplayStatics.GetStreamingLevel` (`self.CurrentlyLoadingLevel`)))
            (set `self.CurrentlyLoadingLevel` "None")
            (if (<= (`KismetArrayLibrary.Array_Length` (`self.LevelsToLoad`)) 0)
              (set `self.LoadingState` "NewEnumerator2"))))))
    (:`NewEnumerator2`
      (`|ExecutionSequence`
        (:`then_0`
          (goto _label :!via `Reset`))
        (:`then_1`
          ;[1 1 1] Camera fade in after load
          (`/Engine/EditorBlueprintResources/StandardMacros.DoOnce` false :!label _label_2
            (:`Completed`
              (`/Game/Blueprints/BP_LoadingWipeScreen.ActivateBlackWipe` (`self.LoadingScreen`) false)
              (`KismetSystemLibrary.Delay` (`self.CameraFadeDuration`))
              (`/Game/Framework/StateMachine/BP_GameState.On Entry` (`self.ActiveState`))
              (set `self.LoadingState` "NewEnumerator3"))))))))

(fn `ChangeState`
  (params (NewState :type "/Game/Framework/StateMachine/EGameState Enum" :default "NewEnumerator9"))
  (locals (UpdatedStateID :type "/Game/Framework/StateMachine/EGameState Enum" :default "NewEnumerator9") (UpdatedState :type "/Game/Framework/StateMachine/BP_GameState Object Reference"))
  (bind (_value _returnvalue) (`BlueprintMapLibrary.Map_Find` (`self.StateMap`) (`self.CurrentState`)))
  ;[1 1 1] Check not same as current state
  (if (and (`|EnumInequality` NewState (`self.CurrentState`)) (`|EnumEquality` (`self.LoadingState`) "NewEnumerator3"))
    ;[1 1 1] Check new state exists
    (bind _output_get (set `local.UpdatedStateID` NewState))
    (bind (_value_2 _returnvalue_2) (`BlueprintMapLibrary.Map_Find` (`self.StateMap`) _output_get))
    (if _returnvalue_2
      (set `local.UpdatedState` _value_2)
      ;[1 1 1] Previous State on exit
      (if _returnvalue
        (`/Game/Framework/StateMachine/BP_GameState.OnExit` _value)
        (else
          (`KismetSystemLibrary.PrintString` "Cannot exit state - does not have an actor associated with it." false)))
      (set `self.TimeInCurrentState` 0.0)
      (set `self.CurrentState` (`local.UpdatedStateID`))
      (set `self.ActiveState` (`local.UpdatedState`))
      ;[1 1 1] Clear
      (`KismetArrayLibrary.Array_Clear` (`self.LevelsToLoad`))
      (`KismetArrayLibrary.Array_Clear` (`self.LevelsToUnload`))
      ;[1 1 1] Set Levels to Load
      (for _array_element (`/Game/Framework/StateMachine/BP_GameState.RequiredLevels` (`local.UpdatedState`))
        (if (`KismetArrayLibrary.Array_Contains` (`self.CurrentLoadedLevels`) _array_element)
          (`KismetSystemLibrary.PrintString` (`KismetStringLibrary.Concat_StrStr` (`KismetStringLibrary.Conv_NameToString` _array_element) " already loaded.") false)
          (else
            (`KismetArrayLibrary.Array_Add` (`self.LevelsToLoad`) _array_element))))
      ;[1 1 1] Set Levels to Unload
      (for _array_element_2 (`self.CurrentLoadedLevels`)
        (if (not (`KismetArrayLibrary.Array_Contains` (`/Game/Framework/StateMachine/BP_GameState.RequiredLevels` (`local.UpdatedState`)) _array_element_2))
          (`KismetArrayLibrary.Array_Add` (`self.LevelsToUnload`) _array_element_2)))
      ;[1 1 1] Check anything to load or unload
      (if (or (> (`KismetArrayLibrary.Array_Length` (`self.LevelsToLoad`)) 0) (> (`KismetArrayLibrary.Array_Length` (`self.LevelsToUnload`)) 0))
        (set `self.LoadingState` "NewEnumerator0")
        (else
          (`KismetSystemLibrary.PrintString` "No need to load or unload anything new" false)
          (`/Game/Framework/StateMachine/BP_GameState.On Entry` (`self.ActiveState`))))
      (else
        (`KismetSystemLibrary.PrintString` "Error: Requested state does not have an associated class" false)))))

(fn `CheckLevelsLoaded`
  (params (Levels :type "Array of Name"))
  (returns (Loaded :type Boolean))
  (locals (LoadFinished :type Boolean))
  (set `local.LoadFinished` true)
  (for _array_element Levels
    (bind _returnvalue (`GameplayStatics.GetStreamingLevel` _array_element))
    (if (not (and (`LevelStreaming.IsLevelLoaded` _returnvalue) (`LevelStreaming.IsLevelVisible` _returnvalue)))
      (set `local.LoadFinished` false)))
  (return (`local.LoadFinished`)))

(fn `CheckLevelsUnloaded`
  (params (Levels :type "Array of Name"))
  (returns (Unloaded :type Boolean))
  (locals (UnloadFinished :type Boolean))
  (set `local.UnloadFinished` true)
  (for _array_element Levels
    (if (`LevelStreaming.IsLevelLoaded` (`GameplayStatics.GetStreamingLevel` _array_element))
      (set `local.UnloadFinished` false)))
  (return (`local.UnloadFinished`)))

(fn `CreateState`
  (params (StateID :type "/Game/Framework/StateMachine/EGameState Enum" :default "NewEnumerator9") (StateClass :type "/Game/Framework/StateMachine/BP_GameState Class Reference"))
  (bind _returnvalue (`|SpawnActorFromClass` StateClass (`KismetMathLibrary.MakeTransform` (0.0 0.0 0.0)) "Undefined" "OverrideRootScale" null null))
  (`BlueprintMapLibrary.Map_Add` (`self.StateMap`) StateID _returnvalue)
  (return))

(fn `GetCurrentState`
  (returns (NewParam :type "/Game/Framework/StateMachine/EGameState Enum"))
  (return (`self.CurrentState`)))

(fn `GetSkipState`
  (returns (SkipState :type "/Game/Framework/StateMachine/EGameState Enum"))
  (bind (_value _returnvalue) (`BlueprintMapLibrary.Map_Find` (`self.StateMap`) (`self.CurrentState`)))
  (if _returnvalue
    (return (`/Game/Framework/StateMachine/BP_GameState.SkipState` _value))
    (else
      (`KismetSystemLibrary.PrintString` "No valid skip state found"))))

(fn `GetTimeInCurrentState`
  (returns (Time :type "Float (double-precision)"))
  (return (`self.TimeInCurrentState`)))

(fn `InitGameStates`
  (`|ExecutionSequence`
    (:`then_0`
      (`/Game/Framework/StateMachine/BP_GameState.Init` (`BlueprintMapLibrary.Map_Find` (`self.StateMap`) "NewEnumerator2")))
    (:`then_1`
      (`/Game/Framework/StateMachine/BP_GameState.Init` (`BlueprintMapLibrary.Map_Find` (`self.StateMap`) "NewEnumerator3")))
    (:`then_2`
      (`/Game/Framework/StateMachine/BP_GameState.Init` (`BlueprintMapLibrary.Map_Find` (`self.StateMap`) "NewEnumerator4")))
    (:`then_3`
      (`/Game/Framework/StateMachine/BP_GameState.Init` (`BlueprintMapLibrary.Map_Find` (`self.StateMap`) "NewEnumerator5")))
    (:`then_4`
      (`/Game/Framework/StateMachine/BP_GameState.Init` (`BlueprintMapLibrary.Map_Find` (`self.StateMap`) "NewEnumerator6")))
    (:`then_5`
      (`/Game/Framework/StateMachine/BP_GameState.Init` (`BlueprintMapLibrary.Map_Find` (`self.StateMap`) "NewEnumerator7")))
    (:`then_6`
      (`/Game/Framework/StateMachine/BP_GameState.Init` (`BlueprintMapLibrary.Map_Find` (`self.StateMap`) "NewEnumerator12")))
    (:`then_7`
      (`/Game/Framework/StateMachine/BP_GameState.Init` (`BlueprintMapLibrary.Map_Find` (`self.StateMap`) "NewEnumerator10")))
    (:`then_8`
      (`/Game/Framework/StateMachine/BP_GameState.Init` (`BlueprintMapLibrary.Map_Find` (`self.StateMap`) "NewEnumerator16")))))

(fn `UserConstructionScript`)