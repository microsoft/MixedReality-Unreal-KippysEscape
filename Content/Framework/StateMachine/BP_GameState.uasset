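; BP_GameState is a base state for a game state machine, with entry, tick and exit hooks and helpers for directing the Astro character.
; Init caches the state manager and Astro, then maps every BP_CharacterWaypoint in the level by name.
; Helpers use that map to move or teleport Astro to a named waypoint, or test arrival by transform tolerance.
; Entry and exit print the state ID, and movement helpers report missing references or waypoints.
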(fn `HasCharacterReachedWaypoint`
  (params (Waypoint :type String))
  (returns (WaypointReached :type Boolean))
  (return (`KismetMathLibrary.NearlyEqual_TransformTransform` (`self.GetTransform` (`BlueprintMapLibrary.Map_Find` (`self.Waypoints`) Waypoint)) (`self.GetTransform` (`self.Astro`)) 8.0 8.0 1.0)))

(fn `Init`
  (bind _returnvalue (`GameplayStatics.GetActorOfClass` "/Game/Framework/StateMachine/BP_StateManager.BP_StateManager_C"))
  (set `self.StateManager` _returnvalue)
  (bind _returnvalue_2 (`GameplayStatics.GetActorOfClass` "/Game/Blueprints/Astro/BP_Astro.BP_Astro_C"))
  (set `self.Astro` _returnvalue_2)
  (bind _outactors (`GameplayStatics.GetAllActorsOfClass` "/Game/Blueprints/BP_CharacterWaypoint.BP_CharacterWaypoint_C"))
  (for _array_element _outactors
    (`BlueprintMapLibrary.Map_Add` (`self.Waypoints`) (`/Game/Blueprints/BP_CharacterWaypoint.WaypointName` _array_element) _array_element)))

(fn `MoveCharacterToWaypoint`
  (params (WaypointName :type String))
  (bind (_value _returnvalue) (`BlueprintMapLibrary.Map_Find` (`self.Waypoints`) WaypointName))
  (`/Engine/EditorBlueprintResources/StandardMacros.IsValid` (`self.Astro`)
    (:`Is Valid`
      (if _returnvalue
        (`/Game/Blueprints/Astro/BP_Astro.MoveTo` (`self.Astro`) _value)
        (else
          (`KismetSystemLibrary.PrintString` (`KismetStringLibrary.Concat_StrStr` "Could not find waypoint: " WaypointName) false))))
    (:`Is Not Valid`
      (`KismetSystemLibrary.PrintString` "Character reference invalid in state" false))))

(fn `On Entry`
  (`KismetSystemLibrary.PrintString` (`KismetStringLibrary.Concat_StrStr` "State entered: " (`|GetEnumeratorNameAsString` (`self.StateID`))) false))

(fn `OnExit`
  (`KismetSystemLibrary.PrintString` (`KismetStringLibrary.Concat_StrStr` "State exited: " (`|GetEnumeratorNameAsString` (`self.StateID`))) false))

(fn `OnTick`
  (params (TimeInState :type "Float (double-precision)")))

(fn `TeleportCharacterToWaypoint`
  (params (WaypointName :type String))
  (bind (_value _returnvalue) (`BlueprintMapLibrary.Map_Find` (`self.Waypoints`) WaypointName))
  (`/Engine/EditorBlueprintResources/StandardMacros.IsValid` (`self.Astro`)
    (:`Is Valid`
      (if _returnvalue
        (`/Game/Blueprints/Astro/BP_Astro.TeleportTo` (`self.Astro`) _value)
        (else
          (`KismetSystemLibrary.PrintString` (`KismetStringLibrary.Concat_StrStr` "Could not find waypoint: " WaypointName) false))))
    (:`Is Not Valid`
      (`KismetSystemLibrary.PrintString` "Character reference invalid in state" false))))

(fn `UserConstructionScript`)